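; BP_FloatingCandle is a Great Hall map prop that makes its static mesh bob up and down like a floating candle.
; From BeginPlay, two eased MoveComponentTo moves alternate in an endless latent loop, rising then falling by random distances over random durations.
; Each target offsets the mesh's current world location but is passed as a relative location, with no fixed origin to prevent drift.
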(event EventBeginPlay
  (bind _staticmesh (Variables|Default|GetStaticMesh))
  (bind _staticmesh_2 (Variables|Default|GetStaticMesh))
  (bind _returnvalue (Transformation|GetWorldLocation _staticmesh_2))
  (bind _returnvalue_2 (Transformation|GetWorldLocation _staticmesh))
  (Components|MoveComponentTo _staticmesh_2 (Math|Vector|MakeVector (.x _returnvalue) (.y _returnvalue) (+ (.z _returnvalue) (Math|Random|RandomFloatinRange 1e+02 2e+02))) "0, 0, 0" true true (Math|Random|RandomFloatinRange 2.0 5.0) false :!label _label)
  (Components|MoveComponentTo _staticmesh (Math|Vector|MakeVector (.x _returnvalue_2) (.y _returnvalue_2) (+ (.z _returnvalue_2) (Math|Random|RandomFloatinRange -1e+02 -2e+02))) "0, 0, 0" true true (Math|Random|RandomFloatinRange 2.0 5.0) false)
  (goto _label))

(fn ConstructionScript)