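; Smithing anvil for the LineageDuel map that upgrades equipment when struck with a smith hammer.
; Interacting places held equipment listed in UpgradeTable onto an empty anvil, attached at AttachPoint.
; Damage counts only from downward-angled left or right hammer strikes; a hit replaces the item with its table upgrade.
; Repeated hits on an empty anvil call SpawnNewItem without a specified type, and items detached from the anvil are forgotten.
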(event EventBeginPlay
  (|CallParentFunction) ; This node is disabled and will not be called.\nDrag off pins to build functionality.
)

(event Collision|EventActorBeginOverlap
  (params (OtherActor :type Actor%20Object%20Reference))
  (|CallParentFunction OtherActor) ; This node is disabled and will not be called.\nDrag off pins to build functionality.
)

(event EventOnInteractionStart
  (params (Character :type Mordhau%20Character%20Object%20Reference))
  (CallFunction|ValidateCurrentItem)
  (Utilities|IsValid (Variables|Default|GetCurrentItem)
    (:Is%20Not%20Valid
      (bind _equipment (CallFunction|GetEquipmenttoPlace Character))
      (Utilities|IsValid _equipment
        (:Is%20Valid
          (Class|MordhauCharacter|DropEquipment Character _equipment)
          (CallFunction|AttachEquipment _equipment))))))

(event EventTick
  (params (DeltaSeconds :type Float%20%28single-precision%29))
  (|CallParentFunction DeltaSeconds) ; This node is disabled and will not be called.\nDrag off pins to build functionality.
)

(event Game|Damage|EventAnyDamage
  (params (Damage :type Float%20%28single-precision%29) (DamageType :type Damage%20Type%20Object%20Reference) (InstigatedBy :type Controller%20Object%20Reference) (DamageCauser :type Actor%20Object%20Reference))
  (bind _asmordhau_character (Utilities|Casting|CastToMordhauCharacter DamageCauser))
  (bind _asattack_motion (Utilities|Casting|CastToAttackMotion (Variables|/Script/Mordhau.MordhauCharacter|GetMotion _asmordhau_character)))
  (if (or (Utilities|Enum|Equal(Enum) (Variables|/Script/Mordhau.AttackMotion|GetMove _asattack_motion) "RightStrike") (Utilities|Enum|Equal(Enum) (Variables|/Script/Mordhau.AttackMotion|GetMove _asattack_motion) "LeftStrike"))
    (if (and (== (Utilities|GetClass (Variables|/Script/Mordhau.AttackMotion|GetWeapon _asattack_motion)) "/Game/Mordhau/Blueprints/Equipment/Weapons/Specific/OneHanded/BP_SmithHammer.BP_SmithHammer_C") (<= (Class|KismetMathLibrary|DegAcos (Math|Vector|DotProduct (Math|Vector|Normalize (* (Variables|/Script/Mordhau.MordhauWeapon|GetLastObservedTraceDirection (Variables|/Script/Mordhau.AttackMotion|GetWeapon _asattack_motion)) -1.0)) (Transformation|GetActorUpVector))) 5e+01))
      (CallFunction|ValidateCurrentItem)
      (Utilities|IsValid (Variables|Default|GetCurrentItem)
        (:Is%20Valid
          (bind _output_get (Variables|Default|SetTotalHits (+ (Variables|Default|GetTotalHits) 1)))
          (if (>= _output_get 1)
            (CallFunction|UpgradeItem)
            (Variables|Default|SetTotalHits 0)))
        (:Is%20Not%20Valid
          (bind _output_get_2 (Variables|Default|SetTotalHits (+ (Variables|Default|GetTotalHits) 1)))
          (if (>= _output_get_2 6)
            (CallFunction|SpawnNewItem)
            (Variables|Default|SetTotalHits 0)))))))

(fn ConstructionScript
  (|CallParentFunction))

(fn SpawnNewItem
  (params (Type :type Mordhau%20Equipment%20Class%20Reference))
  (bind _currentitem (Variables|Default|GetCurrentItem))
  (Utilities|FlowControl|Sequence
    (:then_0
      (Utilities|IsValid _currentitem
        (:Is%20Valid
          (Actor|DestroyActor _currentitem))))
    (:then_1
      (bind _returnvalue (Game|SpawnActorfromClass Type (Transformation|GetWorldTransform (Variables|Default|GetAttachPoint)) "Undefined" 0 0))
      (Utilities|IsValid _returnvalue
        (:Is%20Valid
          (Class|MordhauEquipment|AssignCustomization _returnvalue (Utilities|Struct|MakeEquipmentCustomization 0 (Utilities|Array|MakeArray 0 0 0) (Utilities|Array|MakeArray 0 0 0)))
          (CallFunction|AttachEquipment _returnvalue))))))

(fn UpgradeItem
  (bind _currentitem (Variables|Default|GetCurrentItem))
  (bind _upgradetable (Variables|Default|GetUpgradeTable))
  (bind _returnvalue (Utilities|GetClass _currentitem))
  (if (Utilities|Map|Contains _upgradetable _returnvalue)
    (CallFunction|SpawnNewItem (.Value (Utilities|Map|Find _upgradetable _returnvalue)))))

(fn CanInteract
  (params (Character :type Mordhau%20Character%20Object%20Reference))
  (if (stale _returnvalue)
    (bind _equipment (CallFunction|GetEquipmenttoPlace Character))
    (Utilities|IsValid _equipment
      (:Is%20Valid
        (return true))
      (:Is%20Not%20Valid
        _)))
  (return false))

(fn AttachEquipment
  (params (Equipment :type Mordhau%20Equipment%20Object%20Reference))
  (bind _output_get (Variables|Default|SetCurrentItem Equipment))
  (Class|MordhauEquipment|DestroyPhysicsProxy _output_get)
  (Transformation|SetActorTransform _output_get (Transformation|GetWorldTransform (Variables|Default|GetAttachPoint)))
  (Transformation|AttachActorToActor _output_get self "None" "KeepWorld" "KeepWorld" "KeepWorld" false))

(fn GetEquipmenttoPlace
  (params (Character :type Mordhau%20Character%20Object%20Reference))
  (bind _lefthandequipment (Variables|/Script/Mordhau.MordhauCharacter|GetLeftHandEquipment Character))
  (bind _righthandequipment (Variables|/Script/Mordhau.MordhauCharacter|GetRightHandEquipment Character))
  (Utilities|FlowControl|Sequence
    (:then_0
      (Utilities|FlowControl|Sequence
        (:then_0
          (Utilities|IsValid _righthandequipment
            (:Is%20Valid
              (if (Utilities|Map|Contains (Variables|Default|GetUpgradeTable) (Utilities|GetClass _righthandequipment))
                (LocalVariables|SetToDrop _righthandequipment)))))
        (:then_1
          (Utilities|IsValid (LocalVariables|GetToDrop)
            (:Is%20Not%20Valid
              (Utilities|IsValid _lefthandequipment
                (:Is%20Valid
                  (if (Utilities|Map|Contains (Variables|Default|GetUpgradeTable) (Utilities|GetClass _lefthandequipment))
                    (LocalVariables|SetToDrop _lefthandequipment)))))))))
    (:then_1
      (return (LocalVariables|GetToDrop)))))

(fn ValidateCurrentItem
  (if (not (== (Variables|Default|GetCurrentItem) 0))
    (Utilities|IsValid (Variables|Default|GetCurrentItem)
      (:Is%20Valid
        (if (not (== (Actor|GetAttachParentActor (Variables|Default|GetCurrentItem)) self))
          (Variables|Default|SetCurrentItem 0 :!label _label)
          (Variables|Default|SetTotalHits 0)))
      (:Is%20Not%20Valid
        (goto _label)))))