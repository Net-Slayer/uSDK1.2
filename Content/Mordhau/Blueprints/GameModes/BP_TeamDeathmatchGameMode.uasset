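; Team Deathmatch game mode for Mordhau that decides when a match ends and records the result.
; When a team's score changes during play and reaches the score to win, it ends the match and sets that team as winner.
; When time runs out, it compares the two team scores and records a winner or a draw.
; Results are written to the match end info on the Mordhau game state.
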(event EventOnTeamScoreChanged
  (params (Team :type Integer) (OldValue :type Float%20%28single-precision%29))
  (bind _asbp_mordhau_game_state (Utilities|Casting|CastToBP_MordhauGameState (Game|GetGameState)))
  (if (and (Class|GameMode|IsMatchinProgress) (>= (Utilities|Array|Get(acopy) (Variables|/Script/Mordhau.MordhauGameState|GetTeamScores _asbp_mordhau_game_state) Team) (Variables|Default|GetTeamScoreToWin)))
    (Class|GameMode|EndMatch)
    (Variables|/Game/Mordhau/Blueprints/GameModes/BP_MordhauGameState.BP_MordhauGameState_C|SetMatchEndInfo _asbp_mordhau_game_state (Utilities|Struct|MakeSTRUCT_MatchEndInfo 0 Team (Utilities|Array|Get(acopy) (Variables|/Script/Mordhau.MordhauGameState|GetTeamScores _asbp_mordhau_game_state) Team)))))

(event EventBeginPlay
  (|CallParentFunction))

(event EventTick
  (params (DeltaSeconds :type Float%20%28single-precision%29)))

(event EventMatchTimeRanOut
  (|CallParentFunction)
  (bind _asbp_mordhau_game_state (Utilities|Casting|CastToBP_MordhauGameState (Game|GetGameState)))
  (if (== (Utilities|Array|Get(acopy) (Variables|/Script/Mordhau.MordhauGameState|GetTeamScores _asbp_mordhau_game_state)) (Utilities|Array|Get(acopy) (Variables|/Script/Mordhau.MordhauGameState|GetTeamScores _asbp_mordhau_game_state) 1))
    (Variables|/Game/Mordhau/Blueprints/GameModes/BP_MordhauGameState.BP_MordhauGameState_C|SetMatchEndInfo _asbp_mordhau_game_state (Utilities|Struct|MakeSTRUCT_MatchEndInfo 0 0 0.0 0.0 true))
    (elif (> (Utilities|Array|Get(acopy) (Variables|/Script/Mordhau.MordhauGameState|GetTeamScores _asbp_mordhau_game_state)) (Utilities|Array|Get(acopy) (Variables|/Script/Mordhau.MordhauGameState|GetTeamScores _asbp_mordhau_game_state) 1))
      (Variables|/Game/Mordhau/Blueprints/GameModes/BP_MordhauGameState.BP_MordhauGameState_C|SetMatchEndInfo _asbp_mordhau_game_state (Utilities|Struct|MakeSTRUCT_MatchEndInfo 0 0 (Utilities|Array|Get(acopy) (Variables|/Script/Mordhau.MordhauGameState|GetTeamScores _asbp_mordhau_game_state))))
      (else
        (Variables|/Game/Mordhau/Blueprints/GameModes/BP_MordhauGameState.BP_MordhauGameState_C|SetMatchEndInfo _asbp_mordhau_game_state (Utilities|Struct|MakeSTRUCT_MatchEndInfo 0 1 (Utilities|Array|Get(acopy) (Variables|/Script/Mordhau.MordhauGameState|GetTeamScores _asbp_mordhau_game_state) 1)))))))

(fn ConstructionScript
  (|CallParentFunction))