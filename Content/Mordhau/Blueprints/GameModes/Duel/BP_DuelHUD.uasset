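; BP_DuelHUD is the HUD for Duel mode, extending a parent HUD with duel-specific widgets.
; On BeginPlay it removes the standard post-match screen and puts a hidden BP_DuelEndScreen in its container, shown through ShowDuelEndScreen.
; Game state replication creates the duel overlay widget and opens the main menu.
; Overlay visibility follows minimal/full HUD and menu toggles, with closing the menu restoring UI-only input to a visible end screen.
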(event EventBeginPlay
  (|CallParentFunction)
  (Widget|RemovefromParent (Variables|Default|GetPostMatchScreen))
  (bind _returnvalue (UserInterface|CreateWidget "/Game/Mordhau/Blueprints/GameModes/Duel/BP_DuelEndScreen.BP_DuelEndScreen_C" (Game|GetPlayerController 0)))
  (bind _output_get (Variables|Default|SetDuelEndScreen _returnvalue))
  (Widget|SetVisibility _output_get "Collapsed")
  (Widget|Panel|AddChild (Variables|/Game/Mordhau/UI/BP_HUDWidget.BP_HUDWidget_C|GetPostMatchScreenContainer (Variables|Default|GetHUD)) _output_get))

(event EventOnGameStateReplicated
  (|CallParentFunction)
  (Utilities|FlowControl|Sequence
    (:then_0
      (bind _returnvalue (UserInterface|CreateWidget "/Game/Mordhau/Blueprints/GameModes/Duel/BP_DuelHUDWidget.BP_DuelHUDWidget_C" (Game|GetPlayerController 0)))
      (bind _output_get (Variables|Default|SetDuelHUDWidget _returnvalue))
      (UserInterface|Viewport|AddtoViewport _output_get -5)
      (if (Variables|Default|GetIsHUDMinimal)
        (Widget|SetVisibility _output_get "Collapsed")))
    (:then_1
      (bind _bisvisible (CallFunction|IsMainMenuVisible))
      (if (not _bisvisible)
        (CallFunction|ShowMainMenu "NewEnumerator0")))))

(event EventHideMainMenu
  (bind _returnvalue (Game|GetPlayerController 0))
  (bind _duelendscreen (Variables|Default|GetDuelEndScreen))
  (|CallParentFunction)
  (Widget|SetVisibility (Variables|Default|GetDuelHUDWidget) "Visible")
  (if (Widget|IsVisible _duelendscreen)
    (Variables|/Script/Engine.PlayerController|SetbShowMouseCursor _returnvalue true)
    (Input|SetInputModeUIOnly _returnvalue _duelendscreen "DoNotLock")))

(event EventShowMainMenu
  (params (Armory%20State :type E_ArmoryStates%20Enum :default "NewEnumerator0"))
  (|CallParentFunction Armory%20State)
  (Widget|SetVisibility (Variables|Default|GetDuelHUDWidget) "Collapsed"))

(event EventUseMinimalHUD
  (|CallParentFunction)
  (Utilities|IsValid (Variables|Default|GetDuelHUDWidget)
    (:Is%20Valid
      (Widget|SetVisibility (Variables|Default|GetDuelHUDWidget) "Collapsed"))))

(event EventUseFullHUD
  (|CallParentFunction)
  (Utilities|IsValid (Variables|Default|GetDuelHUDWidget)
    (:Is%20Valid
      (Widget|SetVisibility (Variables|Default|GetDuelHUDWidget) "Visible"))))

(fn ConstructionScript
  (|CallParentFunction))

(fn ShowDuelEndScreen
  (Default|Show (Variables|Default|GetDuelEndScreen)))