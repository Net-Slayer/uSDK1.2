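; Duel game mode that hosts many instanced rooms on one server, pairing players by matchmaking lobby ID.
; New logins queue until their ID is valid, then join a room and its shared controller instance list.
; Tick drives each room's round state machine and copies it to its controllers.
; Wins or departures finish games, awarding MMR and reward drops; an expired map timer blocks joins and ends the match once empty.
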(event EventBeginPlay
  (|CallParentFunction) ; This node is disabled and will not be called.\nDrag off pins to build functionality.
)

(event EventTick
  (params (DeltaSeconds :type Float%20%28single-precision%29))
  (|CallParentFunction DeltaSeconds)
  (if (Class|GameMode|IsMatchinProgress)
    (Utilities|FlowControl|Sequence
      (:then_0
        (CallFunction|HandleUnhandledPlayers))
      (:then_1
        ;[1 1 1] Rooms can be deleted, in this case some rooms can be skipped this tick due to index reordering. This is generally harmless, given that we don't rely on ticking every frame.
        (for _index (range 0 (- (Utilities|Array|Length (Variables|Default|GetRooms)) 1))
          (CallFunction|TickRoom _index)))
      (:then_2
        (bind _output_get (Variables|Default|SetTimeUntilMapChange (- (Variables|Default|GetTimeUntilMapChange) DeltaSeconds)))
        (if (< _output_get 0.0)
          (Utilities|FlowControl|Sequence
            (:then_0
              (if (stale _returnvalue)
                (Class|MordhauGameSession|AllowJoin (Class|MordhauUtilityLibrary|GetMordhauGameSession) false)))
            (:then_1
              (bind _returnvalue (Class|GameModeBase|GetNumPlayers))
              (if (== _returnvalue 0)
                (Class|GameMode|EndMatch)))))))))

(event EventRequestedAssignTeam
  (params (Controller :type Controller%20Object%20Reference) (Team :type Integer)))

(event EventPostLogin
  (params (NewPlayer :type Player%20Controller%20Object%20Reference))
  (Utilities|FlowControl|Sequence
    (:then_0
      (|CallParentFunction NewPlayer))
    (:then_1
      (bind _asmordhau_player_controller (Utilities|Casting|CastToMordhauPlayerController NewPlayer))
      (Utilities|Array|Add (Variables|Default|GetUnhandledControllers) _asmordhau_player_controller))))

(event EventOnLogout
  (params (ExitingController :type Controller%20Object%20Reference))
  (Utilities|FlowControl|Sequence
    (:then_0
      (bind _asmordhau_player_controller (Utilities|Casting|CastToMordhauPlayerController ExitingController))
      (CallFunction|HandlePlayerLeaving _asmordhau_player_controller))
    (:then_1
      (|CallParentFunction ExitingController))))

(fn ConstructionScript
  (|CallParentFunction))

(fn HandleNewPlayer
  (params (NewPlayer :type Mordhau%20Player%20Controller%20Object%20Reference))
  (bind _asmordhau_player_state (Utilities|Casting|CastToMordhauPlayerState (Variables|/Script/Engine.Controller|GetPlayerState NewPlayer)))
  (bind (_array_element _array_index) (Utilities|Array|ForEachLoopwithBreak (Variables|Default|GetRooms) :!label _label)
    (:LoopBody
      (if (Math|Boolean|ANDBoolean (> (Utilities|Array|Length (.Controllers (Utilities|Struct|BreakST_DuelRoom _array_element))) 0) (< (Utilities|Array|Length (.Controllers (Utilities|Struct|BreakST_DuelRoom _array_element))) (Variables|Default|GetMaxPeoplePerRoom)) (Utilities|Enum|Equal(Enum) (.RoomState (Utilities|Struct|BreakST_DuelRoom _array_element)) "NewEnumerator0"))
        (if (or (Utilities|Enum|Equal(Enum) (Class|MordhauUtilityLibrary|SteamIDtoString (Variables|/Script/Mordhau.MordhauPlayerController|GetMatchmakingLobbyID (Utilities|Array|Get(acopy) (.Controllers (Utilities|Struct|BreakST_DuelRoom _array_element))))) (Class|MordhauUtilityLibrary|SteamIDtoString (Variables|/Script/Mordhau.MordhauPlayerController|GetMatchmakingLobbyID NewPlayer))) (Class|MordhauUtilityLibrary|IsPlayinEditor))
          (LocalVariables|SetRoomIdx _array_index)
          (goto _label Break))))
    (:Completed
      (Variables|/Script/Mordhau.MordhauPlayerState|SetTeam _asmordhau_player_state 0)
      (if (== (LocalVariables|GetRoomIdx) -1)
        (bind _returnvalue (Utilities|Array|Add (Variables|Default|GetRooms) (Utilities|Struct|MakeST_DuelRoom (Utilities|Array|MakeArray NewPlayer) (Utilities|Struct|MakeST_DuelRoomGame 0 0 (Utilities|Struct|MakeSTRUCT_DuelRoundInfo "NewEnumerator0" 0 (+ (Utilities|Time|GetTimeSeconds) 9e+01))))))
        (LocalVariables|SetRoomIdx _returnvalue)
        (else
          (for _array_element_2 (.Controllers (Utilities|Struct|BreakST_DuelRoom (Utilities|Array|Get(acopy) (Variables|Default|GetRooms) (LocalVariables|GetRoomIdx))))
            ;[1 1 1] Crude team assignment, only works for 1v1 (first free team set)
            (bind _asmordhau_player_state_2 (Utilities|Casting|CastToMordhauPlayerState (Variables|/Script/Engine.Controller|GetPlayerState _array_element_2)))
            (if (== (Variables|/Script/Mordhau.MordhauPlayerState|GetTeam _asmordhau_player_state_2) 0)
              (Variables|/Script/Mordhau.MordhauPlayerState|SetTeam _asmordhau_player_state 1)))
          (CallFunction|AddControllertoRoom NewPlayer (LocalVariables|GetRoomIdx))
          (if (CallFunction|IsRoomReadytoStart (LocalVariables|GetRoomIdx))
            (CallFunction|PrepareandStartRoom (LocalVariables|GetRoomIdx))))))))

(fn SetRoomGame
  (params (RoomIndex :type Integer) (NewGame :type ST%20Duel%20Room%20Game%20Structure%20%28by%20ref%29))
  (Utilities|Struct|SetmembersinST_DuelRoom (Utilities|Array|Get(acopy) (Variables|Default|GetRooms) RoomIndex) NewGame))

(fn SetRoomGameRound
  (params (RoomIndex :type Integer) (NewRound :type STRUCT%20Duel%20Round%20Info%20Structure%20%28by%20ref%29))
  (bind _rooms (Variables|Default|GetRooms))
  (bind _output (Utilities|Array|Get(acopy) _rooms RoomIndex))
  (bind _game (Utilities|Struct|BreakST_DuelRoom _output))
  (bind (_team1wins _team2wins) (Utilities|Struct|BreakST_DuelRoomGame _game))
  (CallFunction|SetRoomGame RoomIndex (Utilities|Struct|MakeST_DuelRoomGame _team1wins _team2wins NewRound)))

(fn FinishRoomGame
  (params (RoomIndex :type Integer) (Winner :type Byte))
  (bind _returnvalue (Class|MordhauUtilityLibrary|GetMordhauGameSession))
  (CallFunction|SetRoomTerminated RoomIndex)
  (for _array_element (.Controllers (Utilities|Struct|BreakST_DuelRoom (Utilities|Array|Get(acopy) (Variables|Default|GetRooms) RoomIndex)))
    (bind _asbp_duel_player_controller (Utilities|Casting|CastToBP_DuelPlayerController _array_element))
    (bind _asmordhau_player_state (Utilities|Casting|CastToMordhauPlayerState (Variables|/Script/Engine.Controller|GetPlayerState _array_element)))
    (if (== Winner (Math|Conversions|ToByte(Integer) (Variables|/Script/Mordhau.MordhauPlayerState|GetTeam _asmordhau_player_state)))
      (LocalVariables|SetWinnerID (Class|MordhauPlayerState|GetSteamID _asmordhau_player_state))
      (LocalVariables|SetWinnerPlayerController _asbp_duel_player_controller)
      (Class|MordhauPlayerState|AddScore _asmordhau_player_state 10000) ; 1st place
      (else
        (LocalVariables|SetLoserID (Class|MordhauPlayerState|GetSteamID _asmordhau_player_state))
        (LocalVariables|SetLoserPlayerController _asbp_duel_player_controller)
        (Class|MordhauPlayerState|AddScore _asmordhau_player_state 20000) ; 2nd place
      )))
  (Utilities|IsValid (LocalVariables|GetWinnerPlayerController)
    (:Is%20Valid
      (Utilities|IsValid (LocalVariables|GetLoserPlayerController)
        (:Is%20Valid
          (Variables|/Game/Mordhau/Blueprints/GameModes/Duel/BP_DuelPlayerController.BP_DuelPlayerController_C|SetNewMMR (LocalVariables|GetWinnerPlayerController) (.NewWinnerMMR (Class|MordhauUtilityLibrary|AwardDuelMMR (LocalVariables|GetWinnerID) (LocalVariables|GetLoserID))))
          (Variables|/Game/Mordhau/Blueprints/GameModes/Duel/BP_DuelPlayerController.BP_DuelPlayerController_C|SetNewMMR (LocalVariables|GetLoserPlayerController) (.NewLoserMMR (Class|MordhauUtilityLibrary|AwardDuelMMR (LocalVariables|GetWinnerID) (LocalVariables|GetLoserID))))
          (Class|MordhauGameSession|TriggerRewardDropforPlayer _returnvalue (LocalVariables|GetWinnerPlayerController))
          (Class|MordhauGameSession|TriggerRewardDropforPlayer _returnvalue (LocalVariables|GetLoserPlayerController)))))))

(fn PrepareandStartRoom
  (params (RoomIndex :type Integer))
  (Utilities|Struct|SetmembersinST_DuelRoom (Utilities|Array|Get(acopy) (Variables|Default|GetRooms) RoomIndex) 1000 1000 "NewEnumerator1")
  (CallFunction|SetRoomGameRound RoomIndex (Utilities|Struct|MakeSTRUCT_DuelRoundInfo "NewEnumerator4" 0 (+ (Utilities|Time|GetTimeSeconds) 12.0))))

(fn IsRoomReadytoStart
  (params (RoomIndex :type Integer))
  (return (== (Utilities|Array|Length (.Controllers (Utilities|Struct|BreakST_DuelRoom (Utilities|Array|Get(acopy) (Variables|Default|GetRooms) RoomIndex)))) (Variables|Default|GetMaxPeoplePerRoom))))

(fn TickRoom
  (params (RoomIndex :type Integer))
  (bind _returnvalue (Utilities|Time|GetTimeSeconds))
  (bind _rooms (Variables|Default|GetRooms))
  (bind _roundstowin (Variables|Default|GetRoundsToWin))
  (bind _team1living (LocalVariables|GetTeam1Living))
  (bind _team2living (LocalVariables|GetTeam2Living))
  (bind _output (Utilities|Array|Get(acopy) _rooms RoomIndex))
  (bind (_controllers _game) (Utilities|Struct|BreakST_DuelRoom _output))
  (bind (_team1wins _team2wins _roundinfo) (Utilities|Struct|BreakST_DuelRoomGame _game))
  (bind (_stage _winner _starttime) (Utilities|Struct|BreakSTRUCT_DuelRoundInfo _roundinfo))
  (bind _returnvalue_2 (< _starttime _returnvalue))
  (Utilities|FlowControl|Sequence
    (:then_0
      (switch Utilities|FlowControl|Switch|SwitchonE_DuelRoundStage _stage
        (:NewEnumerator0
          (if _returnvalue_2
            (CallFunction|DestroyRoom RoomIndex true)
            (return)))
        (:NewEnumerator4
          (if _returnvalue_2
            (CallFunction|RestartRoom RoomIndex)))
        (:NewEnumerator1
          (if _returnvalue_2
            (CallFunction|SetRoomGameRound RoomIndex (Utilities|Struct|MakeSTRUCT_DuelRoundInfo "NewEnumerator2" 0 0.0))))
        (:NewEnumerator2
          (for _array_element _controllers
            (bind _asmordhau_player_state (Utilities|Casting|CastToMordhauPlayerState (Variables|/Script/Engine.Controller|GetPlayerState _array_element)))
            (if (== (Variables|/Script/Mordhau.MordhauPlayerState|GetTeam _asmordhau_player_state) 0)
              (Math|Integer|IncrementInt (LocalVariables|GetTeam1Total)
                (:%20%20
                  (if (Variables|/Script/Mordhau.MordhauPlayerState|GetbIsAlive _asmordhau_player_state)
                    (Math|Integer|IncrementInt (LocalVariables|GetTeam1Living)))))
              (else
                (Math|Integer|IncrementInt (LocalVariables|GetTeam2Total)
                  (:%20%20
                    (if (Variables|/Script/Mordhau.MordhauPlayerState|GetbIsAlive _asmordhau_player_state)
                      (Math|Integer|IncrementInt (LocalVariables|GetTeam2Living))))))))
          (if (or (== _team1living 0) (== _team2living 0))
            (CallFunction|AwardRoundWin RoomIndex (Math|Integer|SelectInt 0 1 (> _team1living _team2living)) (or (== (LocalVariables|GetTeam1Total) 0) (== (LocalVariables|GetTeam2Total) 0)))))
        (:NewEnumerator3
          (if (and (not (or (== _team1wins _roundstowin) (== _team2wins _roundstowin))) _returnvalue_2)
            (CallFunction|RestartRoom RoomIndex)))))
    (:then_1
      (for _array_element_2 _controllers
        (bind _asbp_duel_player_controller (Utilities|Casting|CastToBP_DuelPlayerController _array_element_2))
        (Variables|/Game/Mordhau/Blueprints/GameModes/Duel/BP_DuelPlayerController.BP_DuelPlayerController_C|SetReplicatedRoomGame _asbp_duel_player_controller _game))
      (if (or (== _team1wins (Variables|Default|GetRoundsToWin)) (== _team2wins (Variables|Default|GetRoundsToWin)))
        (CallFunction|DestroyRoom RoomIndex false)))))

(fn AwardRoundWin
  (params (RoomIndex :type Integer) (Winner :type Integer) (GrantAllWins :type Boolean))
  (bind _rooms (Variables|Default|GetRooms))
  (bind _roundstowin (Variables|Default|GetRoundsToWin))
  (bind _roundstowin_2 (Variables|Default|GetRoundsToWin))
  (bind _rooms_2 (Variables|Default|GetRooms))
  (bind _output (Utilities|Array|Get(acopy) _rooms RoomIndex))
  (bind _output_2 (Utilities|Array|Get(acopy) _rooms_2 RoomIndex))
  (bind _game (Utilities|Struct|BreakST_DuelRoom _output))
  (bind _game_2 (Utilities|Struct|BreakST_DuelRoom _output_2))
  (bind (_team1wins _team2wins) (Utilities|Struct|BreakST_DuelRoomGame _game))
  (bind (_team1wins_2 _team2wins_2) (Utilities|Struct|BreakST_DuelRoomGame _game_2))
  (bind _returnvalue (== _team1wins _roundstowin))
  (LocalVariables|SetNewTeam1Wins (+ _team1wins_2 (Utilities|Select :Index Winner :Option%200 1 :Option%201 0)))
  (LocalVariables|SetNewTeam2Wins (+ _team2wins_2 (Utilities|Select :Index Winner :Option%200 0 :Option%201 1)))
  (Utilities|FlowControl|Sequence
    (:then_0
      (if GrantAllWins
        (if (== Winner 0)
          (LocalVariables|SetNewTeam1Wins _roundstowin_2)
          (else
            (LocalVariables|SetNewTeam2Wins _roundstowin_2)))))
    (:then_1
      (CallFunction|SetRoomGame RoomIndex (Utilities|Struct|MakeST_DuelRoomGame (LocalVariables|GetNewTeam1Wins) (LocalVariables|GetNewTeam2Wins) (Utilities|Struct|MakeSTRUCT_DuelRoundInfo "NewEnumerator3" (Math|Conversions|ToByte(Integer) Winner) (+ (Utilities|Time|GetTimeSeconds) 2.0))))
      (if (or _returnvalue (== _team2wins (Variables|Default|GetRoundsToWin)))
        (CallFunction|FinishRoomGame RoomIndex (Math|Conversions|ToByte(Integer) (Math|Integer|SelectInt 0 1 _returnvalue)))))))

(fn RestartRoom
  (params (RoomIndex :type Integer))
  (Utilities|FlowControl|Sequence
    (:then_0
      (bind _outactors (Actor|GetAllActorsOfClass "/Script/Mordhau.MordhauActor"))
      (for _array_element _outactors
        (if (stale _returnvalue)
          (Actor|DestroyActor _array_element))))
    (:then_1
      (for _array_element_2 (.Controllers (Utilities|Struct|BreakST_DuelRoom (Utilities|Array|Get(acopy) (Variables|Default|GetRooms) RoomIndex)))
        (CallFunction|UnpossessandDestroyPawn _array_element_2 true)))
    (:then_2
      (CallFunction|SetRoomGameRound RoomIndex (Utilities|Struct|MakeSTRUCT_DuelRoundInfo "NewEnumerator1" 0 (+ (Utilities|Time|GetTimeSeconds) 3.0))))))

(fn DestroyRoom
  (params (RoomIndex :type Integer) (KickPlayers :type Boolean))
  (bind _rooms (Variables|Default|GetRooms))
  (CallFunction|SetRoomTerminated RoomIndex)
  (Utilities|FlowControl|Sequence
    (:then_0
      (if KickPlayers
        (for _array_element (.Controllers (Utilities|Struct|BreakST_DuelRoom (Utilities|Array|Get(acopy) _rooms RoomIndex)))
          (Class|MordhauGameSession|KickPlayer (Class|MordhauUtilityLibrary|GetMordhauGameSession) _array_element (Utilities|Text|MakeLiteralText "Match ended")))))
    (:then_1
      (Utilities|Array|RemoveIndex _rooms RoomIndex))))

(fn HandlePlayerLeaving
  (params (Player :type Mordhau%20Player%20Controller%20Object%20Reference))
  (Utilities|Array|RemoveItem (Variables|Default|GetUnhandledControllers) Player)
  (bind _asmordhau_player_state (Utilities|Casting|CastToMordhauPlayerState (Variables|/Script/Engine.Controller|GetPlayerState Player)))
  (bind (_array_element _array_index) (Utilities|Array|ForEachLoopwithBreak (Variables|Default|GetRooms) :!label _label)
    (:LoopBody
      (if (and (Utilities|Array|ContainsItem (.Controllers (Utilities|Struct|BreakST_DuelRoom _array_element)) Player) (Utilities|Enum|NotEqual(Enum) (.RoomState (Utilities|Struct|BreakST_DuelRoom _array_element)) "NewEnumerator2"))
        (LocalVariables|SetFoundRoomIdx _array_index)
        (goto _label Break)))
    (:Completed
      (if (!= (LocalVariables|GetFoundRoomIdx) -1)
        (if (Utilities|Enum|Equal(Enum) (.RoomState (Utilities|Struct|BreakST_DuelRoom _array_element)) "NewEnumerator1")
          (CallFunction|FinishRoomGame (LocalVariables|GetFoundRoomIdx) (Utilities|Select :Index (Variables|/Script/Mordhau.MordhauPlayerState|GetTeam _asmordhau_player_state) :Option%200 1 :Option%201 0))
          (elif (Utilities|Enum|Equal(Enum) (.RoomState (Utilities|Struct|BreakST_DuelRoom _array_element)) "NewEnumerator0")
            (CallFunction|DestroyRoom (LocalVariables|GetFoundRoomIdx) true)))))))

(fn AddControllertoRoom
  (params (NewController :type Mordhau%20Player%20Controller%20Object%20Reference) (RoomIndex :type Integer))
  (bind _rooms (Variables|Default|GetRooms))
  (bind _output (Utilities|Array|Get(acopy) _rooms RoomIndex))
  (bind (_controllers _game _team1mmr _team2mmr _roomstate) (Utilities|Struct|BreakST_DuelRoom _output))
  (bind _output_get (LocalVariables|SetNewArray _controllers))
  (for _array_element _output_get
    (Utilities|Set|Add (Variables|/Script/Mordhau.MordhauPlayerController|GetInInstanceWithControllers NewController) _array_element)
    (Utilities|Set|Add (Variables|/Script/Mordhau.MordhauPlayerController|GetInInstanceWithControllers _array_element) NewController))
  (Utilities|Array|Add (LocalVariables|GetNewArray) NewController)
  (Utilities|Array|SetArrayElem _rooms RoomIndex (Utilities|Struct|MakeST_DuelRoom (LocalVariables|GetNewArray) _game _team1mmr _team2mmr _roomstate)))

(fn HandleUnhandledPlayers
  (bind _unhandledcontrollers (Variables|Default|GetUnhandledControllers))
  (for _array_element _unhandledcontrollers
    (if (or (Class|MordhauUtilityLibrary|IsValidSteamID (Variables|/Script/Mordhau.MordhauPlayerController|GetMatchmakingLobbyID _array_element)) (Class|MordhauUtilityLibrary|IsPlayinEditor))
      (CallFunction|HandleNewPlayer _array_element)
      (Class|MordhauUtilityLibrary|ResetController _array_element)
      (Utilities|Array|Add (LocalVariables|GetToRemove) _array_element)))
  (for _array_element_2 (LocalVariables|GetToRemove)
    (Utilities|Array|RemoveItem _unhandledcontrollers _array_element_2)))

(fn SetRoomTerminated
  (params (Index :type Integer))
  (bind _rooms (Variables|Default|GetRooms))
  (bind _output (Utilities|Array|Get(acopy) _rooms Index))
  (bind (_controllers _game _team1mmr _team2mmr) (Utilities|Struct|BreakST_DuelRoom _output))
  (Utilities|Array|SetArrayElem _rooms Index (Utilities|Struct|MakeST_DuelRoom _controllers _game _team1mmr _team2mmr "NewEnumerator2")))