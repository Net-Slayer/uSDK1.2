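; Battle Royale spawn manager that randomly distributes a configured count of each spawner type across the level's BP_BattleRoyaleSpawnPoint actors.
; For each key in SpawnerCounts, ActivateSpawns gathers valid points that allow that spawner, then picks random ones to assign and activate until the count is met or candidates run out.
; Chosen points activate and destroy themselves; afterwards any remaining points and the manager itself are destroyed.
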(fn ConstructionScript)

(fn ActivateSpawns
  (bind _currentlist (LocalVariables|GetCurrentList))
  (bind _returnvalue (Utilities|Array|Length _currentlist))
  (bind _keys (Utilities|Map|Keys (Variables|Default|GetSpawnerCounts)))
  (bind _outactors (Actor|GetAllActorsOfClass "/Game/Mordhau/Blueprints/GameModes/BattleRoyale/BP_BattleRoyaleSpawnPoint.BP_BattleRoyaleSpawnPoint_C"))
  (for _array_element _keys
    (Utilities|Array|Clear (LocalVariables|GetCurrentList))
    (for _array_element_2 _outactors
      (Utilities|IsValid _array_element_2
        (:Is%20Valid
          (if (Utilities|Set|Contains (Variables|/Game/Mordhau/Blueprints/GameModes/BattleRoyale/BP_BattleRoyaleSpawnPoint.BP_BattleRoyaleSpawnPoint_C|GetAllowedSpawners _array_element_2) _array_element)
            (Utilities|Array|Add _currentlist _array_element_2)))))
    (Utilities|FlowControl|ForLoopwithBreak 0 (- (.Value (Utilities|Map|Find (Variables|Default|GetSpawnerCounts) _array_element)) 1) :!label _label
      (:LoopBody
        (if (== _returnvalue 0)
          (goto _label Break)
          (else
            (bind _output_get (LocalVariables|SetCurrentChoice (Math|Random|RandomInteger _returnvalue)))
            (Variables|/Game/Mordhau/Blueprints/GameModes/BattleRoyale/BP_BattleRoyaleSpawnPoint.BP_BattleRoyaleSpawnPoint_C|SetAssignedSpawner (Utilities|Array|Get(acopy) _currentlist _output_get) _array_element)
            (Default|ActivateandDestroy (Utilities|Array|Get(acopy) _currentlist _output_get))
            (Utilities|Array|RemoveIndex _currentlist _output_get))))))
  (for _array_element_3 _outactors
    (Utilities|IsValid _array_element_3
      (:Is%20Valid
        (Actor|DestroyActor _array_element_3))))
  (Actor|DestroyActor))