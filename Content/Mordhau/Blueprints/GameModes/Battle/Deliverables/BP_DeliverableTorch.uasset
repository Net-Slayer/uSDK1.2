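; Torch deliverable for the Battle game mode whose flame and sound react to how it moves.
; Each tick, the particle system's per-frame displacement raises the FireWind volume and smoothly tilts the flame through a clamped pitch and roll lerp.
; This movement is not scaled by delta time, so the effect varies with frame rate.
; When the torch thuds, its particle system deactivates.
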(event EventBeginPlay
  (|CallParentFunction) ; This node is disabled and will not be called.\nDrag off pins to build functionality.
)

(event Collision|EventActorBeginOverlap
  (params (OtherActor :type Actor%20Object%20Reference))
  (|CallParentFunction OtherActor) ; This node is disabled and will not be called.\nDrag off pins to build functionality.
)

(event EventTick
  (params (DeltaSeconds :type Float%20%28single-precision%29))
  (bind _particlesystem (Variables|Default|GetParticleSystem))
  (bind _particlesystem_2 (Variables|Default|GetParticleSystem))
  (bind _returnvalue (Transformation|GetWorldLocation _particlesystem_2))
  (|CallParentFunction DeltaSeconds)
  (Audio|Components|Audio|SetVolumeMultiplier (Variables|Default|GetFireWind) (+ (* (Math|Vector|VectorLength (- _returnvalue (Variables|Default|GetLastActorLocation))) 0.08) 0.3) :!class /Script/Engine.AudioComponent)
  (Transformation|SetWorldRotation _particlesystem (Math|Rotator|Lerp(Rotator) (Transformation|GetWorldRotation _particlesystem) (Math|Rotator|MakeRotator (Math|Float|Clamp(Float) (* (.Y (Math|Vector|BreakVector (- _returnvalue (Variables|Default|GetLastActorLocation)))) -8.0) -7e+01 7e+01) (Math|Float|Clamp(Float) (* (.X (Math|Vector|BreakVector (- _returnvalue (Variables|Default|GetLastActorLocation)))) 8.0) -7e+01 7e+01) 0.0) 0.3) false false)
  (Variables|Default|SetLastActorLocation _returnvalue))

(event EventOnThud
  (bind _particlesystem (Variables|Default|GetParticleSystem))
  (|CallParentFunction)
  (Utilities|IsValid _particlesystem
    (:Is%20Valid
      (Components|Activation|Deactivate _particlesystem))))

(fn ConstructionScript
  (|CallParentFunction))