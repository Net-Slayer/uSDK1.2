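; BP_TrebRockDelivery is a Battle mode delivery spot that shows trebuchet rocks piling up as deliverables come in.
; When deliverables change, it scales Progress into four stages.
; Each stage past its threshold unhides a pair of static meshes and enables their collision, ending with the top pair.
; Nothing here hides meshes again, so the pile only grows.
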(event EventBeginPlay)

(event Collision|EventActorBeginOverlap
  (params (OtherActor :type Actor%20Object%20Reference))
  (|CallParentFunction OtherActor) ; This node is disabled and will not be called.\nDrag off pins to build functionality.
)

(event EventTick
  (params (DeltaSeconds :type Float%20%28single-precision%29))
  (|CallParentFunction DeltaSeconds) ; This node is disabled and will not be called.\nDrag off pins to build functionality.
)

(event EventOnDeliverablesChanged
  (bind _staticmesh6 (Variables|Default|GetStaticMesh6))
  (bind _progress (Variables|Default|GetProgress))
  (bind _returnvalue (* _progress 4.0))
  (|CallParentFunction)
  (Utilities|FlowControl|Sequence
    (:then_0
      (if (> _returnvalue 0.0)
        (Development|SetHiddeninGame _staticmesh6 false false)
        (Collision|SetCollisionEnabled _staticmesh6 "QueryAndPhysics")))
    (:then_1
      (if (> _returnvalue 1.0)
        (Development|SetHiddeninGame (Variables|Default|GetStaticMesh3) false false)
        (Collision|SetCollisionEnabled (Variables|Default|GetStaticMesh4) "QueryAndPhysics")))
    (:then_2
      (if (> _returnvalue 2.0)
        (Development|SetHiddeninGame (Variables|Default|GetStaticMesh5) false false)
        (Collision|SetCollisionEnabled (Variables|Default|GetStaticMesh1) "QueryAndPhysics")))
    (:then_3
      (if (> _returnvalue 3.0)
        (Development|SetHiddeninGame (Variables|Default|GetStaticMeshTop2) false false)
        (Collision|SetCollisionEnabled (Variables|Default|GetStaticMeshTop1) "QueryAndPhysics")))))

(fn ConstructionScript
  (|CallParentFunction))