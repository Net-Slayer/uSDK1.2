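; Game state for Frontline and its Push variant, tracking tickets, capture-point control and match results.
; On the server, Frontline periodically drains the team holding fewer points, or both when tied, declaring a draw if both empty.
; Push instead times the attackers using BP_PushModeInfo settings; a team left without points has its score zeroed, after a delay in Push.
; Client-side, it shows objectives, victory/defeat/draw screens and refreshes capture-point widgets on team change.
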(event Custom|TriggerWinDelayed
  (Variables|Default|SetAllObjectivesCompletedTime (Utilities|Time|GetTimeSeconds))
  (Utilities|FlowControl|Delay (Variables|Default|GetPushWinDelay))
  (bind _asbp_frontline_game_mode (Utilities|Casting|CastToBP_FrontlineGameMode (Game|GetGameMode)))
  (if (Class|GameMode|IsMatchinProgress _asbp_frontline_game_mode)
    (if (== (Variables|Default|GetTeam2CapturePoints) 0)
      ;[1 1 1] team 2 has no points, team 1 wins.
      (Class|MordhauGameMode|SetTeamScore (stale EventTick _asbp_mordhau_game_mode) 1 0.0)
      (else
        ;[1 1 1] team 1 has no points, team 2 wins.
        (Class|MordhauGameMode|SetTeamScore (stale EventTick _asbp_mordhau_game_mode) 0 0.0)))))

(event EventHandleMatchEndInfo
  (bind _matchendinfo (Variables|Default|GetMatchEndInfo))
  (bind (_winner _winnerteam _winnerscore _otherscore _draw) (Utilities|Struct|BreakSTRUCT_MatchEndInfo _matchendinfo))
  (|CallParentFunction)
  (bind _asbp_mordhau_hud (Utilities|Casting|CastToBP_MordhauHUD (Class|MordhauUtilityLibrary|GetMordhauHUD)))
  (bind _asmordhau_player_state (Utilities|Casting|CastToMordhauPlayerState (Variables|/Script/Engine.Controller|GetPlayerState (Game|GetPlayerController 0))))
  (if _draw
    (Default|ShowMatchResult _asbp_mordhau_hud false "draw")
    (elif (or (== (Variables|/Script/Mordhau.MordhauPlayerState|GetTeam _asmordhau_player_state) _winnerteam) (== (Variables|/Script/Mordhau.MordhauPlayerState|GetTeam _asmordhau_player_state) -1))
      (Default|ShowMatchResult _asbp_mordhau_hud true "victory")
      (else
        (Default|ShowMatchResult _asbp_mordhau_hud false "defeat")))))

(event EventLocalPlayerChangedTeam
  (|CallParentFunction)
  (for _array_element (Variables|Default|GetAllCapturePoints)
    (Class|ControlPoint|UpdateUIWidgets _array_element)))

(event EventBeginPlay
  (bind _teamscores (Variables|Default|GetTeamScores))
  (Utilities|FlowControl|Sequence
    (:then_0
      (Networking|SwitchHasAuthority
        (:Authority
          (Utilities|Array|SetArrayElem _teamscores 0 (Variables|Default|GetTeam1StartingTickets))
          (Utilities|Array|SetArrayElem _teamscores 1 (Variables|Default|GetTeam2StartingTickets)))))
    (:then_1
      (bind _outactors (Actor|GetAllActorsOfClass "/Game/Mordhau/Blueprints/GameModes/Push/BP_PushModeInfo.BP_PushModeInfo_C"))
      (if (> (Utilities|Array|Length _outactors) 0)
        (bind _output_get (Variables|Default|SetAttackingTeam (Variables|/Game/Mordhau/Blueprints/GameModes/Push/BP_PushModeInfo.BP_PushModeInfo_C|GetAttackingTeam (Utilities|Array|Get(acopy) _outactors))))
        (Variables|Default|SetDefendingTeam (Utilities|Select :Index _output_get :Option%200 1 :Option%201 0))
        (Variables|Default|SetInitialStageTime (Variables|/Game/Mordhau/Blueprints/GameModes/Push/BP_PushModeInfo.BP_PushModeInfo_C|GetInitialTime (Utilities|Array|Get(acopy) _outactors)))
        (Variables|Default|SetPushTopologicalProgressAttackingTeam _output_get)))))

(event EventTick
  (params (DeltaSeconds :type Float%20%28single-precision%29))
  (bind _team2capturepoints (Variables|Default|GetTeam2CapturePoints))
  (bind _returnvalue (== _team2capturepoints 0))
  (|CallParentFunction DeltaSeconds)
  (Utilities|FlowControl|Sequence
    (:then_0
      (Networking|CanExecuteCosmeticEvents
        (:True
          (if (Class|GameStateBase|HasMatchStarted)
            (Utilities|FlowControl|DoOnce false
              (:Completed
                (bind _asbp_frontline_player_controller (Utilities|Casting|CastToBP_FrontlinePlayerController (Game|GetPlayerController 0)))
                (bind _asbp_frontline_hud (Utilities|Casting|CastToBP_FrontlineHUD (Class|MordhauUtilityLibrary|GetMordhauHUD)))
                (Default|ShowObjectives _asbp_frontline_hud)
                (bind _asbp_push_player_controller (Utilities|Casting|CastToBP_PushPlayerController _asbp_frontline_player_controller))
                (Default|ShowCurrentObjective _asbp_push_player_controller true)))))))
    (:then_1
      (Networking|SwitchHasAuthority
        (:Authority
          (bind _asbp_mordhau_game_mode (Utilities|Casting|CastToBP_MordhauGameMode (Game|GetGameMode)))
          (if (Class|GameMode|IsMatchinProgress _asbp_mordhau_game_mode)
            (if (or (== (Variables|Default|GetTeam1CapturePoints) 0) _returnvalue)
              (if (Variables|Default|GetIsPushMode)
                (CallFunction|TriggerWinDelayed)
                (elif _returnvalue
                  ;[1 1 1] team 2 has no points, team 1 wins.
                  (Class|MordhauGameMode|SetTeamScore _asbp_mordhau_game_mode 1 0.0)
                  (else
                    ;[1 1 1] team 1 has no points, team 2 wins.
                    (Class|MordhauGameMode|SetTeamScore _asbp_mordhau_game_mode 0 0.0))))
              (elif (Variables|Default|GetIsPushMode)
                (Utilities|FlowControl|Sequence
                  (:then_0
                    ;[1 1 1] Time mode
                    (Utilities|FlowControl|DoOnce false
                      (:Completed
                        (Variables|Default|SetStageEndTime (+ (Utilities|Time|GetTimeSeconds) (Variables|Default|GetInitialStageTime))))))
                  (:then_1
                    (if (< (Variables|Default|GetStageEndTime) (Utilities|Time|GetTimeSeconds))
                      (Class|MordhauGameMode|SetTeamScore _asbp_mordhau_game_mode (Math|Conversions|ToInteger(Byte) (Variables|Default|GetAttackingTeam)) 0.0))))
                (else
                  ;[1 1 1] Ticket mode
                  (Variables|Default|SetTicketDrainCounter (+ DeltaSeconds (Variables|Default|GetTicketDrainCounter)))
                  (if (>= (Variables|Default|GetTicketDrainCounter) (Variables|Default|GetTicketDrainInterval))
                    (Variables|Default|SetTicketDrainCounter (- (Variables|Default|GetTicketDrainCounter) (Variables|Default|GetTicketDrainInterval)))
                    (CallFunction|DrainTickets _asbp_mordhau_game_mode)))))))))))

(fn ConstructionScript
  (|CallParentFunction))

(fn DrainTickets
  (params (GameMode :type BP%20Mordhau%20Game%20Mode%20Object%20Reference))
  (bind _teamscores (Variables|Default|GetTeamScores))
  (bind _team1capturepoints (Variables|Default|GetTeam1CapturePoints))
  (bind _team2capturepoints (Variables|Default|GetTeam2CapturePoints))
  (bind _ticketdrainamount (Variables|Default|GetTicketDrainAmount))
  (Utilities|FlowControl|Sequence
    (:then_0
      (LocalVariables|SetTeam1Score (Utilities|Array|Get(acopy) _teamscores))
      (LocalVariables|SetTeam2Score (Utilities|Array|Get(acopy) _teamscores 1))
      (if (> _team1capturepoints _team2capturepoints)
        (LocalVariables|SetTeam2Score (- (LocalVariables|GetTeam2Score) _ticketdrainamount))
        (elif (> _team2capturepoints _team1capturepoints)
          (LocalVariables|SetTeam1Score (- (LocalVariables|GetTeam1Score) _ticketdrainamount))
          (else
            (LocalVariables|SetTeam1Score (- (LocalVariables|GetTeam1Score) 1.0))
            (LocalVariables|SetTeam2Score (- (LocalVariables|GetTeam2Score) 1.0))))))
    (:then_1
      (if (and (<= (LocalVariables|GetTeam1Score) 0.0) (<= (LocalVariables|GetTeam2Score) 0.0))
        ;[1 1 1] Draw
        (Class|GameMode|EndMatch GameMode)
        (Variables|Default|SetMatchEndInfo (Utilities|Struct|MakeSTRUCT_MatchEndInfo 0 0 0.0 0.0 true)))
      (Class|MordhauGameMode|SetTeamScore GameMode 0 (Math|Float|Max(Float) (LocalVariables|GetTeam1Score) 0.0))
      (Class|MordhauGameMode|SetTeamScore GameMode 1 (Math|Float|Max(Float) (LocalVariables|GetTeam2Score) 0.0)))))