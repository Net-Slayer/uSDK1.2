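; Battle mode interaction point that hands out deliverable items to the team opposing its capture point's owner.
; Interacting spawns the deliverable class, team-restricted, into the character's hands, refusing anyone already holding a deliverable in the right hand.
; A per-character map breaks or destroys that player's previous item if unheld.
; Activate shows a team-restricted widget and enables interaction; Disable hides it and destroys all spawned deliverables.
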(event EventBeginPlay)

(event Collision|EventActorBeginOverlap
  (params (OtherActor :type Actor%20Object%20Reference)))

(event EventTick
  (params (DeltaSeconds :type Float%20%28single-precision%29)))

(event EventOnInteractionStart
  (params (Character :type Mordhau%20Character%20Object%20Reference))
  (bind _capturepoint (Variables|Default|GetCapturePoint))
  (bind _spawnedbycharacter (Variables|Default|GetSpawnedByCharacter))
  (bind (_value _returnvalue) (Utilities|Map|Find _spawnedbycharacter Character))
  (Utilities|IsValid Character
    (:Is%20Valid
      (Utilities|IsValid _capturepoint
        (:Is%20Valid
          (bind _returnvalue_2 (Game|SpawnActorfromClass (Variables|Default|GetDeliverableClass) (Transformation|GetActorTransform) "Undefined" 0 0))
          (Variables|/Game/Mordhau/Blueprints/GameModes/Battle/BP_DeliverableEquipment.BP_DeliverableEquipment_C|SetUsableByTeam _returnvalue_2 (Utilities|Select :Index (Variables|/Script/Mordhau.ControlPoint|GetOwningTeam _capturepoint) :Option%200 1 :Option%201 0))
          (bind _returnvalue_3 (Class|MordhauCharacter|PickUp Character _returnvalue_2))
          (if _returnvalue_3
            (Utilities|Array|Add (Variables|Default|GetSpawnedDeliverables) _returnvalue_2)
            (Utilities|FlowControl|Sequence
              (:then_0
                (if _returnvalue
                  (Utilities|IsValid _value
                    (:Is%20Valid
                      (Utilities|IsValid (Class|MordhauEquipment|GetParentCharacter _value)
                        (:Is%20Not%20Valid
                          (bind _asbp_deliverable_equipment (Utilities|Casting|CastToBP_DeliverableEquipment _value)
                            (:then
                              (Default|Break _asbp_deliverable_equipment))
                            (:CastFailed
                              (Actor|DestroyActor _value)))))))))
              (:then_1
                (Utilities|Map|Add _spawnedbycharacter Character _returnvalue_2)))
            (else
              (Actor|DestroyActor _returnvalue_2))))))))

(fn ConstructionScript)

(fn CanInteract
  (params (Character :type Mordhau%20Character%20Object%20Reference))
  (bind _capturepoint (Variables|Default|GetCapturePoint))
  (Utilities|IsValid Character
    (:Is%20Valid
      (Utilities|IsValid _capturepoint
        (:Is%20Valid
          (if (!= (Variables|/Script/Mordhau.AdvancedCharacter|GetTeam Character) (Variables|/Script/Mordhau.ControlPoint|GetOwningTeam _capturepoint))
            (Utilities|Casting|CastToBP_DeliverableEquipment (Variables|/Script/Mordhau.MordhauCharacter|GetRightHandEquipment Character)
              (:then
                (return false))
              (:CastFailed
                _))
            (else
              (return false))))
        (:Is%20Not%20Valid
          _)))
    (:Is%20Not%20Valid
      _))
  (return (stale _returnvalue)))

(fn Activate
  (bind _mordhauwidget (Variables|Default|GetMordhauWidget))
  (Variables|Default|SetbIsInteractable true)
  (Variables|/Script/Mordhau.MordhauWidgetComponent|SetOverrideVisible _mordhauwidget -1)
  (Variables|/Script/Mordhau.MordhauWidgetComponent|SetViewTargetTeamRestriction _mordhauwidget (Math|Conversions|ToInteger(Byte) (Utilities|Select :Index (Variables|/Script/Mordhau.ControlPoint|GetOwningTeam (Variables|Default|GetCapturePoint)) :Option%200 1 :Option%201 0))))

(fn Disable
  (Variables|Default|SetbIsInteractable false)
  (Variables|/Script/Mordhau.MordhauWidgetComponent|SetOverrideVisible (Variables|Default|GetMordhauWidget) 0)
  (for _array_element (Variables|Default|GetSpawnedDeliverables)
    (Utilities|IsValid _array_element
      (:Is%20Valid
        (Actor|DestroyActor _array_element))))
  (Utilities|Array|Clear (Variables|Default|GetSpawnedDeliverables)))