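; Frontline capture point that can be taken by teams or driven by objectives (destroyables, deliveries, pushables, interactables, kill targets).
; Objectives are gathered at construction and their progress averaged, counting invalid ones as done.
; The server maps that to capture progress by point type: hidden and push points go to the opposing team, while others zero the owner's score after a delay on completion.
; Cosmetic events drive team-relative announcements, sounds, widget colors and pulses.
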(event Custom|TriggerWinDelayed
  (Utilities|FlowControl|Delay (Variables|Default|GetObjectiveWinDelay))
  (bind _asbp_frontline_game_mode (Utilities|Casting|CastToBP_FrontlineGameMode (Game|GetGameMode)))
  (if (Class|GameMode|IsMatchinProgress _asbp_frontline_game_mode)
    (Utilities|FlowControl|Sequence
      (:then_0
        (switch int (Math|Conversions|ToInteger(Byte) (Variables|Default|GetOwningTeam))
          (:0
            (Class|MordhauGameMode|SetTeamScore _asbp_frontline_game_mode 0 0.0))
          (:1
            (Class|MordhauGameMode|SetTeamScore _asbp_frontline_game_mode 1 0.0))))
      (:then_1
        (Class|ControlPoint|SetCaptureProgress 0.0 (Variables|Default|GetOwningTeam) false)
        (Class|ControlPoint|UpdateVisuals)))))

(event Custom|Pulse
  (bind _topbar_cap_point_widget (Variables|Default|GetTopBar%20Cap%20Point%20Widget))
  (bind _floaterwidget (Variables|Default|GetFloaterWidget))
  (UserInterface|Animation|PlayAnimation _topbar_cap_point_widget (Variables|/Game/Mordhau/Blueprints/GameModes/Battle/BP_CapPointWidget.BP_CapPointWidget_C|GetPulseAnim _topbar_cap_point_widget) 0.0 0 "Forward" 0.2)
  (Appearance|SetColorandOpacity (Variables|/Game/Mordhau/Blueprints/GameModes/Battle/BP_CapPointWidget.BP_CapPointWidget_C|GetPulse _topbar_cap_point_widget) "(R=1.000000,G=1.000000,B=1.000000,A=1.000000)" :!class /Script/UMG.Image)
  (Utilities|IsValid _floaterwidget
    (:Is%20Valid
      (UserInterface|Animation|PlayAnimation _floaterwidget (Variables|/Game/Mordhau/Blueprints/GameModes/Battle/BP_FloatingCapPointWidget.BP_FloatingCapPointWidget_C|GetPulseAnim _floaterwidget) 0.0 0 "Forward" 0.2)
      (Appearance|SetColorandOpacity (Variables|/Game/Mordhau/Blueprints/GameModes/Battle/BP_FloatingCapPointWidget.BP_FloatingCapPointWidget_C|GetPulse _floaterwidget) "(R=1.000000,G=1.000000,B=1.000000,A=1.000000)" :!class /Script/UMG.Image))))

(event EventBeginPlay
  (bind _mordhauwidget (Variables|Components|GetMordhauWidget))
  (bind _objectives (Variables|Default|GetObjectives))
  (Utilities|FlowControl|Sequence
    (:then_0
      (Networking|CanExecuteCosmeticEvents
        (:True
          (if (or (> (Utilities|Array|Length (Variables|Default|GetObjectives)) 0) (Variables|Default|GetbIsHiddenPoint))
            (Components|DestroyComponent _mordhauwidget)
            (Variables|Default|SetWidgetComponent 0)
            (else
              (bind _asbp_floating_cap_point_widget (Utilities|Casting|CastToBP_FloatingCapPointWidget (UserInterface|GetUserWidgetObject _mordhauwidget)))
              (Variables|Default|SetFloaterWidget _asbp_floating_cap_point_widget)
              (Default|Initialize _asbp_floating_cap_point_widget self))))))
    (:then_1
      (if (> (Utilities|Array|Length _objectives) 0)
        (for _array_element _objectives
          (Utilities|IsValid (Utilities|ToObject(Interface) _array_element)
            (:Is%20Valid
              (Default|OnInitialize _array_element self))))
        (CallFunction|ObjectivesChanged)))))

(event EventOnCapturingTeamChanged
  (bind _name (Variables|Default|GetName))
  (bind _capturingteam (Variables|Default|GetCapturingTeam))
  (|CallParentFunction)
  (Networking|CanExecuteCosmeticEvents
    (:True
      (if (not (or (Variables|Default|GetbIsHiddenPoint) (Variables|Default|GetIsPushPoint)))
        (if (and (> (Utilities|Time|GetTimeSeconds) 3.0) (Variables|Default|GetShowAnnouncements))
          (if (!= _capturingteam 255)
            (bind _relevance (CallFunction|GetTeamRelevance _capturingteam))
            (bind _asbp_mordhau_hud (Utilities|Casting|CastToBP_MordhauHUD (Class|MordhauUtilityLibrary|GetMordhauHUD)))
            (switch int _relevance
              (:0
                (Default|ShowAnnouncement _asbp_mordhau_hud (Utilities|Text|FormatText "We are capturing {a}!" _name) "" 4.0))
              (:1
                (Default|ShowAnnouncement _asbp_mordhau_hud (Utilities|Text|FormatText "Enemy is capturing {a}!" _name) "" 4.0)
                (Audio|PlaySound2D 0 2.0 1.0 0.0 0 0)))))))))

(event EventOnOwningTeamChanged
  (bind _topbar_cap_point_widget (Variables|Default|GetTopBar%20Cap%20Point%20Widget))
  (bind _name (Variables|Default|GetName))
  (bind _bishiddenpoint (Variables|Default|GetbIsHiddenPoint))
  (bind _ispushpoint (Variables|Default|GetIsPushPoint))
  (bind _owningteam (Variables|Default|GetOwningTeam))
  (bind _returnvalue (or _bishiddenpoint _ispushpoint))
  (|CallParentFunction)
  (Networking|CanExecuteCosmeticEvents
    (:True
      (Utilities|FlowControl|Sequence
        (:then_0
          (if (and (> (Utilities|Time|GetTimeSeconds) 3.0) (Variables|Default|GetShowAnnouncements))
            (if (!= _owningteam 255)
              (bind _relevance (CallFunction|GetTeamRelevance _owningteam))
              (bind _asbp_frontline_hud (Utilities|Casting|CastToBP_FrontlineHUD (Class|MordhauUtilityLibrary|GetMordhauHUD)))
              (Utilities|FlowControl|Sequence
                (:then_0
                  (switch int _relevance
                    (:0
                      (Utilities|FlowControl|Sequence
                        (:then_0
                          (if _returnvalue
                            (if _ispushpoint
                              (CallFunction|ShowPushAttackerAnnouncement))
                            (else
                              (Default|ShowAnnouncement _asbp_frontline_hud (Utilities|Text|FormatText "We have taken {a}!" _name) "" 4.0))))
                        (:then_1
                          (Audio|PlaySound2D 0 2.0 1.0 0.0 0 0)
                          (Utilities|IsValid _topbar_cap_point_widget :!label _label
                            (:Is%20Valid
                              (UserInterface|Animation|PlayAnimation _topbar_cap_point_widget (Variables|/Game/Mordhau/Blueprints/GameModes/Battle/BP_CapPointWidget.BP_CapPointWidget_C|GetCapAnim _topbar_cap_point_widget) 0.0 1 "Forward" 0.8)
                              (Utilities|IsValid (Variables|/Game/Mordhau/Blueprints/GameModes/Battle/BP_FrontlineHUD.BP_FrontlineHUD_C|GetFrontlineHUDWidget _asbp_frontline_hud)
                                (:Is%20Valid
                                  (UserInterface|Animation|PlayAnimation (Variables|/Game/Mordhau/Blueprints/GameModes/Battle/BP_FrontlineHUDWidget.BP_FrontlineHUDWidget_C|GetBP_CapPointInfoPanelWidget (Variables|/Game/Mordhau/Blueprints/GameModes/Battle/BP_FrontlineHUD.BP_FrontlineHUD_C|GetFrontlineHUDWidget _asbp_frontline_hud)) (Variables|/Game/Mordhau/Blueprints/GameModes/Battle/BP_CapPointInfoPanelWidget.BP_CapPointInfoPanelWidget_C|GetFlashAnim (Variables|/Game/Mordhau/Blueprints/GameModes/Battle/BP_FrontlineHUDWidget.BP_FrontlineHUDWidget_C|GetBP_CapPointInfoPanelWidget (Variables|/Game/Mordhau/Blueprints/GameModes/Battle/BP_FrontlineHUD.BP_FrontlineHUD_C|GetFrontlineHUDWidget _asbp_frontline_hud))) 0.0 1 "Forward" 1.0))))))))
                    (:1
                      (Utilities|FlowControl|Sequence
                        (:then_0
                          (if _returnvalue
                            (if _ispushpoint
                              (CallFunction|ShowPushDefenderAnnouncement))
                            (else
                              (Default|ShowAnnouncement _asbp_frontline_hud (Utilities|Text|FormatText "Enemy has taken {a}!" _name) "" 4.0))))
                        (:then_1
                          (Audio|PlaySound2D 0 2.0 1.0 0.0 0 0)
                          (goto _label))))))
                (:then_1
                  ;[1 1 1] This is hacky, but we need a slight delay so requirements update next frame
                  (if (Variables|Default|GetbIsHiddenPoint)
                    (Utilities|FlowControl|Delay 0.1)
                    (bind _asbp_frontline_hud_2 (Utilities|Casting|CastToBP_FrontlineHUD (Class|MordhauUtilityLibrary|GetMordhauHUD)))
                    (Default|ShowObjectives _asbp_frontline_hud_2)))))))))))

(event EventEnemyGainedPrerequisites
  (for _array_element (Variables|Default|GetObjectives)
    (Utilities|IsValid (Utilities|ToObject(Interface) _array_element)
      (:Is%20Valid
        (Default|OnEnemyGainedPrerequisites _array_element)))))

(event EventEnemyLostPrerequisites
  (for _array_element (Variables|Default|GetObjectives)
    (Utilities|IsValid (Utilities|ToObject(Interface) _array_element)
      (:Is%20Valid
        (Default|OnEnemyLostPrerequisites _array_element)))))

(event EventUpdateUIWidgets
  (bind _owningteam (Variables|Default|GetOwningTeam))
  (bind _capturingteam (Variables|Default|GetCapturingTeam))
  (bind _returnvalue (Math|Conversions|ToInteger(Byte) _owningteam))
  (bind _returnvalue_2 (Math|Conversions|ToInteger(Byte) _capturingteam))
  (Utilities|FlowControl|Sequence
    (:then_0
      (bind _asmordhau_game_state (Utilities|Casting|CastToMordhauGameState (Game|GetGameState)))
      (if (!= (Variables|Default|GetOwningTeam) 255)
        (if (Utilities|Array|IsValidIndex (Variables|/Script/Mordhau.MordhauGameState|GetTeamColors _asmordhau_game_state) _returnvalue)
          (CallFunction|SetCapPointWidgetColors (Utilities|Array|Get(acopy) (Variables|/Script/Mordhau.MordhauGameState|GetTeamColors _asmordhau_game_state) _returnvalue) (Utilities|Struct|MakeLinearColor (* (.R (Utilities|Struct|BreakLinearColor (Utilities|Array|Get(acopy) (Variables|/Script/Mordhau.MordhauGameState|GetTeamColors _asmordhau_game_state) _returnvalue))) 4.0) (* (.G (Utilities|Struct|BreakLinearColor (Utilities|Array|Get(acopy) (Variables|/Script/Mordhau.MordhauGameState|GetTeamColors _asmordhau_game_state) _returnvalue))) 4.0) (* (.B (Utilities|Struct|BreakLinearColor (Utilities|Array|Get(acopy) (Variables|/Script/Mordhau.MordhauGameState|GetTeamColors _asmordhau_game_state) _returnvalue))) 4.0) (.A (Utilities|Struct|BreakLinearColor (Utilities|Array|Get(acopy) (Variables|/Script/Mordhau.MordhauGameState|GetTeamColors _asmordhau_game_state) _returnvalue))))))
        (elif (Utilities|Array|IsValidIndex (Variables|/Script/Mordhau.MordhauGameState|GetTeamColors _asmordhau_game_state) _returnvalue_2)
          (CallFunction|SetCapPointWidgetColors "(R=0.000000,G=0.000000,B=0.000000,A=0.750000)" (Utilities|Struct|MakeLinearColor (* (.R (Utilities|Struct|BreakLinearColor (Utilities|Array|Get(acopy) (Variables|/Script/Mordhau.MordhauGameState|GetTeamColors _asmordhau_game_state) _returnvalue_2))) 4.0) (* (.G (Utilities|Struct|BreakLinearColor (Utilities|Array|Get(acopy) (Variables|/Script/Mordhau.MordhauGameState|GetTeamColors _asmordhau_game_state) _returnvalue_2))) 4.0) (* (.B (Utilities|Struct|BreakLinearColor (Utilities|Array|Get(acopy) (Variables|/Script/Mordhau.MordhauGameState|GetTeamColors _asmordhau_game_state) _returnvalue_2))) 4.0) (.A (Utilities|Struct|BreakLinearColor (Utilities|Array|Get(acopy) (Variables|/Script/Mordhau.MordhauGameState|GetTeamColors _asmordhau_game_state) _returnvalue_2)))))
          (else
            (CallFunction|SetCapPointWidgetColors "(R=0.000000,G=0.000000,B=0.000000,A=0.750000)" "(R=1.000000,G=1.000000,B=1.000000,A=1.000000)")))))
    (:then_1
      (for _array_element (Variables|Default|GetObjectives)
        (Utilities|IsValid (Utilities|ToObject(Interface) _array_element)
          (:Is%20Valid
            (Default|OnUpdateUIWidgets _array_element)))))))

(event EventOnStartedFlashing
  (bind _topbar_cap_point_widget (Variables|Default|GetTopBar%20Cap%20Point%20Widget))
  (bind _capwarninganim (Variables|/Game/Mordhau/Blueprints/GameModes/Battle/BP_CapPointWidget.BP_CapPointWidget_C|GetCapWarningAnim _topbar_cap_point_widget))
  (bind _asmordhau_game_state (Utilities|Casting|CastToMordhauGameState (Game|GetGameState)))
  (Utilities|IsValid _topbar_cap_point_widget
    (:Is%20Valid
      (if (Variables|Default|GetFlashShouldOnlyPulse)
        (CallFunction|Pulse)
        (else
          (UserInterface|Animation|PlayAnimation _topbar_cap_point_widget _capwarninganim 0.0 1 "Forward" 1.0) ; Play alert anim first
          (EventDispatchers|AssignOnAnimationFinished _capwarninganim (delegate Custom|Pulse)) ; Then start pulsing when it's done
        )))))

(event EventOnStoppedFlashing
  (bind _topbar_cap_point_widget (Variables|Default|GetTopBar%20Cap%20Point%20Widget))
  (bind _floaterwidget (Variables|Default|GetFloaterWidget))
  (bind _captureprogress (Variables|Default|GetCaptureProgress))
  (bind _returnvalue (== _captureprogress 0.0))
  (bind _pulseanim (Variables|/Game/Mordhau/Blueprints/GameModes/Battle/BP_FloatingCapPointWidget.BP_FloatingCapPointWidget_C|GetPulseAnim _floaterwidget))
  (bind _pulseanim_2 (Variables|/Game/Mordhau/Blueprints/GameModes/Battle/BP_CapPointWidget.BP_CapPointWidget_C|GetPulseAnim _topbar_cap_point_widget))
  (bind _capwarninganim (Variables|/Game/Mordhau/Blueprints/GameModes/Battle/BP_CapPointWidget.BP_CapPointWidget_C|GetCapWarningAnim _topbar_cap_point_widget))
  (Utilities|IsValid _topbar_cap_point_widget
    (:Is%20Valid
      (EventDispatchers|UnbindEventfromOnAnimationFinished _capwarninganim (delegate Custom|Pulse))
      (Utilities|FlowControl|Sequence
        (:then_0
          (if _returnvalue
            (if (Class|UserWidget|IsAnimationPlaying _topbar_cap_point_widget _capwarninganim)
              (Utilities|FlowControl|Delay (- (Class|WidgetAnimation|GetEndTime _capwarninganim) (Class|UserWidget|GetAnimationCurrentTime _topbar_cap_point_widget _capwarninganim))))
            (Class|UserWidget|StopAnimation _topbar_cap_point_widget _pulseanim_2)
            (else
              (UserInterface|Animation|PlayAnimation _topbar_cap_point_widget _pulseanim_2 0.0 1 "Forward" 0.2))))
        (:then_1
          (Utilities|IsValid _floaterwidget
            (:Is%20Valid
              (if _returnvalue
                (Class|UserWidget|StopAnimation _floaterwidget _pulseanim)
                (else
                  (UserInterface|Animation|PlayAnimation _floaterwidget _pulseanim 0.0 1 "Forward" 0.2))))))))))

(fn ConstructionScript
  (bind _objectives (Variables|Default|GetObjectives))
  (Variables|Default|SetCaptureArea (Variables|Components|GetCaptureAreaCollision))
  (Variables|Default|SetWidgetComponent (Variables|Components|GetMordhauWidget))
  (for _array_element (Variables|Default|GetDestroyables)
    (Utilities|IsValid _array_element
      (:Is%20Valid
        (Utilities|Array|Add _objectives _array_element))))
  (for _array_element_2 (Variables|Default|GetDeliverySpots)
    (Utilities|IsValid _array_element_2
      (:Is%20Valid
        (Utilities|Array|Add _objectives _array_element_2))))
  (for _array_element_3 (Variables|Default|GetPushables)
    (Utilities|IsValid _array_element_3
      (:Is%20Valid
        (Utilities|Array|Add _objectives _array_element_3))))
  (for _array_element_4 (Variables|Default|GetInteractables)
    (Utilities|IsValid _array_element_4
      (:Is%20Valid
        (Utilities|Array|Add _objectives _array_element_4))))
  (for _array_element_5 (Variables|Default|GetKill)
    (Utilities|IsValid _array_element_5
      (:Is%20Valid
        (Utilities|Array|Add _objectives _array_element_5)))))

(fn GetTeamRelevance
  (params (Team :type Byte))
  (bind _returnvalue (Game|GetPlayerController 0))
  (Utilities|IsValid _returnvalue
    (:Is%20Valid
      (bind _asmordhau_player_state (Utilities|Casting|CastToMordhauPlayerState (Variables|/Script/Engine.Controller|GetPlayerState _returnvalue))
        (:then
          (if (or (== (Variables|/Script/Mordhau.MordhauPlayerState|GetTeam _asmordhau_player_state) 0) (== (Variables|/Script/Mordhau.MordhauPlayerState|GetTeam _asmordhau_player_state) 1))
            (return (Math|Conversions|ToInteger(Boolean) (!= (Math|Conversions|ToInteger(Byte) Team) (Variables|/Script/Mordhau.MordhauPlayerState|GetTeam _asmordhau_player_state))))
            (else
              _)))
        (:CastFailed
          _)))
    (:Is%20Not%20Valid
      _))
  (return 2))

(fn SetCapPointWidgetColors
  (params (Fill%20Color :type Linear%20Color%20Structure) (Progress%20Bar%20Color :type Linear%20Color%20Structure))
  (bind _spawnpointwidget (Variables|Default|GetSpawnPointWidget))
  (bind _topbar_cap_point_widget (Variables|Default|GetTopBar%20Cap%20Point%20Widget))
  (bind _floaterwidget (Variables|Default|GetFloaterWidget))
  (bind _topbar_cap_point_teambase_widget (Variables|Default|GetTopBar%20Cap%20Point%20TeamBase%20Widget))
  (Utilities|FlowControl|Sequence
    (:then_0
      (Utilities|IsValid _topbar_cap_point_widget
        (:Is%20Valid
          (Appearance|SetColorandOpacity (Variables|/Game/Mordhau/Blueprints/GameModes/Battle/BP_CapPointWidget.BP_CapPointWidget_C|GetFill _topbar_cap_point_widget) Fill%20Color :!class /Script/UMG.Image)
          (Appearance|SetColorandOpacity (Variables|/Game/Mordhau/Blueprints/GameModes/Battle/BP_CapPointWidget.BP_CapPointWidget_C|GetCapProgressBar _topbar_cap_point_widget) Progress%20Bar%20Color :!class /Script/UMG.Image))))
    (:then_1
      (Utilities|IsValid _topbar_cap_point_teambase_widget
        (:Is%20Valid
          (Appearance|SetColorandOpacity (Variables|/Game/Mordhau/Blueprints/GameModes/Battle/BP_CapPointTeamBaseWidget.BP_CapPointTeamBaseWidget_C|GetFill _topbar_cap_point_teambase_widget) Fill%20Color :!class /Script/UMG.Image)
          (Appearance|SetColorandOpacity (Variables|/Game/Mordhau/Blueprints/GameModes/Battle/BP_CapPointTeamBaseWidget.BP_CapPointTeamBaseWidget_C|GetCapProgressBar _topbar_cap_point_teambase_widget) Progress%20Bar%20Color :!class /Script/UMG.Image))))
    (:then_2
      (Utilities|IsValid _spawnpointwidget
        (:Is%20Valid
          (Appearance|SetColorandOpacity (Variables|/Game/Mordhau/Blueprints/GameModes/Battle/BP_CapPointWidget.BP_CapPointWidget_C|GetFill _spawnpointwidget) Fill%20Color :!class /Script/UMG.Image)
          (Appearance|SetColorandOpacity (Variables|/Game/Mordhau/Blueprints/GameModes/Battle/BP_CapPointWidget.BP_CapPointWidget_C|GetCapProgressBar _spawnpointwidget) Progress%20Bar%20Color :!class /Script/UMG.Image))))
    (:then_3
      (Utilities|IsValid _floaterwidget
        (:Is%20Valid
          (Appearance|SetColorandOpacity (Variables|/Game/Mordhau/Blueprints/GameModes/Battle/BP_FloatingCapPointWidget.BP_FloatingCapPointWidget_C|GetCap _floaterwidget) Progress%20Bar%20Color :!class /Script/UMG.Image))))))

(fn ObjectivesChanged
  (bind _topbar_cap_point_teambase_widget (Variables|Default|GetTopBar%20Cap%20Point%20TeamBase%20Widget))
  (bind _objectives (Variables|Default|GetObjectives))
  (bind _owningteam (Variables|Default|GetOwningTeam))
  (bind _returnvalue (Utilities|Select :Index _owningteam :Option%200 1 :Option%201 0))
  (LocalVariables|SetPreviousProgress (Variables|Default|GetObjectiveProgress))
  (Variables|Default|SetObjectiveProgress 0.0)
  (for _array_element _objectives
    (Utilities|IsValid (Utilities|ToObject(Interface) _array_element)
      (:Is%20Valid
        (bind _progress (Default|GetObjectiveProgress _array_element))
        (Variables|Default|SetObjectiveProgress (+ _progress (Variables|Default|GetObjectiveProgress))))
      (:Is%20Not%20Valid
        (Variables|Default|SetObjectiveProgress (+ 1.0 (Variables|Default|GetObjectiveProgress))))))
  (Variables|Default|SetObjectiveProgress (Math|Float|Clamp(Float) (/ (Variables|Default|GetObjectiveProgress) (Math|Conversions|ToFloat(Integer) (Utilities|Array|Length _objectives)))))
  (Utilities|FlowControl|Sequence
    (:then_0
      (for _array_element_2 (Variables|Default|GetObjectives)
        (Utilities|IsValid (Utilities|ToObject(Interface) _array_element_2)
          (:Is%20Valid
            (Default|OnAnyObjectiveProgressChanged _array_element_2)))))
    (:then_1
      (Networking|CanExecuteCosmeticEvents
        (:True
          (if (< (LocalVariables|GetPreviousProgress) (Variables|Default|GetObjectiveProgress))
            (Utilities|IsValid _topbar_cap_point_teambase_widget
              (:Is%20Valid
                (if (not (Class|UserWidget|IsPlayingAnimation _topbar_cap_point_teambase_widget))
                  (UserInterface|Animation|PlayAnimation _topbar_cap_point_teambase_widget (Variables|/Game/Mordhau/Blueprints/GameModes/Battle/BP_CapPointTeamBaseWidget.BP_CapPointTeamBaseWidget_C|GetPulseAnim _topbar_cap_point_teambase_widget) 0.0 1 "Forward" 1.0))))))))
    (:then_2
      (Networking|SwitchHasAuthority
        (:Authority
          (if (not (Variables|Default|GetObjectivesCompleted))
            (if (Variables|Default|GetbIsHiddenPoint)
              (if (not (== (Variables|Default|GetObjectiveProgress) 0.0))
                (Class|ControlPoint|SetCaptureProgress (Variables|Default|GetObjectiveProgress) _returnvalue false)
                (Class|ControlPoint|UpdateVisuals))
              (elif (Variables|Default|GetIsPushPoint)
                (if (not (== (Variables|Default|GetObjectiveProgress) 0.0))
                  (if (== (Variables|Default|GetObjectiveProgress) 1.0)
                    (Class|ControlPoint|SetCaptureProgress 1.0 _returnvalue false)
                    (else
                      (Class|ControlPoint|SetCaptureProgress (- 1.0 (Variables|Default|GetObjectiveProgress)) _returnvalue false)))
                  (Utilities|FlowControl|Sequence
                    (:then_0
                      (bind _asbp_frontline_game_state (Utilities|Casting|CastToBP_FrontlineGameState (Game|GetGameState)))
                      (Variables|/Game/Mordhau/Blueprints/GameModes/Battle/BP_FrontlineGameState.BP_FrontlineGameState_C|SetPushWinDelay _asbp_frontline_game_state (Variables|Default|GetObjectiveWinDelay)))
                    (:then_1
                      (Class|ControlPoint|UpdateVisuals))))
                (elif (== (Variables|Default|GetObjectiveProgress) 1.0)
                  (CallFunction|TriggerWinDelayed)
                  (else
                    (Class|ControlPoint|SetCaptureProgress (- 1.0 (Variables|Default|GetObjectiveProgress)) (Variables|Default|GetOwningTeam) false)
                    (Class|ControlPoint|UpdateVisuals)))))))))
    (:then_3
      (if (and (not (Variables|Default|GetObjectivesCompleted)) (== (Variables|Default|GetObjectiveProgress) 1.0))
        (Variables|Default|SetObjectivesCompleted true)
        (CallFunction|OnObjectivesCompleted)))))

(fn ShowPushAttackerAnnouncement)

(fn ShowPushDefenderAnnouncement)

(fn OnObjectivesCompleted)