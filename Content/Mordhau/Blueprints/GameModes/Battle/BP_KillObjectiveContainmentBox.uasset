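; A containment volume for Battle mode that tells one assigned kill objective when it is inside or outside its allowed area.
; On overlap, it increments the objective's containment volume counter and calls its left-out-of-bounds function.
; On end overlap, it decrements the counter and calls the entered-out-of-bounds function only when the count reaches zero or below.
; The counter lives on the objective, so multiple overlapping boxes can form one containment area.
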(event EventBeginPlay)

(event Collision|EventActorBeginOverlap
  (params (OtherActor :type Actor%20Object%20Reference))
  (bind _killobjectivetocontain (Variables|Default|GetKillObjectiveToContain))
  (if (== _killobjectivetocontain OtherActor)
    (bind _output_get (Variables|/Game/Mordhau/Blueprints/GameModes/Battle/BP_FrontlineKillObjective.BP_FrontlineKillObjective_C|SetContainmentVolumeCounter _killobjectivetocontain (+ (Variables|/Game/Mordhau/Blueprints/GameModes/Battle/BP_FrontlineKillObjective.BP_FrontlineKillObjective_C|GetContainmentVolumeCounter _killobjectivetocontain) 1)))
    (Class|AdvancedCharacter|LeftOutOfBoundsArea _killobjectivetocontain)))

(event Collision|EventActorEndOverlap
  (params (OtherActor :type Actor%20Object%20Reference))
  (bind _killobjectivetocontain (Variables|Default|GetKillObjectiveToContain))
  (if (== OtherActor _killobjectivetocontain)
    (bind _output_get (Variables|/Game/Mordhau/Blueprints/GameModes/Battle/BP_FrontlineKillObjective.BP_FrontlineKillObjective_C|SetContainmentVolumeCounter _killobjectivetocontain (- (Variables|/Game/Mordhau/Blueprints/GameModes/Battle/BP_FrontlineKillObjective.BP_FrontlineKillObjective_C|GetContainmentVolumeCounter _killobjectivetocontain) 1)))
    (if (<= _output_get 0)
      (Class|AdvancedCharacter|EnteredOutOfBoundsArea _killobjectivetocontain))))

(fn ConstructionScript)