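; Wrapper objective for Mordhau's Frontline mode that stands in for a referenced kill objective.
; It forwards initialization, progress-change, enemy prerequisite and UI update events to that KillObjective whenever the reference is valid.
; Reported progress is the kill objective's progress scaled by Weight, or the full Weight when the reference is invalid.
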(event Collision|EventActorBeginOverlap
  (params (OtherActor :type Actor%20Object%20Reference)))

(event EventTick
  (params (DeltaSeconds :type Float%20%28single-precision%29)))

(event EventOnAnyObjectiveProgressChanged
  (bind _killobjective (Variables|Default|GetKillObjective))
  (Utilities|IsValid _killobjective
    (:Is%20Valid
      (Default|OnAnyObjectiveProgressChanged _killobjective))))

(event EventOnEnemyGainedPrerequisites
  (bind _killobjective (Variables|Default|GetKillObjective))
  (Utilities|IsValid _killobjective
    (:Is%20Valid
      (Default|OnEnemyGainedPrerequisites _killobjective))))

(event EventOnEnemyLostPrerequisites
  (bind _killobjective (Variables|Default|GetKillObjective))
  (Utilities|IsValid _killobjective
    (:Is%20Valid
      (Default|OnEnemyLostPrerequisites _killobjective))))

(event EventOnInitialize
  (params (Point :type BP%20Capture%20Point%20Object%20Reference))
  (bind _killobjective (Variables|Default|GetKillObjective))
  (Utilities|IsValid _killobjective
    (:Is%20Valid
      (Default|OnInitialize _killobjective Point))))

(event EventOnUpdateUIWidgets
  (bind _killobjective (Variables|Default|GetKillObjective))
  (Utilities|IsValid _killobjective
    (:Is%20Valid
      (Default|OnUpdateUIWidgets _killobjective))))

(fn ConstructionScript)

(fn GetObjectiveProgress
  (bind _killobjective (Variables|Default|GetKillObjective))
  (Utilities|IsValid _killobjective
    (:Is%20Valid
      (bind _progress (Default|GetObjectiveProgress _killobjective))
      (return (* _progress (Variables|Default|GetWeight))))
    (:Is%20Not%20Valid
      (return (Variables|Default|GetWeight)))))