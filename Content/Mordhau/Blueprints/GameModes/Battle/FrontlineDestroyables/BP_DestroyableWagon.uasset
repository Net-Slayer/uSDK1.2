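; Destroyable wagon objective for the Frontline game mode, extending a parent destroyable that supplies replicated health and the damage stage index.
; When health drops, it pushes a changed damage stage into the wagon's AnimBP, or calls a montage play if the stage is unchanged.
; On authority, the skeletal mesh always ticks pose and refreshes bones, keeping server-side bone transforms current even when not rendered.
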(event EventBeginPlay
  (|CallParentFunction)
  (Networking|SwitchHasAuthority
    (:Authority
      (Variables|/Script/Engine.SkinnedMeshComponent|SetMeshComponentUpdateFlag (Variables|Default|GetSkeletalMesh) "AlwaysTickPoseAndRefreshBones"))))

(event Collision|EventActorBeginOverlap
  (params (OtherActor :type Actor%20Object%20Reference))
  (|CallParentFunction OtherActor) ; This node is disabled and will not be called.\nDrag off pins to build functionality.
)

(event EventTick
  (params (DeltaSeconds :type Float%20%28single-precision%29))
  (|CallParentFunction DeltaSeconds) ; This node is disabled and will not be called.\nDrag off pins to build functionality.
)

(event EventUpdateAnimInstance
  (bind _bestdamageidx (Variables|Default|GetBestDamageIdx))
  (if (> (Variables|Default|GetLastReplicatedHealth) (Variables|Default|GetReplicatedHealth))
    (bind _asab_destroyable_wagon (Utilities|Casting|CastToAB_DestroyableWagon (Components|SkeletalMesh|GetAnimInstance (Variables|Default|GetSkeletalMesh))))
    (if (== (Variables|/Game/Mordhau/Animations/Blueprints/AB_DestroyableWagon.AB_DestroyableWagon_C|GetHealthStage _asab_destroyable_wagon) _bestdamageidx)
      (Animation|Montage|PlayMontage (Variables|Default|GetSkeletalMesh) 0)
      (else
        (Variables|/Game/Mordhau/Animations/Blueprints/AB_DestroyableWagon.AB_DestroyableWagon_C|SetHealthStage _asab_destroyable_wagon _bestdamageidx)))))

(fn ConstructionScript
  (|CallParentFunction))