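; BP_CrossroadsWagon is a horse-drawn wagon that travels along a target spline on a timer once the match starts.
; The authority records the start time, and Tick derives progress from it using server world time.
; Spline position drives the wagon AnimBP's two joint rotations and distance-based wheel spin, and the OnRep matches horse play rate to travel speed.
; Construction links horse hair and harnesses via master pose, and Tick fades in wheel audio.
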(event Collision|EventActorBeginOverlap
  (params (OtherActor :type Actor%20Object%20Reference))
  (|CallParentFunction OtherActor) ; This node is disabled and will not be called.\nDrag off pins to build functionality.
)

(event EventTick
  (params (DeltaSeconds :type Float%20%28single-precision%29))
  (bind _returnvalue (Game|GetGameMode))
  (bind _splinerange (Variables|Default|GetSplineRange))
  (bind _secondjointdistanceoffset (Variables|Default|GetSecondJointDistanceOffset))
  (bind _wheelssound (Variables|Default|GetWheelsSound))
  (bind _progress (Variables|Default|GetProgress))
  (bind _targetsplineactor (Variables|Default|GetTargetSplineActor))
  (bind (_x _y) (Math|Vector2D|BreakVector2D _splinerange))
  (bind _spline (Variables|/Game/Mordhau/Blueprints/Interactables/BP_SplineActor.BP_SplineActor_C|GetSpline _targetsplineactor))
  (bind _returnvalue_2 (Math|Float|Lerp _x _y _progress))
  (bind _returnvalue_3 (Spline|GetSplineLength _spline))
  (bind _returnvalue_4 (* _returnvalue_2 _returnvalue_3))
  (|CallParentFunction DeltaSeconds)
  (Utilities|FlowControl|Sequence
    (:then_0
      (Networking|SwitchHasAuthority
        (:Authority
          (Utilities|Casting|CastToMordhauGameMode _returnvalue)
          (if (Class|GameModeBase|HasMatchStarted _returnvalue)
            (Utilities|FlowControl|DoOnce false
              (:Completed
                (Variables|Default|SetServerMoveStartTime (Utilities|Time|GetTimeSeconds))))))))
    (:then_1
      (if (!= (Variables|Default|GetServerMoveStartTime) -1.0)
        (bind _asmordhau_game_state (Utilities|Casting|CastToMordhauGameState (Game|GetGameState)))
        (if (!= (Class|MordhauUtilityLibrary|GetNormalizedTime (Variables|Default|GetServerMoveStartTime) (+ (Variables|Default|GetServerMoveStartTime) (Variables|Default|GetTimeToReachGoal)) (GameState|GetServerWorldTimeSeconds _asmordhau_game_state)) (Variables|Default|GetProgress))
          (Class|PushableActor|SetProgress (Class|MordhauUtilityLibrary|GetNormalizedTime (Variables|Default|GetServerMoveStartTime) (+ (Variables|Default|GetServerMoveStartTime) (Variables|Default|GetTimeToReachGoal)) (GameState|GetServerWorldTimeSeconds _asmordhau_game_state))))))
    (:then_2
      (Utilities|IsValid _targetsplineactor
        (:Is%20Valid
          (bind _asab_foot_soldier_wagon (Utilities|Casting|CastToAB_FootSoldierWagon (Components|SkeletalMesh|GetAnimInstance (Variables|Default|GetSkeletalMesh))))
          (bind _output (CallFunction|GetTransformAlongSplineOffset 6.2e+02 _secondjointdistanceoffset))
          (Variables|/Game/Mordhau/Animations/Blueprints/AB_FootSoldierWagon.AB_FootSoldierWagon_C|SetJoint1RotationWorld _asab_foot_soldier_wagon (.Rotation (Math|Transform|BreakTransform _output)))
          (bind _output_2 (CallFunction|GetTransformAlongSplineOffset _secondjointdistanceoffset 1.6e+03))
          (Variables|/Game/Mordhau/Animations/Blueprints/AB_FootSoldierWagon.AB_FootSoldierWagon_C|SetJoint2RotationWorld _asab_foot_soldier_wagon (.Rotation (Math|Transform|BreakTransform _output_2)))
          (Variables|/Game/Mordhau/Animations/Blueprints/AB_FootSoldierWagon.AB_FootSoldierWagon_C|SetFrontWheelRotationLocal _asab_foot_soldier_wagon (Math|Rotator|MakeRotator 0.0 (* (/ _returnvalue_4 (Math|Float|MultiplybyPi (Variables|Default|GetFrontWheelDiameter))) -3.6e+02) 0.0))
          (Variables|/Game/Mordhau/Animations/Blueprints/AB_FootSoldierWagon.AB_FootSoldierWagon_C|SetBackWheelRotationLocal _asab_foot_soldier_wagon (Math|Rotator|MakeRotator 0.0 (* (/ _returnvalue_4 (Math|Float|MultiplybyPi (Variables|Default|GetBackWheelDiameter))) -3.6e+02) 0.0)))))
    (:then_3
      (Networking|CanExecuteCosmeticEvents
        (:True
          (if (not (Audio|Components|Audio|IsPlaying _wheelssound))
            (Audio|Components|Audio|FadeIn _wheelssound 1.0 1.0 0.0 :!class /Script/Engine.AudioComponent)))))))

(fn ConstructionScript
  (bind _horse2 (Variables|Default|GetHorse2))
  (bind _horse1 (Variables|Default|GetHorse1))
  (bind _horse4 (Variables|Default|GetHorse4))
  (bind _horse3 (Variables|Default|GetHorse3))
  (|CallParentFunction)
  (Utilities|FlowControl|Sequence
    (:then_0
      (if (not (== (Variables|/Script/Engine.SkinnedMeshComponent|GetSkeletalMesh _horse4) 0))
        (Class|SkinnedMeshComponent|SetMasterPoseComponent (Variables|Default|GetHair4) _horse4 false)))
    (:then_1
      (if (not (== (Variables|/Script/Engine.SkinnedMeshComponent|GetSkeletalMesh _horse3) 0))
        (Class|SkinnedMeshComponent|SetMasterPoseComponent (Variables|Default|GetHair3) _horse3 false)))
    (:then_2
      (if (not (== (Variables|/Script/Engine.SkinnedMeshComponent|GetSkeletalMesh _horse2) 0))
        (Class|SkinnedMeshComponent|SetMasterPoseComponent (Variables|Default|GetHair2) _horse2 false)))
    (:then_3
      (if (not (== (Variables|/Script/Engine.SkinnedMeshComponent|GetSkeletalMesh _horse1) 0))
        (Class|SkinnedMeshComponent|SetMasterPoseComponent (Variables|Default|GetHair1) _horse1 false)))))

(fn OnRepServerMoveStartTime
  (bind _splinerange (Variables|Default|GetSplineRange))
  (bind _targetsplineactor (Variables|Default|GetTargetSplineActor))
  (bind (_x _y) (Math|Vector2D|BreakVector2D _splinerange))
  (Utilities|IsValid _targetsplineactor
    (:Is%20Valid
      (Components|Timeline|SetPlayRate (Variables|Default|GetHorse1) (/ (/ (* (Spline|GetSplineLength (Variables|/Game/Mordhau/Blueprints/Interactables/BP_SplineActor.BP_SplineActor_C|GetSpline _targetsplineactor)) (- _y _x)) (Variables|Default|GetTimeToReachGoal)) 105.0)))))