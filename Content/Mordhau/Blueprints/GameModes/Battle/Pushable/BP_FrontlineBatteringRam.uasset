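; Pushable battering ram for Frontline that travels along a spline and plays a ramming animation when it reaches its destination.
; On cosmetic-capable instances, Tick derives wheel rotation in AB_BatteringRam from distance along the spline and fades the wheel sound in or out based on forward speed.
; Arrival sets the anim instance's play flag, and a separate DoDoorHit function triggers the linked RamDoor's animation.
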(event EventTick
  (params (DeltaSeconds :type Float%20%28single-precision%29))
  (bind _progress (Variables|Default|GetProgress))
  (bind _wheelssound (Variables|Default|GetWheelsSound))
  (bind _targetsplineactor (Variables|Default|GetTargetSplineActor))
  (bind _wheelssound_2 (Variables|Default|GetWheelsSound))
  (bind _returnvalue (Audio|Components|Audio|IsPlaying _wheelssound))
  (bind _spline (Variables|/Game/Mordhau/Blueprints/Interactables/BP_SplineActor.BP_SplineActor_C|GetSpline _targetsplineactor))
  (bind _returnvalue_2 (Spline|GetSplineLength _spline))
  (|CallParentFunction DeltaSeconds)
  (Networking|CanExecuteCosmeticEvents
    (:True
      (if (not (Math|Float|NearlyEqual(Float) DeltaSeconds 0.0 1e-06))
        (Utilities|FlowControl|Sequence
          (:then_0
            (bind _asab_battering_ram (Utilities|Casting|CastToAB_BatteringRam (Components|SkeletalMesh|GetAnimInstance (Variables|Default|GetSkeletalMesh))))
            (Variables|/Game/Mordhau/Animations/Blueprints/AB_BatteringRam.AB_BatteringRam_C|SetWheels _asab_battering_ram (Math|Rotator|MakeRotator (* (/ (* _returnvalue_2 _progress) 95.0) -1e+02) 0.0 0.0))
            (if (> (/ (* _returnvalue_2 (- _progress (Variables|Default|GetPreviousProgress))) DeltaSeconds) 1.0)
              (if (not _returnvalue)
                (Audio|Components|Audio|FadeIn _wheelssound_2 1.0 1.0 0.0 :!class /Script/Engine.AudioComponent))
              (elif _returnvalue
                (Audio|Components|Audio|FadeOut _wheelssound_2 0.2 0.0 :!class /Script/Engine.AudioComponent))))
          (:then_1
            (Variables|Default|SetPreviousProgress (Variables|Default|GetProgress))))))))

(event EventPushableArrivedatDestination
  (bind _asab_battering_ram (Utilities|Casting|CastToAB_BatteringRam (Components|SkeletalMesh|GetAnimInstance (Variables|Default|GetSkeletalMesh))))
  (Variables|/Game/Mordhau/Animations/Blueprints/AB_BatteringRam.AB_BatteringRam_C|SetPlayAnimation _asab_battering_ram 1.0))

(fn ConstructionScript
  (|CallParentFunction))

(fn DoDoorHit
  (bind _ramdoor (Variables|Default|GetRamDoor))
  (Utilities|IsValid _ramdoor
    (:Is%20Valid
      (Default|PlayAnim _ramdoor))))