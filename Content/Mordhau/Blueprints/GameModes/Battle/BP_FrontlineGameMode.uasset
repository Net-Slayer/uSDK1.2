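; Frontline game mode for Mordhau in which team scores act as ticket pools that drain as players die.
; OnKilled subtracts DeathTicketCost from the dead player's team score, clamped at zero.
; OnTeamScoreChanged ends an in-progress match when a team hits zero and records the other team as winner.
; When match time runs out, the higher score wins or equal scores give a draw, written to the game state's MatchEndInfo.
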(event EventOnTeamScoreChanged
  (params (Team :type Integer) (OldValue :type Float%20%28single-precision%29))
  (bind _asbp_mordhau_game_state (Utilities|Casting|CastToBP_MordhauGameState (Game|GetGameState)))
  (if (and (Class|GameMode|IsMatchinProgress) (== (Utilities|Array|Get(acopy) (Variables|/Script/Mordhau.MordhauGameState|GetTeamScores _asbp_mordhau_game_state) Team) 0.0))
    (Class|GameMode|EndMatch)
    (if (== Team 0)
      (Variables|/Game/Mordhau/Blueprints/GameModes/BP_MordhauGameState.BP_MordhauGameState_C|SetMatchEndInfo _asbp_mordhau_game_state (Utilities|Struct|MakeSTRUCT_MatchEndInfo 0 1 (Utilities|Array|Get(acopy) (Variables|/Script/Mordhau.MordhauGameState|GetTeamScores _asbp_mordhau_game_state) 1)))
      (else
        (Variables|/Game/Mordhau/Blueprints/GameModes/BP_MordhauGameState.BP_MordhauGameState_C|SetMatchEndInfo _asbp_mordhau_game_state (Utilities|Struct|MakeSTRUCT_MatchEndInfo 0 0 (Utilities|Array|Get(acopy) (Variables|/Script/Mordhau.MordhauGameState|GetTeamScores _asbp_mordhau_game_state))))))))

(event EventOnKilled
  (params (Killer :type Controller%20Object%20Reference) (KilledPlayer :type Controller%20Object%20Reference) (KilledPawn :type Pawn%20Object%20Reference) (Type :type EMordhauDamageType%20Enum :default "Generic") (SubType :type Byte :default 0) (DamageSource :type Actor%20Object%20Reference) (DamageAgent :type Actor%20Object%20Reference))
  (bind _deathticketcost (Variables|Default|GetDeathTicketCost))
  (|CallParentFunction Killer KilledPlayer KilledPawn Type SubType DamageSource DamageAgent)
  (Utilities|IsValid KilledPlayer
    (:Is%20Valid
      (bind _asmordhau_player_state (Utilities|Casting|CastToMordhauPlayerState (Variables|/Script/Engine.Controller|GetPlayerState KilledPlayer)))
      (bind _asmordhau_game_state (Utilities|Casting|CastToMordhauGameState (Game|GetGameState)))
      (if (== (Variables|/Script/Mordhau.MordhauPlayerState|GetTeam _asmordhau_player_state) 0)
        (Class|MordhauGameMode|SetTeamScore 0 (Math|Float|Max(Float) (- (Utilities|Array|Get(acopy) (Variables|/Script/Mordhau.MordhauGameState|GetTeamScores _asmordhau_game_state)) _deathticketcost) 0.0))
        (elif (== (Variables|/Script/Mordhau.MordhauPlayerState|GetTeam _asmordhau_player_state) 1)
          (Class|MordhauGameMode|SetTeamScore 1 (Math|Float|Max(Float) (- (Utilities|Array|Get(acopy) (Variables|/Script/Mordhau.MordhauGameState|GetTeamScores _asmordhau_game_state) 1) _deathticketcost) 0.0)))))))

(event EventBeginPlay
  (|CallParentFunction))

(event EventTick
  (params (DeltaSeconds :type Float%20%28single-precision%29)))

(event EventMatchTimeRanOut
  (|CallParentFunction)
  (bind _asbp_mordhau_game_state (Utilities|Casting|CastToBP_MordhauGameState (Game|GetGameState)))
  (if (== (Utilities|Array|Get(acopy) (Variables|/Script/Mordhau.MordhauGameState|GetTeamScores _asbp_mordhau_game_state)) (Utilities|Array|Get(acopy) (Variables|/Script/Mordhau.MordhauGameState|GetTeamScores _asbp_mordhau_game_state) 1))
    (Variables|/Game/Mordhau/Blueprints/GameModes/BP_MordhauGameState.BP_MordhauGameState_C|SetMatchEndInfo _asbp_mordhau_game_state (Utilities|Struct|MakeSTRUCT_MatchEndInfo 0 0 0.0 0.0 true))
    (elif (> (Utilities|Array|Get(acopy) (Variables|/Script/Mordhau.MordhauGameState|GetTeamScores _asbp_mordhau_game_state)) (Utilities|Array|Get(acopy) (Variables|/Script/Mordhau.MordhauGameState|GetTeamScores _asbp_mordhau_game_state) 1))
      (Variables|/Game/Mordhau/Blueprints/GameModes/BP_MordhauGameState.BP_MordhauGameState_C|SetMatchEndInfo _asbp_mordhau_game_state (Utilities|Struct|MakeSTRUCT_MatchEndInfo 0 0 (Utilities|Array|Get(acopy) (Variables|/Script/Mordhau.MordhauGameState|GetTeamScores _asbp_mordhau_game_state))))
      (else
        (Variables|/Game/Mordhau/Blueprints/GameModes/BP_MordhauGameState.BP_MordhauGameState_C|SetMatchEndInfo _asbp_mordhau_game_state (Utilities|Struct|MakeSTRUCT_MatchEndInfo 0 1 (Utilities|Array|Get(acopy) (Variables|/Script/Mordhau.MordhauGameState|GetTeamScores _asbp_mordhau_game_state) 1)))))))

(fn ConstructionScript
  (|CallParentFunction))