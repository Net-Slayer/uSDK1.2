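; Interactable Frontline objective for a peasant on Grad, freed once enough interactions accumulate.
; The construction script sets the initial animation, and the server keeps bones refreshing from BeginPlay.
; Reaching the required interactions plays the freed animation with a material dissolve timed to its length.
; When it ends, the mesh hides, loses collision and switches to ticking pose only when rendered.
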(event EventBeginPlay
  (|CallParentFunction)
  (Networking|SwitchHasAuthority
    (:Authority
      (Variables|/Script/Engine.SkinnedMeshComponent|SetMeshComponentUpdateFlag (Variables|Default|GetSkeletalMesh) "AlwaysTickPoseAndRefreshBones"))))

(event Collision|EventActorBeginOverlap
  (params (OtherActor :type Actor%20Object%20Reference))
  (|CallParentFunction OtherActor) ; This node is disabled and will not be called.\nDrag off pins to build functionality.
)

(event EventTick
  (params (DeltaSeconds :type Float%20%28single-precision%29))
  (|CallParentFunction DeltaSeconds) ; This node is disabled and will not be called.\nDrag off pins to build functionality.
)

(event EventOnInteractionsChanged
  (bind _freedanimation (Variables|Default|GetFreedAnimation))
  (bind _skeletalmesh (Variables|Default|GetSkeletalMesh))
  (if (>= (Variables|Default|GetInteractions) (Variables|Default|GetRequiredInteractions))
    (Components|Animation|PlayAnimation (Variables|Default|GetSkeletalMesh) _freedanimation false)
    (bind _returnvalue (Animation|GetPlayLength _freedanimation))
    (bind _returnvalue_2 (Rendering|Material|CreateDynamicMaterialInstance (Variables|Default|GetSkeletalMesh) 0 0 "None" :!class /Script/Engine.PrimitiveComponent))
    (Rendering|Material|SetScalarParameterValue _returnvalue_2 "DissolveDuration" _returnvalue :!class /Script/Engine.MaterialInstanceDynamic)
    (Rendering|Material|SetScalarParameterValue _returnvalue_2 "DissolveStartTime" (Utilities|Time|GetTimeSeconds) :!class /Script/Engine.MaterialInstanceDynamic)
    (Utilities|FlowControl|Delay _returnvalue)
    (Development|SetHiddeninGame _skeletalmesh true false)
    (Collision|SetCollisionEnabled _skeletalmesh "NoCollision")
    (Variables|/Script/Engine.SkinnedMeshComponent|SetMeshComponentUpdateFlag (Variables|Default|GetSkeletalMesh) "OnlyTickPoseWhenRendered")))

(fn ConstructionScript
  (|CallParentFunction)
  (Components|Animation|OverrideAnimationData (Variables|Default|GetSkeletalMesh) (Variables|Default|GetInitialAnimation) true true 0.0 1.0))