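; BP_GoldChest is an interactable objective for the Battle game mode, a gold chest that visibly empties as it is interacted with.
; Each interaction change calls the parent, then plays the coin sound and activates the coin splash effect.
; The interaction count progressively hides chalices, a plate and a book, then the gold pile once the required count is reached.
; All other events are disabled stubs, and the construction script only calls its parent.
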(event EventBeginPlay)

(event Collision|EventActorBeginOverlap
  (params (OtherActor :type Actor%20Object%20Reference))
  (|CallParentFunction OtherActor) ; This node is disabled and will not be called.\nDrag off pins to build functionality.
)

(event EventTick
  (params (DeltaSeconds :type Float%20%28single-precision%29))
  (|CallParentFunction DeltaSeconds) ; This node is disabled and will not be called.\nDrag off pins to build functionality.
)

(event EventOnInteractionsChanged
  (bind _interactions (Variables|Default|GetInteractions))
  (|CallParentFunction)
  (Audio|Components|Audio|Play (Variables|Default|GetSC_CoinObjective) 0.0)
  (Components|Activation|Activate (Variables|Default|GetP_CoinSplash) false)
  (if (> _interactions 0)
    (Transformation|SetWorldScale3D (Variables|Default|GetPile) "1.000000,1.000000,1.000000")
    (Development|SetHiddeninGame (Variables|Default|Gettr_plate_01) true false)
    (if (> _interactions 1)
      (Transformation|SetWorldScale3D (Variables|Default|GetPile) "1.000000,1.000000,1.000000")
      (Development|SetHiddeninGame (Variables|Default|Getchalice_01) true false)
      (if (>= _interactions (Variables|Default|GetRequiredInteractions))
        (Development|SetHiddeninGame (Variables|Default|GetPile) true false)))))

(fn ConstructionScript
  (|CallParentFunction))