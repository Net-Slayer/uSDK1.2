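; BP_CaptureFlag is a flag actor for the Battle game mode, with waving and capturing audio.
; The construction script assigns its WavingAudio and CapturingAudio components to the corresponding audio component variables.
; On BeginPlay, it optionally spawns a point-type WindDirectionalSource at a placement component's transform and applies its gust, speed, strength and radius settings.
; It then destroys that placement component, whether or not wind was spawned.
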(event EventBeginPlay
  (Utilities|FlowControl|Sequence
    (:then_0
      (if (Variables|Default|GetbAddWindActor)
        (bind _returnvalue (Game|SpawnActorfromClass "/Script/Engine.WindDirectionalSource" (Transformation|GetWorldTransform (Variables|Default|GetWindActorSpawnTransform)) "Undefined" 0 0))
        (bind _output_get (Variables|Default|SetWindActor _returnvalue))
        (Class|WindDirectionalSourceComponent|SetWindType (Variables|/Script/Engine.WindDirectionalSource|GetComponent _output_get) "Point")
        (Class|WindDirectionalSourceComponent|SetMaximumGustAmount (Variables|/Script/Engine.WindDirectionalSource|GetComponent _output_get) (Variables|Default|GetWindMaxGustAmount))
        (Class|WindDirectionalSourceComponent|SetMinimumGustAmount (Variables|/Script/Engine.WindDirectionalSource|GetComponent _output_get) (Variables|Default|GetWindMinGustAmount))
        (Class|WindDirectionalSourceComponent|SetSpeed (Variables|/Script/Engine.WindDirectionalSource|GetComponent _output_get) (Variables|Default|GetWindSpeed))
        (Class|WindDirectionalSourceComponent|SetStrength (Variables|/Script/Engine.WindDirectionalSource|GetComponent _output_get) (Variables|Default|GetWindStrength))
        (Control|SetRadius (Variables|/Script/Engine.WindDirectionalSource|GetComponent _output_get) (Variables|Default|GetWindRadius) :!class /Script/Engine.WindDirectionalSourceComponent)))
    (:then_1
      (Components|DestroyComponent (Variables|Default|GetWindActorSpawnTransform)))))

(fn ConstructionScript
  (Variables|Default|SetWavingAudioComponent (Variables|Default|GetWavingAudio))
  (Variables|Default|SetCapturingAudioComponent (Variables|Default|GetCapturingAudio)))