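; Frontline hero destroyable with a skeletal mesh that reacts visually to replicated health loss.
; Health changes select a damage-stage index from thresholds, then call UpdateAnimInstance, which is empty here.
; Large enough drops play a damage animation unless one is running, and zero health plays a one-time death animation after any current one ends.
; Remote instances disable overlap events on the mesh.
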(event EventBeginPlay
  (|CallParentFunction)
  (Networking|SwitchHasAuthority
    (:Remote
      (Variables|/Script/Engine.PrimitiveComponent|SetbGenerateOverlapEvents (Variables|Default|GetSkeletalMesh) false))))

(event Collision|EventActorBeginOverlap
  (params (OtherActor :type Actor%20Object%20Reference))
  (|CallParentFunction OtherActor) ; This node is disabled and will not be called.\nDrag off pins to build functionality.
)

(event EventTick
  (params (DeltaSeconds :type Float%20%28single-precision%29))
  (|CallParentFunction DeltaSeconds) ; This node is disabled and will not be called.\nDrag off pins to build functionality.
)

(event EventOnReplicatedHealthChanged
  (bind _returnvalue (Utilities|Time|GetTimeSeconds))
  (bind _replicatedhealth (Variables|Default|GetReplicatedHealth))
  (bind _damageanimation (Variables|Default|GetDamageAnimation))
  (bind _skeletalmesh (Variables|Default|GetSkeletalMesh))
  (Utilities|FlowControl|Sequence
    (:then_0
      (for (_array_element _array_index) (Variables|Default|GetDamageMeshesHealth)
        (if (<= (Variables|Default|GetReplicatedHealth) _array_element)
          (Variables|Default|SetBestDamageIdx _array_index))))
    (:then_1
      (CallFunction|UpdateAnimInstance))
    (:then_2
      (Utilities|IsValid (Variables|Default|GetDamageAnimation)
        (:Is%20Valid
          (if (Math|Boolean|ANDBoolean (>= (- (Math|Conversions|ToInteger(Byte) (Variables|Default|GetLastReplicatedHealth)) (Math|Conversions|ToInteger(Byte) _replicatedhealth)) (Math|Conversions|ToInteger(Byte) (Variables|Default|GetThresholdToPlayDamageAnimation))) (not (Variables|Default|GetPlayedDeathAnimation)) (> _replicatedhealth 0))
            (if (> (Utilities|Time|GetTimeSeconds) (Variables|Default|GetAnimTimeEnd))
              (Components|Animation|PlayAnimation _skeletalmesh _damageanimation false)
              (bind _returnvalue_2 (Animation|GetPlayLength _damageanimation))
              (Variables|Default|SetAnimTimeEnd (+ (Utilities|Time|GetTimeSeconds) _returnvalue_2)))))))
    (:then_3
      (|CallParentFunction))
    (:then_4
      (if (and (== (Variables|Default|GetReplicatedHealth) 0) (not (Variables|Default|GetPlayedDeathAnimation)))
        (Variables|Default|SetPlayedDeathAnimation true)
        (Utilities|IsValid (Variables|Default|GetDeathAnimation)
          (:Is%20Valid
            (if (< _returnvalue (Variables|Default|GetAnimTimeEnd))
              (Utilities|FlowControl|Delay (- (Variables|Default|GetAnimTimeEnd) _returnvalue)))
            (Components|Animation|PlayAnimation _skeletalmesh (Variables|Default|GetDeathAnimation) false)))))))

(fn ConstructionScript
  (|CallParentFunction))

(fn UpdateAnimInstance)