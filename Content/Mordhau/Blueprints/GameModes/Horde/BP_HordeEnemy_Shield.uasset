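; BP_HordeEnemy_Shield is a Horde mode enemy that holds up its block when its AI controller's closest enemy is near.
; On each LOD tick it holds block while that enemy is alive and close, requesting a regular parry from idle motion.
; A hold timer caps how long the block stays up and resets when attacking or starting a parry.
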(event EventBeginPlay
  (|CallParentFunction) ; This node is disabled and will not be called.\nDrag off pins to build functionality.
)

(event Collision|EventActorBeginOverlap
  (params (OtherActor :type Actor%20Object%20Reference))
  (|CallParentFunction OtherActor) ; This node is disabled and will not be called.\nDrag off pins to build functionality.
)

(event EventTick
  (params (DeltaSeconds :type Float%20%28single-precision%29))
  (|CallParentFunction DeltaSeconds) ; This node is disabled and will not be called.\nDrag off pins to build functionality.
)

(event EventBPLODTick
  (params (DeltaTime :type Float%20%28single-precision%29))
  (|CallParentFunction DeltaTime)
  (Utilities|FlowControl|Sequence
    (:then_0
      (Utilities|Casting|CastToAttackMotion (Variables|Default|GetMotion))
      (Variables|Default|SetHoldTime 0.0))
    (:then_1
      (bind _asbp_mordhau_aicontroller (Utilities|Casting|CastToBP_MordhauAIController (Pawn|GetController)))
      (bind _returnvalue (Class|MordhauAIController|GetClosestEnemy _asbp_mordhau_aicontroller))
      (Utilities|IsValid _returnvalue
        (:Is%20Valid
          (if (stale _returnvalue)
            (Variables|Default|SetbIsHoldingBlock false :!label _label)
            (elif (and (<= (Transformation|GetDistanceTo _returnvalue) 4e+02) (< (Variables|Default|GetHoldTime) 7.5))
              (Variables|Default|SetHoldTime (+ (Variables|Default|GetHoldTime) DeltaTime))
              (Variables|Default|SetbIsHoldingBlock true)
              (Utilities|Casting|CastToIdleMotion (Variables|Default|GetMotion))
              (Class|MordhauCharacter|RequestParry "Regular" false)
              (Variables|Default|SetHoldTime 0.0)
              (else
                (goto _label)))))
        (:Is%20Not%20Valid
          (goto _label))))))

(fn ConstructionScript
  (|CallParentFunction))