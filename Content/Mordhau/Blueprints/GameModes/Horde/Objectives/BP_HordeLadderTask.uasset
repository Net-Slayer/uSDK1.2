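; Horde mode task that makes characters use a ladder when triggered, valid only for characters that allow vehicles.
; If the interactable ladder has no movers and is in state 1, it toggles that state and holds the character through a delay before entering; otherwise it enters immediately.
; Entry requires a living character able to interact.
; Busy, missing or non-interactable ladders fall straight through to the parent task logic.
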(event EventBeginPlay
  (|CallParentFunction) ; This node is disabled and will not be called.\nDrag off pins to build functionality.
)

(event Collision|EventActorBeginOverlap
  (params (OtherActor :type Actor%20Object%20Reference))
  (|CallParentFunction OtherActor) ; This node is disabled and will not be called.\nDrag off pins to build functionality.
)

(event EventTick
  (params (DeltaSeconds :type Float%20%28single-precision%29))
  (|CallParentFunction DeltaSeconds) ; This node is disabled and will not be called.\nDrag off pins to build functionality.
)

(event EventTaskTriggered
  (params (Character :type BP%20Horde%20Enemy%20Object%20Reference))
  (bind _ladder (Variables|Default|GetLadder))
  (Utilities|IsValid (Variables|Default|GetWaitingToEnter)
    (:Is%20Valid
      (|CallParentFunction Character :!label _label))
    (:Is%20Not%20Valid
      (Utilities|IsValid _ladder
        (:Is%20Valid
          (if (> (Utilities|Array|Length (Variables|/Game/Mordhau/Blueprints/Interactables/SiegeEngines/BP_Ladder.BP_Ladder_C|GetMovers _ladder)) 0)
            (goto _label)
            (elif (Variables|/Script/Mordhau.MordhauActor|GetbIsInteractable _ladder)
              (if (== (Variables|/Game/Mordhau/Blueprints/Interactables/SiegeEngines/BP_Ladder.BP_Ladder_C|GetLadderState _ladder) 1)
                (Default|ToggleLadderState _ladder)
                (Variables|Default|SetWaitingToEnter Character)
                (Utilities|FlowControl|Delay 3.5)
                (Utilities|FlowControl|Sequence
                  (:then_0
                    (CallFunction|EnterLadder (Variables|Default|GetWaitingToEnter))
                    (Utilities|IsValid (Variables|Default|GetWaitingToEnter)
                      (:Is%20Valid
                        (|CallParentFunction (Variables|Default|GetWaitingToEnter)))))
                  (:then_1
                    (Variables|Default|SetWaitingToEnter 0)))
                (else
                  (CallFunction|EnterLadder Character)
                  (goto _label)))
              (else
                (goto _label)))))
        (:Is%20Not%20Valid
          (goto _label))))))

(fn ConstructionScript
  (|CallParentFunction))

(fn EnterLadder
  (params (Character :type BP%20Horde%20Enemy%20Object%20Reference))
  (Utilities|IsValid Character
    (:Is%20Valid
      (if (not (stale _returnvalue))
        (if (stale _returnvalue)
          (Class|MordhauActor|InteractionStart (Variables|Default|GetLadder) Character))))))

(fn IsTaskValidfor
  (params (Character :type BP%20Horde%20Enemy%20Object%20Reference))
  (if (Variables|/Script/Mordhau.MordhauCharacter|GetbAllowVehicles Character)
    (return (|CallParentFunction Character))
    (else
      (return false))))