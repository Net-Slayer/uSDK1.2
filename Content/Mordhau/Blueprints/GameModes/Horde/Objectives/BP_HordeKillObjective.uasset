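; Horde mode objective character on team 0 whose death triggers defeat through BP_HordeGameMode.
; On the authority, after a short delay, it spawns and possesses itself with a frontline enemy AI controller, applies a customization profile and picks up randomly customized equipment.
; A floating destroyable-style widget tracks its health and is set to slowly hide on death.
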(event EventBeginPlay
  (bind _mordhauwidget (Variables|Default|GetMordhauWidget))
  (|CallParentFunction)
  (Utilities|FlowControl|Sequence
    (:then_0
      (Utilities|IsValid _mordhauwidget
        (:Is%20Valid
          (bind _asbp_destroyable_widget_floater (Utilities|Casting|CastToBP_DestroyableWidgetFloater (UserInterface|GetUserWidgetObject _mordhauwidget)))
          (Default|UpdateHealth _asbp_destroyable_widget_floater (Math|Conversions|ToFloat(Byte) (Variables|Default|GetHealth))))))
    (:then_1
      (Networking|SwitchHasAuthority
        (:Authority
          (Utilities|FlowControl|Delay 0.2)
          (bind _returnvalue (Game|SpawnActorfromClass "/Game/Mordhau/Blueprints/GameModes/Battle/BP_FrontlineEnemyAIController.BP_FrontlineEnemyAIController_C" (Math|Transform|MakeTransform "0, 0, 0") "Undefined" 0 0))
          (bind _returnvalue_2 (Game|ConstructObjectfromClass (Variables|Default|GetBehaviorProfile) _returnvalue))
          (Variables|/Script/Mordhau.MordhauAIController|SetBehaviorProfile _returnvalue _returnvalue_2)
          (bind _returnvalue_3 (Game|SpawnActorfromClass "/Script/Mordhau.CustomizationReplicationActor" (Math|Transform|MakeTransform "0, 0, 0") "Undefined" 0 0))
          (Class|CustomizationReplicationActor|AssignDatafromProfile _returnvalue_3 (Variables|Default|GetProfileToAssign))
          (bind _output_get (Variables|/Script/Mordhau.MordhauAIController|SetCustomizationReplicationActor _returnvalue _returnvalue_3))
          (Class|MordhauCharacter|SetCustomizationReplicationActor _output_get)
          (Pawn|Possess _returnvalue self)
          (CallFunction|SpawnOurEquipment)
          (Class|MordhauCharacter|OnPostProfileAssigned))))))

(event Collision|EventActorBeginOverlap
  (params (OtherActor :type Actor%20Object%20Reference)))

(event EventTick
  (params (DeltaSeconds :type Float%20%28single-precision%29)))

(event EventOnDied
  (params (Angle :type Float%20%28single-precision%29) (Type :type EMordhauDamageType%20Enum :default "Generic") (SubType :type Byte :default 0) (Bone :type Name :default "None") (Point :type Vector :default "0, 0, 0") (Source :type Actor%20Object%20Reference) (Agent :type Actor%20Object%20Reference))
  (bind _mordhauwidget (Variables|Default|GetMordhauWidget))
  (Utilities|FlowControl|Sequence
    (:then_0
      (Variables|/Script/Mordhau.MordhauWidgetComponent|SetOverrideVisible _mordhauwidget 0)
      (Variables|/Script/Mordhau.MordhauWidgetComponent|SetbIsSlowHideOverride _mordhauwidget true)
      (Variables|/Script/Mordhau.MordhauWidgetComponent|SetVisibilityWeightInterpolationSpeed _mordhauwidget 1.0)
      (bind _asbp_destroyable_widget_floater (Utilities|Casting|CastToBP_DestroyableWidgetFloater (UserInterface|GetUserWidgetObject (Variables|Default|GetMordhauWidget))))
      (Default|UpdateHealth _asbp_destroyable_widget_floater 0.0))
    (:then_1
      (|CallParentFunction Angle Type SubType Bone Point Source Agent))
    (:then_2
      (bind _asbp_horde_game_mode (Utilities|Casting|CastToBP_HordeGameMode (Game|GetGameMode)))
      (Default|TriggerDefeat _asbp_horde_game_mode))))

(event EventOnHealthChanged
  (bind _mordhauwidget (Variables|Default|GetMordhauWidget))
  (if (not (Class|AdvancedCharacter|GetIsDead))
    (Utilities|IsValid _mordhauwidget
      (:Is%20Valid
        (bind _asbp_destroyable_widget_floater (Utilities|Casting|CastToBP_DestroyableWidgetFloater (UserInterface|GetUserWidgetObject _mordhauwidget)))
        (Default|UpdateHealth _asbp_destroyable_widget_floater (Math|Conversions|ToFloat(Byte) (Variables|Default|GetHealth)))))))

(fn ConstructionScript
  (|CallParentFunction)
  (Variables|Default|SetTeam 0))

(fn SpawnOurEquipment
  (for _array_element (Variables|Default|GetEquipmentToSpawn)
    (if (Utilities|IsValidClass _array_element)
      (bind _returnvalue (Game|SpawnActorfromClass _array_element (Math|Transform|MakeTransform "0, 0, 0") "Undefined" 0 0))
      (bind _returnvalue_2 (Class|MordhauEquipment|GetRandomCustomization _returnvalue false))
      (Class|MordhauEquipment|AssignCustomization _returnvalue _returnvalue_2)
      (Class|MordhauCharacter|PickUp _returnvalue -1))))

(fn UpdateUIWidgets
  (bind _slatebrush (Utilities|Struct|MakeSlateBrush "(X=40.000000,Y=40.000000)" "(Left=0.000000,Top=0.000000,Right=0.000000,Bottom=0.000000)" "(SpecifiedColor=(R=1.000000,G=1.000000,B=1.000000,A=1.000000),ColorUseRule=UseColor_Specified)" "/Game/Mordhau/UI/UIAssets/Textures/ic_defence_lvl1.ic_defence_lvl1" "Image" "NoTile" "NoMirror"))
  (bind _mordhauwidget (Variables|Default|GetMordhauWidget))
  (Utilities|IsValid _mordhauwidget
    (:Is%20Valid
      (bind _asbp_destroyable_widget_floater (Utilities|Casting|CastToBP_DestroyableWidgetFloater (UserInterface|GetUserWidgetObject _mordhauwidget)))
      (Variables|/Script/UMG.ProgressBar|SetWidgetStyle (Variables|/Game/Mordhau/Blueprints/GameModes/Battle/BP_DestroyableWidgetFloater.BP_DestroyableWidgetFloater_C|GetProgressBar_0 _asbp_destroyable_widget_floater) (Utilities|Struct|MakeProgressBarStyle (Utilities|Struct|MakeSlateBrush "(X=40.000000,Y=40.000000)" "(Left=0.000000,Top=0.000000,Right=0.000000,Bottom=0.000000)" (Utilities|Struct|MakeSlateColor "(R=0.025187,G=0.025187,B=0.025187,A=1.000000)") "/Game/Mordhau/UI/UIAssets/Textures/ic_defence_lvl1.ic_defence_lvl1" "Image" "NoTile" "NoMirror") _slatebrush _slatebrush)))))