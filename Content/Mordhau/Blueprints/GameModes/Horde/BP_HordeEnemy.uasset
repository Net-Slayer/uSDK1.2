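; Horde mode enemy character that picks a random valid game-mode task on spawn and damages destructibles blocking its path.
; Damage, block and parry overrides apply attacking players' skills: outgoing damage modifiers, lifesteal, leg-hit trips, stun on block and parry bypass.
; Trip, stun and timed slow effects skip bosses.
; In ModifyDamage, the fire-skill multiplier sits after the return, so it never affects the result.
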(event Custom|CompleteTask
  (Variables|Default|SetCurrentTask 0))

(event Custom|LegSweep
  (if (not (Variables|Default|GetIsBoss))
    (Utilities|FlowControl|Delay 0.001)
    (if (not (stale _returnvalue))
      (Class|AdvancedCharacter|Trip))))

(event Custom|Recoil
  (if (not (stale _returnvalue))
    (Utilities|FlowControl|Delay 0.001)
    (if (not (Variables|Default|GetIsBoss))
      (Class|MordhauCharacter|AssignNetMotionSimple (Utilities|Enum|LiteralenumEMotionType "Stunned") 127))))

(event Custom|Cripple
  (params (Duration :type Float%20%28single-precision%29))
  (bind _charactermovement (Variables|Character|GetCharacterMovement))
  (if (not (stale _returnvalue))
    (if (not (Variables|Default|GetIsBoss))
      (Utilities|FlowControl|Sequence
        (:then_0
          (if (not (Variables|Default|GetIsCrippled))
            (Variables|Default|SetPreCrippleMaxWalkSpeed (Variables|/Script/Engine.CharacterMovementComponent|GetMaxWalkSpeed _charactermovement))
            (Variables|Default|SetIsCrippled true)
            (Variables|/Script/Engine.CharacterMovementComponent|SetMaxWalkSpeed _charactermovement (* (Variables|/Script/Engine.CharacterMovementComponent|GetMaxWalkSpeed _charactermovement) 0.5))))
        (:then_1
          (Utilities|FlowControl|RetriggerableDelay Duration)
          (if (not (stale _returnvalue))
            (Variables|Default|SetIsCrippled false)
            (Variables|/Script/Engine.CharacterMovementComponent|SetMaxWalkSpeed _charactermovement (Variables|Default|GetPreCrippleMaxWalkSpeed))))))))

(event EventBeginPlay
  (|CallParentFunction)
  (Networking|SwitchHasAuthority
    (:Authority
      (bind _asbp_horde_game_mode (Utilities|Casting|CastToBP_HordeGameMode (Game|GetGameMode)))
      (if (> (Utilities|Array|Length (Variables|/Game/Mordhau/Blueprints/GameModes/Horde/BP_HordeGameMode.BP_HordeGameMode_C|GetHordeTasks _asbp_horde_game_mode)) 0)
        (bind _output_get (Variables|Default|SetCurrentTask (Utilities|Array|Get(acopy) (Variables|/Game/Mordhau/Blueprints/GameModes/Horde/BP_HordeGameMode.BP_HordeGameMode_C|GetHordeTasks _asbp_horde_game_mode) (Math|Random|RandomIntegerinRange 0 (- (Utilities|Array|Length (Variables|/Game/Mordhau/Blueprints/GameModes/Horde/BP_HordeGameMode.BP_HordeGameMode_C|GetHordeTasks _asbp_horde_game_mode)) 1)))))
        (Utilities|IsValid _output_get
          (:Is%20Valid
            (if (not (Default|IsTaskValidfor _output_get self))
              (Variables|Default|SetCurrentTask 0))))))))

(event Collision|EventActorBeginOverlap
  (params (OtherActor :type Actor%20Object%20Reference))
  (|CallParentFunction OtherActor) ; This node is disabled and will not be called.\nDrag off pins to build functionality.
)

(event EventTick
  (params (DeltaSeconds :type Float%20%28single-precision%29))
  (|CallParentFunction DeltaSeconds) ; This node is disabled and will not be called.\nDrag off pins to build functionality.
)

(event EventOnDied
  (params (Angle :type Float%20%28single-precision%29) (Type :type EMordhauDamageType%20Enum :default "Generic") (SubType :type Byte :default 0) (bone :type Name%20%28by%20ref%29 :default "None") (Point :type Vector%20%28by%20ref%29 :default "0, 0, 0") (Source :type Actor%20Object%20Reference) (Agent :type Actor%20Object%20Reference))
  (Variables|/Script/Mordhau.MordhauWidgetComponent|SetOverrideVisible (Variables|Default|GetMordhauWidget) 0)
  (|CallParentFunction Angle Type SubType bone Point Source Agent))

(event EventMoveBlockedbySlow
  (params (Impact :type Hit%20Result%20Structure%20%28by%20ref%29))
  (bind _asbp_destroyable_actor (Utilities|Casting|CastToBP_DestroyableActor (.HitActor (Collision|BreakHitResult Impact))))
  (Game|Damage|ApplyDamage _asbp_destroyable_actor (Variables|Default|GetWoodDamageForPathClearing) (Pawn|GetController) self))

(event EventMordhauDamage
  (params (Damage :type Float%20%28single-precision%29) (HitResult :type Hit%20Result%20Structure%20%28by%20ref%29) (DamageType :type EMordhauDamageType%20Enum :default "Generic") (SubDamageType :type Byte :default 0) (Source :type Actor%20Object%20Reference) (Agent :type Actor%20Object%20Reference) (EventInstigator :type Controller%20Object%20Reference))
  (bind _hitbonename (Collision|BreakHitResult HitResult))
  (|CallParentFunction Damage HitResult DamageType SubDamageType Source Agent EventInstigator)
  (if (and (Utilities|Enum|Equal(Enum) DamageType "Melee") (> Damage 0.0))
    (bind _asbp_horde_character (Utilities|Casting|CastToBP_HordeCharacter Source))
    (Utilities|FlowControl|Sequence
      (:then_0
        (if (> (Default|GetSkill _asbp_horde_character "NewEnumerator19") 0)
          (Class|AdvancedCharacter|OffsetHealth _asbp_horde_character (Math|Float|Ceil (* (Default|GetSkillFloat _asbp_horde_character "NewEnumerator19") Damage)) false)))
      (:then_1
        (if (<= (Math|Random|RandomFloat) (* (Default|GetSkillFloat _asbp_horde_character "NewEnumerator27") 0.1))
          (if (Math|Boolean|ORBoolean (Utilities|Name|Equal(Name) _hitbonename "RightFoot") (Utilities|Name|Equal(Name) _hitbonename "LeftFoot") (Utilities|Name|Equal(Name) _hitbonename "RightLeg") (Utilities|Name|Equal(Name) _hitbonename "LeftLeg"))
            (CallFunction|LegSweep)))))))

(event EventOnBlockedMelee
  (params (HitResult :type Hit%20Result%20Structure%20%28by%20ref%29) (Attacker :type Mordhau%20Character%20Object%20Reference))
  (|CallParentFunction HitResult Attacker)
  (if (not (stale _returnvalue))
    (bind _asbp_horde_character (Utilities|Casting|CastToBP_HordeCharacter Attacker))
    (Utilities|FlowControl|Sequence
      (:then_0
        (if (not (Variables|Default|GetIsBoss))
          (if (<= (Math|Random|RandomFloat) (* (Default|GetSkillFloat _asbp_horde_character "NewEnumerator29") 0.1))
            (Class|MordhauCharacter|AssignNetMotionSimple (Utilities|Enum|LiteralenumEMotionType "Stunned") 127)))))))

(fn ConstructionScript
  (|CallParentFunction))

(fn ModifyDamage
  (params (DamageAmount :type Float%20%28single-precision%29) (DamageType :type EMordhauDamageType%20Enum :default "Generic") (HitInfo :type Hit%20Result%20Structure%20%28by%20ref%29) (Source :type Actor%20Object%20Reference) (Agent :type Actor%20Object%20Reference) (EventInstigator :type Controller%20Object%20Reference))
  (bind _returnvalue (|CallParentFunction DamageAmount DamageType HitInfo Source Agent EventInstigator))
  (bind _output_get (LocalVariables|SetDamage _returnvalue))
  (Utilities|FlowControl|Sequence
    (:then_0
      (bind _asbp_horde_character (Utilities|Casting|CastToBP_HordeCharacter Source))
      (bind _outdamage (Default|ModifyOutgoingDamage _asbp_horde_character self DamageType HitInfo Agent _output_get))
      (LocalVariables|SetDamage _outdamage))
    (:then_1
      (return (LocalVariables|GetDamage)))
    (:then_2
      (if (Utilities|Enum|Equal(Enum) DamageType "Fire")
        (bind _asbp_horde_player_controller (Utilities|Casting|CastToBP_HordePlayerController EventInstigator))
        (LocalVariables|SetDamage (* (LocalVariables|GetDamage) (+ (* (Default|GetSkillLevelFloat _asbp_horde_player_controller "NewEnumerator20") 0.2) 1.0)))))))

(fn ModifyParryResult
  (params (InResult :type Boolean) (HitResult :type Hit%20Result%20Structure%20%28by%20ref%29) (Attacker :type Mordhau%20Character%20Object%20Reference))
  (Utilities|FlowControl|Sequence
    (:then_0
      (if InResult
        (bind _asbp_horde_character (Utilities|Casting|CastToBP_HordeCharacter Attacker))
        (if (Variables|/Game/Mordhau/Blueprints/Characters/BP_HordeCharacter.BP_HordeCharacter_C|GetLastAttackBypassesParry _asbp_horde_character)
          (return false))))
    (:then_1
      (return InResult))))