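; Player controller for the Battle Royale mode, handling incoming character profiles and the player's end-of-match display.
; New profiles from the client are passed through StripProfile before validation.
; When the replicated placement position updates, the local controller shows a defeat result with the placement on the HUD, then opens the Battle Royale end screen after a delay.
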(event Custom|ShowBREndScreenDelayed
  (Utilities|FlowControl|Delay 1e+01)
  (bind _asbp_battle_royale_hud (Utilities|Casting|CastToBP_BattleRoyaleHUD (Variables|Default|GetHUD)))
  (Default|ShowBattleRoyaleEndScreen _asbp_battle_royale_hud))

(event EventBeginPlay
  (|CallParentFunction) ; This node is disabled and will not be called.\nDrag off pins to build functionality.
)

(event EventTick
  (params (DeltaSeconds :type Float%20%28single-precision%29))
  (|CallParentFunction DeltaSeconds) ; This node is disabled and will not be called.\nDrag off pins to build functionality.
)

(event EventOnNewProfilefromClientPreValidation
  (|CallParentFunction)
  (Variables|Default|SetPendingCharacterProfile (Class|MordhauUtilityLibrary|StripProfile (Variables|Default|GetPendingCharacterProfile) false false false)))

(fn ConstructionScript
  (|CallParentFunction))

(fn OnRepPlacementPosition
  (if (Pawn|IsLocalPlayerController)
    (bind _asbp_mordhau_hud (Utilities|Casting|CastToBP_MordhauHUD (Class|MordhauUtilityLibrary|GetMordhauHUD)))
    (Default|ShowMatchResult _asbp_mordhau_hud false "defeat" (Utilities|Text|FormatText "Placed #{a}" (Variables|Default|GetPlacementPosition)))
    (CallFunction|ShowBREndScreenDelayed)))