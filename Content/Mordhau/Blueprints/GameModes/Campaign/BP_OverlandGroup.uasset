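; BP_OverlandGroup is a movable group actor for campaign mode, apparently an overland map unit, with click-to-move and a free camera.
; A left click traces from the cursor on Visibility, stores the hit as MoveTarget and prints a debug position.
; Tick moves the actor toward that target at constant speed, keeping its Z.
; The camera uses absolute transforms, so movement axes pan it horizontally independently of the actor.
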(event EventBeginPlay
  (Transformation|SetAbsolute (Variables|Default|GetCamera) true true true))

(event Collision|EventActorBeginOverlap
  (params (OtherActor :type Actor%20Object%20Reference)))

(event EventTick
  (params (DeltaSeconds :type Float%20%28single-precision%29))
  (bind _returnvalue (Transformation|GetActorLocation))
  (bind _movetarget (Variables|Default|GetMoveTarget))
  (bind _returnvalue_2 (Math|Interpolation|VInterptoConstant _returnvalue _movetarget DeltaSeconds 5e+03))
  (bind (_x _y) (Math|Vector|BreakVector _returnvalue_2))
  (Transformation|SetActorLocation (Math|Vector|MakeVector _x _y (.Z (Math|Vector|BreakVector _returnvalue))) false false))

(event Input|AxisEvents|InputAxisMoveForward
  (params (AxisValue :type Float%20%28single-precision%29))
  (Transformation|AddWorldOffset (Variables|Default|GetCamera) (Math|Vector|MakeVector (* AxisValue (Utilities|Time|GetWorldDeltaSeconds) 5e+03) (* (stale Input|AxisEvents|InputAxisMoveRight AxisValue) (Utilities|Time|GetWorldDeltaSeconds) 5e+03) 0.0) false false))

(event Input|AxisEvents|InputAxisMoveRight
  (params (AxisValue :type Float%20%28single-precision%29))
  (Transformation|AddWorldOffset (Variables|Default|GetCamera) (Math|Vector|MakeVector (* (stale Input|AxisEvents|InputAxisMoveForward AxisValue) (Utilities|Time|GetWorldDeltaSeconds) 5e+03) (* AxisValue (Utilities|Time|GetWorldDeltaSeconds) 5e+03) 0.0) false false))

(event Input|MouseEvents|LeftMouseButton
  (params (Key :type Key%20Structure))
  (bind _returnvalue (Game|GetPlayerController 0))
  (bind (_worldlocation _worlddirection) (Game|Player|ConvertMouseLocationToWorldSpace _returnvalue))
  (:Pressed
    (bind (_outhit _returnvalue_2) (Collision|LineTraceByChannel _worldlocation (+ _worldlocation (* _worlddirection 1e+05)) "TraceTypeQuery1" false 0 "None"))
    (if _returnvalue_2
      (Variables|Default|SetMoveTarget (.Location (Collision|BreakHitResult _outhit)))
      (Development|PrintString (Utilities|String|ToString(Vector) _worldlocation)))))

(fn ConstructionScript)