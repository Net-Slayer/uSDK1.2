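; BP_ScenarioHUD is the HUD for the Scenario game mode, extending its parent HUD with a scenario-specific widget.
; When the game state replicates, it creates BP_ScenarioHUDWidget for the local player and adds it to the viewport at a negative Z-order.
; The widget collapses for minimal HUD or while the main menu shows; hiding the menu makes it visible again without rechecking minimal mode.
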(event EventBeginPlay
  (|CallParentFunction))

(event EventOnGameStateReplicated
  (|CallParentFunction)
  (bind _returnvalue (UserInterface|CreateWidget "/Game/Mordhau/Blueprints/GameModes/Scenario/BP_ScenarioHUDWidget.BP_ScenarioHUDWidget_C" (Game|GetPlayerController 0)))
  (bind _output_get (Variables|Default|SetScenarioHUDWidget _returnvalue))
  (UserInterface|Viewport|AddtoViewport _output_get -5)
  (if (Variables|Default|GetIsHUDMinimal)
    (Widget|SetVisibility _output_get "Collapsed")))

(event EventHideMainMenu
  (|CallParentFunction)
  (Widget|SetVisibility (Variables|Default|GetScenarioHUDWidget) "Visible"))

(event EventShowMainMenu
  (params (Armory%20State :type E_ArmoryStates%20Enum :default "NewEnumerator0"))
  (|CallParentFunction Armory%20State)
  (Widget|SetVisibility (Variables|Default|GetScenarioHUDWidget) "Collapsed"))

(event EventUseMinimalHUD
  (|CallParentFunction)
  (Utilities|IsValid (Variables|Default|GetScenarioHUDWidget)
    (:Is%20Valid
      (Widget|SetVisibility (Variables|Default|GetScenarioHUDWidget) "Collapsed"))))

(event EventUseFullHUD
  (|CallParentFunction)
  (Utilities|IsValid (Variables|Default|GetScenarioHUDWidget)
    (:Is%20Valid
      (Widget|SetVisibility (Variables|Default|GetScenarioHUDWidget) "Visible"))))

(fn ConstructionScript
  (|CallParentFunction))