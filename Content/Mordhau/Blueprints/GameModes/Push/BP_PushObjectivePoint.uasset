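; Push mode objective point that reacts to changes of owning team.
; On BeginPlay and ownership change it disables both teams' spawn protection boxes, then re-enables the owner's, forcing overlaps to update in order.
; Capture by a team extends the Frontline stage timer on authority and shows added time on the local HUD.
; Ownership changes also briefly open the Push forward spawn for players stuck inside protection; announcement and spawn-switching logic is left unwired.
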(event EventBeginPlay
  (|CallParentFunction)
  (CallFunction|UpdateSpawnProtection))

(event Collision|EventActorBeginOverlap
  (params (OtherActor :type Actor%20Object%20Reference)))

(event EventTick
  (params (DeltaSeconds :type Float%20%28single-precision%29)))

(event EventOnObjectivesCompleted
  (|CallParentFunction))

(event EventEnemyGainedPrerequisites
  (|CallParentFunction))

(event EventOnOwningTeamChanged
  (bind _returnvalue (Game|GetPlayerController 0))
  (bind _timeboostoncapture (Variables|Default|GetTimeBoostOnCapture))
  (|CallParentFunction)
  (Utilities|FlowControl|Sequence
    (:then_0
      (CallFunction|UpdateSpawnProtection)
      (if (!= (Variables|Default|GetOwningTeam) 255)
        (Utilities|FlowControl|Sequence
          (:then_0
            (Networking|SwitchHasAuthority
              (:Authority
                (bind _asbp_frontline_game_state (Utilities|Casting|CastToBP_FrontlineGameState (Game|GetGameState)))
                (Variables|/Game/Mordhau/Blueprints/GameModes/Battle/BP_FrontlineGameState.BP_FrontlineGameState_C|SetStageEndTime _asbp_frontline_game_state (+ (Variables|/Game/Mordhau/Blueprints/GameModes/Battle/BP_FrontlineGameState.BP_FrontlineGameState_C|GetStageEndTime _asbp_frontline_game_state) _timeboostoncapture)))))
          (:then_1
            (Utilities|IsValid _returnvalue
              (:Is%20Valid
                (if (Pawn|IsLocalPlayerController _returnvalue)
                  (bind _asbp_frontline_hud (Utilities|Casting|CastToBP_FrontlineHUD (Class|MordhauUtilityLibrary|GetMordhauHUD)))
                  (Utilities|IsValid (Variables|/Game/Mordhau/Blueprints/GameModes/Battle/BP_FrontlineHUD.BP_FrontlineHUD_C|GetPushHUDWidget _asbp_frontline_hud)
                    (:Is%20Valid
                      (Default|AddTime (Variables|/Game/Mordhau/Blueprints/GameModes/Battle/BP_FrontlineHUD.BP_FrontlineHUD_C|GetPushHUDWidget _asbp_frontline_hud) _timeboostoncapture))))))))))
    (:then_1
      ;[1 1 1] Enable the forward spawn for those stuck inside spawn protection now
      (bind _asbp_push_game_state (Utilities|Casting|CastToBP_PushGameState (Game|GetGameState)))
      (Variables|/Game/Mordhau/Blueprints/GameModes/Push/BP_PushGameState.BP_PushGameState_C|SetForwardSpawnUntil _asbp_push_game_state (+ (Utilities|Time|GetTimeSeconds) 6.0)))))

(event EventShowPushAttackerAnnouncement)

(event EventShowPushDefenderAnnouncement)

(fn ConstructionScript
  (|CallParentFunction)
  (Variables|Default|SetCaptureArea 0))

(fn UpdateSpawnProtection
  ;[1 1 1] Disable both first, this forces the overlaps to update nicer, since we rely on a certain order (spawn protection boxes should not overlap normally, but they do in this case...)
  (for _array_element (Variables|Default|GetTeam1SpawnProtection)
    (Default|Disable _array_element))
  (for _array_element_2 (Variables|Default|GetTeam2SpawnProtection)
    (Default|Disable _array_element_2))
  (if (== (Variables|Default|GetOwningTeam) 0)
    (for _array_element_3 (Variables|Default|GetTeam1SpawnProtection)
      (Default|Enable _array_element_3))
    (elif (== (Variables|Default|GetOwningTeam) 1)
      (for _array_element_4 (Variables|Default|GetTeam2SpawnProtection)
        (Default|Enable _array_element_4)))))