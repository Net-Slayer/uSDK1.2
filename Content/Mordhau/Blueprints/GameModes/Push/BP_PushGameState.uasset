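; BP_PushGameState is the game state for the Push game mode, supplying values for the scoreboard.
; The scoreboard timer shows time left in the current stage, computed from StageEndTime minus replicated server world time and clamped at zero.
; The objective name and per-team objective value functions return empty strings, and the event graph holds no active logic.
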(event EventBeginPlay
  (|CallParentFunction) ; This node is disabled and will not be called.\nDrag off pins to build functionality.
)

(event EventTick
  (params (DeltaSeconds :type Float%20%28single-precision%29))
  (|CallParentFunction DeltaSeconds) ; This node is disabled and will not be called.\nDrag off pins to build functionality.
)

(fn ConstructionScript
  (|CallParentFunction))

(fn GetScoreboardTeamObjectiveValue
  (params (Team :type Integer))
  (return ""))

(fn GetScoreboardObjectiveName
  (return ""))

(fn GetScoreboardTimeinProgress
  (return (Math|Timespan|FromSeconds (Math|Float|Max(Float) (- (Variables|Default|GetStageEndTime) (GameState|GetServerWorldTimeSeconds)) 0.0))))