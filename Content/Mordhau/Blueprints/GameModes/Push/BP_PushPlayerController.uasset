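; Player controller for the Push game mode that announces the current objective on the Frontline HUD.
; After possessing a character with no last vehicle time, it shows the announcement if the match has started.
; ShowCurrentObjective can play a horn, then shows "Survive" for kill-objective pawns.
; Otherwise, it finds the capture point open to the attacking team and picks its attacker or defender text based on the player's team.
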(event EventBeginPlay
  (|CallParentFunction) ; This node is disabled and will not be called.\nDrag off pins to build functionality.
)

(event EventTick
  (params (DeltaSeconds :type Float%20%28single-precision%29))
  (|CallParentFunction DeltaSeconds) ; This node is disabled and will not be called.\nDrag off pins to build functionality.
)

(event EventOnAfterPossess
  (params (APawn :type Pawn%20Object%20Reference))
  (Utilities|FlowControl|Sequence
    (:then_0
      (bind _asmordhau_character (Utilities|Casting|CastToMordhauCharacter APawn))
      (if (== (Variables|/Script/Mordhau.MordhauCharacter|GetLastVehicleTime _asmordhau_character) 0.0)
        (bind _asbp_frontline_game_state (Utilities|Casting|CastToBP_FrontlineGameState (Game|GetGameState)))
        (if (Class|GameStateBase|HasMatchStarted _asbp_frontline_game_state)
          (CallFunction|ShowCurrentObjective false))))
    (:then_1
      (|CallParentFunction APawn))))

(fn ConstructionScript
  (|CallParentFunction))

(fn ShowCurrentObjective
  (params (PlayHorn :type Boolean))
  (bind _returnvalue (Utilities|Text|MakeLiteralText "CURRENT OBJECTIVE"))
  (bind _asbp_frontline_hud (Utilities|Casting|CastToBP_FrontlineHUD (Class|MordhauUtilityLibrary|GetMordhauHUD)))
  (bind _asmordhau_character (Utilities|Casting|CastToMordhauCharacter (Pawn|GetControlledPawn)))
  (Utilities|FlowControl|Sequence
    (:then_0
      (if PlayHorn
        (Audio|PlaySound2D 0 1.0 1.0 0.0 0 0)))
    (:then_1
      (Utilities|Casting|CastToBP_FrontlineKillObjective _asmordhau_character
        (:then
          (Default|ShowAnnouncement _asbp_frontline_hud _returnvalue "Survive" 4.0))
        (:CastFailed
          (bind _asbp_push_game_state (Utilities|Casting|CastToBP_PushGameState (Game|GetGameState)))
          (bind _asmordhau_player_state (Utilities|Casting|CastToMordhauPlayerState (Variables|Default|GetPlayerState)))
          (bind _array_element (Utilities|Array|ForEachLoopwithBreak (Variables|/Script/Mordhau.MordhauGameState|GetAllCapturePoints _asbp_push_game_state) :!label _label)
            (:LoopBody
              (bind _asbp_push_objective_point (Utilities|Casting|CastToBP_PushObjectivePoint _array_element))
              (if (and (Utilities|Select :Index (Variables|/Game/Mordhau/Blueprints/GameModes/Battle/BP_FrontlineGameState.BP_FrontlineGameState_C|GetAttackingTeam _asbp_push_game_state) :Option%200 (Variables|/Script/Mordhau.ControlPoint|GetbTeam1OwnsPrerequisites _array_element) :Option%201 (Variables|/Script/Mordhau.ControlPoint|GetbTeam2OwnsPrerequisites _array_element)) (!= (Variables|/Script/Mordhau.ControlPoint|GetOwningTeam _array_element) (Variables|/Game/Mordhau/Blueprints/GameModes/Battle/BP_FrontlineGameState.BP_FrontlineGameState_C|GetAttackingTeam _asbp_push_game_state)))
                (if (== (Variables|/Script/Mordhau.MordhauPlayerState|GetTeam _asmordhau_player_state) (Math|Conversions|ToInteger(Byte) (Utilities|Select :Index (Variables|/Game/Mordhau/Blueprints/GameModes/Battle/BP_FrontlineGameState.BP_FrontlineGameState_C|GetAttackingTeam _asbp_push_game_state) :Option%200 1 :Option%201 0)))
                  (LocalVariables|SetTextToShow (Variables|/Game/Mordhau/Blueprints/GameModes/Push/BP_PushObjectivePoint.BP_PushObjectivePoint_C|GetAnnouncementDefendersText _asbp_push_objective_point))
                  (goto _label Break)
                  (else
                    (LocalVariables|SetTextToShow (Variables|/Game/Mordhau/Blueprints/GameModes/Push/BP_PushObjectivePoint.BP_PushObjectivePoint_C|GetAnnouncementAttackersText _asbp_push_objective_point))
                    (goto _label Break)))))
            (:Completed
              (Default|ShowAnnouncement _asbp_frontline_hud _returnvalue (LocalVariables|GetTextToShow) 4.0))))))))