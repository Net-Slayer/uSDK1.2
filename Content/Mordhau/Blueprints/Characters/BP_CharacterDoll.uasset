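; BP_CharacterDoll is a character Blueprint that strikes preview poses based on its held equipment.
; AssumePreviewPose prefers left-hand equipment over right, then uses the Random input modulo the array length to pick one of that item's preview pose montages.
; Without a valid pose, it falls back to an unarmed pose, empties the hands and flags an instant anim switch before playing the montage.
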(fn ConstructionScript
  (|CallParentFunction))

(fn AssumePreviewPose
  (params (Random :type Integer))
  (bind _lefthandequipment (Variables|Default|GetLeftHandEquipment))
  (bind _unarmedpreviewposes (Variables|Default|GetUnarmedPreviewPoses))
  (bind _returnvalue (Utilities|Array|Length _unarmedpreviewposes))
  (Utilities|FlowControl|Sequence
    (:then_0
      (Utilities|IsValid _lefthandequipment
        (:Is%20Valid
          (LocalVariables|SetEqToUse _lefthandequipment))
        (:Is%20Not%20Valid
          (LocalVariables|SetEqToUse (Variables|Default|GetRightHandEquipment)))))
    (:then_1
      (Utilities|IsValid (LocalVariables|GetEqToUse)
        (:Is%20Valid
          (if (> (Utilities|Array|Length (Variables|/Script/Mordhau.MordhauEquipment|GetCharacterPreviewPoses (LocalVariables|GetEqToUse))) 0)
            (LocalVariables|SetPoseToUse (Utilities|Array|Get(acopy) (Variables|/Script/Mordhau.MordhauEquipment|GetCharacterPreviewPoses (LocalVariables|GetEqToUse)) (Math|Integer|%(Integer) Random (Utilities|Array|Length (Variables|/Script/Mordhau.MordhauEquipment|GetCharacterPreviewPoses (LocalVariables|GetEqToUse))))))))))
    (:then_2
      (Utilities|IsValid (LocalVariables|GetPoseToUse)
        (:Is%20Not%20Valid
          (if (> _returnvalue 0)
            (LocalVariables|SetPoseToUse (Utilities|Array|Get(acopy) _unarmedpreviewposes (Math|Integer|%(Integer) Random _returnvalue)))
            (Class|MordhauCharacter|EmptyHands)
            (bind _asmordhau_anim_instance (Utilities|Casting|CastToMordhauAnimInstance (Components|SkeletalMesh|GetAnimInstance (Variables|Character|GetMesh))))
            (Variables|/Script/Mordhau.MordhauAnimInstance|SetbShouldPerformInstantAnimSwitch _asmordhau_anim_instance true)))))
    (:then_3
      (Utilities|IsValid (LocalVariables|GetPoseToUse)
        (:Is%20Valid
          (Animation|PlayAnimMontage (LocalVariables|GetPoseToUse) 1.0 "None"))))))