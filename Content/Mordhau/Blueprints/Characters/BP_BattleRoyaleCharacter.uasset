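; Battle Royale character Blueprint that tracks head, chest and leg armor picked up as wearable pickup classes.
; On death, unless equipment is destroyed, it spawns each armor piece as a pickup at the character's transform.
; RepNotifies on each armor slot play the pickup's equip sound, read from its class default object.
; For the local player, they also flash the matching HUD armor widget in either the Battle Royale or Horde HUD.
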(event EventBeginPlay
  (|CallParentFunction) ; This node is disabled and will not be called.\nDrag off pins to build functionality.
)

(event Collision|EventActorBeginOverlap
  (params (OtherActor :type Actor%20Object%20Reference)))

(event EventTick
  (params (DeltaSeconds :type Float%20%28single-precision%29)))

(event EventOnKilled
  (params (EventInstigator :type Controller%20Object%20Reference))
  (Utilities|FlowControl|Sequence
    (:then_0
      (if (not (Variables|Default|GetbDestroyEquipmentOnDeath))
        (Utilities|FlowControl|Sequence
          (:then_0
            (CallFunction|SpawnArmorPiece (Variables|Default|GetHeadArmor)))
          (:then_1
            (CallFunction|SpawnArmorPiece (Variables|Default|GetChestArmor)))
          (:then_2
            (CallFunction|SpawnArmorPiece (Variables|Default|GetLegArmor))))))
    (:then_1
      (|CallParentFunction EventInstigator))))

(fn ConstructionScript
  (|CallParentFunction))

(fn SpawnArmorPiece
  (params (WearablePickupClass :type BP%20Wearable%20Pickup%20Class%20Reference))
  (if (Utilities|IsValidClass WearablePickupClass)
    (Game|SpawnActorfromClass WearablePickupClass (Transformation|GetActorTransform) "Undefined" 0 0)))

(fn OnRepHeadArmor
  (CallFunction|PlayWearablePickupSound (Variables|Default|GetHeadArmor))
  (CallFunction|OnArmorReplicated "Head"))

(fn OnRepChestArmor
  (CallFunction|PlayWearablePickupSound (Variables|Default|GetChestArmor))
  (CallFunction|OnArmorReplicated "UpperChest"))

(fn OnRepLegArmor
  (CallFunction|PlayWearablePickupSound (Variables|Default|GetLegArmor))
  (CallFunction|OnArmorReplicated "Legs"))

(fn PlayWearablePickupSound
  (params (Wearable :type BP%20Wearable%20Pickup%20Class%20Reference))
  (bind _asbp_wearable_pickup (Utilities|Casting|CastToBP_WearablePickup (Class|MordhauUtilityLibrary|GetDefaultActor Wearable)))
  (Class|AdvancedCharacter|PlayCharacterSound (Variables|/Game/Mordhau/Blueprints/Interactables/WearablePickups/BP_WearablePickup.BP_WearablePickup_C|GetEquipSound _asbp_wearable_pickup) "Spine1" (Math|Vector|MakeVector 0.0 0.0 0.0) "0, 0, 0" false 0 0.0 0.0))

(fn OnArmorReplicated
  (params (Slot :type EWearableSlot%20Enum :default "Head"))
  (bind _returnvalue (Class|MordhauUtilityLibrary|GetMordhauHUD))
  (bind _asmordhau_player_controller (Utilities|Casting|CastToMordhauPlayerController (Pawn|GetController)))
  (if (Pawn|IsLocalPlayerController _asmordhau_player_controller)
    (bind _asbp_battle_royale_hud (Utilities|Casting|CastToBP_BattleRoyaleHUD _returnvalue)
      (:then
        (switch Utilities|FlowControl|Switch|SwitchonEWearableSlot Slot
          (:Head
            (Default|Flash (Variables|/Game/Mordhau/Blueprints/GameModes/BattleRoyale/BP_BattleRoyaleHUDWidget.BP_BattleRoyaleHUDWidget_C|GetHeadArmor (Variables|/Game/Mordhau/Blueprints/GameModes/BattleRoyale/BP_BattleRoyaleHUD.BP_BattleRoyaleHUD_C|GetBattleRoyaleHUDWidget _asbp_battle_royale_hud))))
          (:UpperChest
            (Default|Flash (Variables|/Game/Mordhau/Blueprints/GameModes/BattleRoyale/BP_BattleRoyaleHUDWidget.BP_BattleRoyaleHUDWidget_C|GetTorsoArmor (Variables|/Game/Mordhau/Blueprints/GameModes/BattleRoyale/BP_BattleRoyaleHUD.BP_BattleRoyaleHUD_C|GetBattleRoyaleHUDWidget _asbp_battle_royale_hud))))
          (:Legs
            (Default|Flash (Variables|/Game/Mordhau/Blueprints/GameModes/BattleRoyale/BP_BattleRoyaleHUDWidget.BP_BattleRoyaleHUDWidget_C|GetLegArmor (Variables|/Game/Mordhau/Blueprints/GameModes/BattleRoyale/BP_BattleRoyaleHUD.BP_BattleRoyaleHUD_C|GetBattleRoyaleHUDWidget _asbp_battle_royale_hud))))))
      (:CastFailed
        (bind _asbp_horde_hud (Utilities|Casting|CastToBP_HordeHUD _returnvalue))
        (switch Utilities|FlowControl|Switch|SwitchonEWearableSlot Slot
          (:Head
            (Default|Flash (Variables|/Game/Mordhau/Blueprints/GameModes/Horde/BP_HordeHUDWidget.BP_HordeHUDWidget_C|GetHeadArmor (Variables|/Game/Mordhau/Blueprints/GameModes/Horde/BP_HordeHUD.BP_HordeHUD_C|GetHordeHUDWidget _asbp_horde_hud))))
          (:UpperChest
            (Default|Flash (Variables|/Game/Mordhau/Blueprints/GameModes/Horde/BP_HordeHUDWidget.BP_HordeHUDWidget_C|GetTorsoArmor (Variables|/Game/Mordhau/Blueprints/GameModes/Horde/BP_HordeHUD.BP_HordeHUD_C|GetHordeHUDWidget _asbp_horde_hud))))
          (:Legs
            (Default|Flash (Variables|/Game/Mordhau/Blueprints/GameModes/Horde/BP_HordeHUDWidget.BP_HordeHUDWidget_C|GetLegArmor (Variables|/Game/Mordhau/Blueprints/GameModes/Horde/BP_HordeHUD.BP_HordeHUD_C|GetHordeHUDWidget _asbp_horde_hud)))))))))