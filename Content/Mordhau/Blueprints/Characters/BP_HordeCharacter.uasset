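; BP_HordeCharacter is the Horde mode player character, turning a replicated skill array into combat and movement perks.
; ApplySkills sets stats like speed, dodge and kill healing, plus shield blocking on authority.
; Damage hooks and melee events add skill-scaled multipliers, mitigation, chip damage and random crit, recoil or parry-bypass rolls.
; It saves armor changes and death-time equipment with ammo to BP_HordePlayerController, and plays a sound when other characters die.
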(event EventBeginPlay
  (|CallParentFunction))

(event Collision|EventActorBeginOverlap
  (params (OtherActor :type Actor%20Object%20Reference))
  (|CallParentFunction OtherActor) ; This node is disabled and will not be called.\nDrag off pins to build functionality.
)

(event EventTick
  (params (DeltaSeconds :type Float%20%28single-precision%29))
  (|CallParentFunction DeltaSeconds) ; This node is disabled and will not be called.\nDrag off pins to build functionality.
)

(event EventOnDied
  (params (Angle :type Float%20%28single-precision%29) (Type :type EMordhauDamageType%20Enum :default "Generic") (SubType :type Byte :default 0) (bone :type Name%20%28by%20ref%29 :default "None") (Point :type Vector%20%28by%20ref%29 :default "0, 0, 0") (Source :type Actor%20Object%20Reference) (Agent :type Actor%20Object%20Reference))
  (Utilities|FlowControl|Sequence
    (:then_0
      (bind _asmordhau_player_controller (Utilities|Casting|CastToMordhauPlayerController (Game|GetPlayerController 0)))
      (if (Pawn|IsLocalPlayerController _asmordhau_player_controller)
        (bind _returnvalue (Class|MordhauPlayerController|GetLastControlledCharacter _asmordhau_player_controller))
        (Utilities|IsValid _returnvalue
          (:Is%20Valid
            (if (!= _returnvalue self)
              (Audio|PlaySound2D 0 1.0 1.0 0.0 0 0 :!label _label)))
          (:Is%20Not%20Valid
            (goto _label)))))
    (:then_1
      (|CallParentFunction Angle Type SubType bone Point Source Agent))))

(event EventOnArmorReplicated
  (params (Slot :type EWearableSlot%20Enum :default "Head"))
  (|CallParentFunction Slot)
  (bind _asbp_horde_player_controller (Utilities|Casting|CastToBP_HordePlayerController (Pawn|GetController)))
  (if (Ability|HasAuthority _asbp_horde_player_controller)
    (switch Utilities|FlowControl|Switch|SwitchonEWearableSlot Slot
      (:Head
        (Variables|/Game/Mordhau/Blueprints/GameModes/Horde/BP_HordePlayerController.BP_HordePlayerController_C|SetLastHeadArmor _asbp_horde_player_controller (Variables|Default|GetHeadArmor)))
      (:UpperChest
        (Variables|/Game/Mordhau/Blueprints/GameModes/Horde/BP_HordePlayerController.BP_HordePlayerController_C|SetLastChestArmor _asbp_horde_player_controller (Variables|Default|GetChestArmor)))
      (:Legs
        (Variables|/Game/Mordhau/Blueprints/GameModes/Horde/BP_HordePlayerController.BP_HordePlayerController_C|SetLastLegArmor _asbp_horde_player_controller (Variables|Default|GetLegArmor))))))

(event EventOnKilled
  (params (EventInstigator :type Controller%20Object%20Reference))
  (Utilities|FlowControl|Sequence
    (:then_0
      (bind _asbp_horde_player_controller (Utilities|Casting|CastToBP_HordePlayerController (Pawn|GetController)))
      (Utilities|Array|Clear (Variables|/Game/Mordhau/Blueprints/GameModes/Horde/BP_HordePlayerController.BP_HordePlayerController_C|GetLastEquipment _asbp_horde_player_controller))
      (Utilities|Array|Clear (Variables|/Game/Mordhau/Blueprints/GameModes/Horde/BP_HordePlayerController.BP_HordePlayerController_C|GetLastEquipmentAmmo _asbp_horde_player_controller))
      (for _array_element (Variables|Default|GetEquipment)
        (Utilities|IsValid _array_element
          (:Is%20Valid
            (Utilities|Casting|CastToFistsWeapon _array_element
              (:then
                (Utilities|Array|Add (Variables|/Game/Mordhau/Blueprints/GameModes/Horde/BP_HordePlayerController.BP_HordePlayerController_C|GetLastEquipment _asbp_horde_player_controller) 0 :!label _label)
                (Utilities|Array|Add (Variables|/Game/Mordhau/Blueprints/GameModes/Horde/BP_HordePlayerController.BP_HordePlayerController_C|GetLastEquipmentAmmo _asbp_horde_player_controller) 0))
              (:CastFailed
                (Utilities|Array|Add (Variables|/Game/Mordhau/Blueprints/GameModes/Horde/BP_HordePlayerController.BP_HordePlayerController_C|GetLastEquipment _asbp_horde_player_controller) (Utilities|GetClass _array_element))
                (Utilities|Array|Add (Variables|/Game/Mordhau/Blueprints/GameModes/Horde/BP_HordePlayerController.BP_HordePlayerController_C|GetLastEquipmentAmmo _asbp_horde_player_controller) (Class|MordhauEquipment|GetAmmo _array_element)))))
          (:Is%20Not%20Valid
            (goto _label)))))
    (:then_1
      (|CallParentFunction EventInstigator))))

(event EventOnPickedUp
  (params (Eq :type Mordhau%20Equipment%20Object%20Reference))
  (|CallParentFunction Eq)
  (CallFunction|ApplySkillstoEquipment Eq))

(event EventOnBlockedMelee
  (params (HitResult :type Hit%20Result%20Structure%20%28by%20ref%29) (Attacker :type Mordhau%20Character%20Object%20Reference))
  (|CallParentFunction HitResult Attacker)
  (bind _asbp_horde_enemy (Utilities|Casting|CastToBP_HordeEnemy Attacker))
  (if (<= (Math|Random|RandomFloat) (* (CallFunction|GetSkillFloat "NewEnumerator28") 0.1))
    (Default|Recoil _asbp_horde_enemy)))

(event EventOnAttackStarted
  (bind _lastattackmotion (Variables|Default|GetLastAttackMotion))
  (|CallParentFunction)
  (Variables|Default|SetLastAttackBypassesParry false)
  (Utilities|IsValid _lastattackmotion
    (:Is%20Valid
      (bind _structout (Utilities|Struct|SetmembersinAttackInfo (Variables|/Script/Mordhau.AttackMotion|GetAttackInfo _lastattackmotion) (+ (.ChipDamagePercentageOnBlock (Utilities|Struct|BreakAttackInfo (Variables|/Script/Mordhau.AttackMotion|GetAttackInfo _lastattackmotion))) (* (CallFunction|GetSkillFloat "NewEnumerator31") 0.1))))
      (Variables|/Script/Mordhau.AttackMotion|SetAttackInfo _lastattackmotion _structout)
      (if (Utilities|Enum|Equal(Enum) (Variables|/Script/Mordhau.AttackMotion|GetType _lastattackmotion) "Riposte")
        (if (<= (Math|Random|RandomFloat) (* (CallFunction|GetSkillFloat "NewEnumerator30") 0.2))
          (Variables|Default|SetLastAttackBypassesParry true))))))

(fn ConstructionScript
  (|CallParentFunction))

(fn OnRepReplicatedSkills)

(fn GetSkill
  (params (Skill :type E_HordeSkill%20Enum :default "NewEnumerator0"))
  (bind _returnvalue (Math|Conversions|ToInteger(Byte) Skill))
  (bind _replicatedskills (Variables|Default|GetReplicatedSkills))
  (if (Utilities|Array|IsValidIndex _replicatedskills _returnvalue)
    (return (Utilities|Array|Get(acopy) _replicatedskills _returnvalue))
    (else
      (return 0))))

(fn ApplySkills
  (bind _level (CallFunction|GetSkill "NewEnumerator3"))
  (Utilities|FlowControl|Sequence
    (:then_0
      (Utilities|FlowControl|Sequence
        (:then_0
          (Variables|Default|SetLastChanceHealAmount (select (> _level 1) (* _level 25) 1)))
        (:then_1
          (Variables|/Script/Engine.CharacterMovementComponent|SetMaxWalkSpeed (Variables|Character|GetCharacterMovement) (* (CallFunction|GetSkillFloat "NewEnumerator2") 7.0)))
        (:then_2
          (Variables|Default|SetbCanJumpKick (> (CallFunction|GetSkill "NewEnumerator18") 0)))
        (:then_3
          (if (> (CallFunction|GetSkill "NewEnumerator5") 0)
            (Variables|Default|SetbCanDodge true)
            (Variables|Default|SetDodgeDuration (+ 0.35 (* (CallFunction|GetSkillFloat "NewEnumerator5") 0.02)))))
        (:then_4
          (Variables|Default|SetUnflinchableDamageThreshold (* (CallFunction|GetSkillFloat "NewEnumerator7") 12.0)))
        (:then_5
          (Variables|Default|SetReflectMeleeDamagePercentage (* (CallFunction|GetSkillFloat "NewEnumerator8") 2e+01)))
        (:then_6
          (Variables|Default|SetMeleeWindupModifier (- 1.0 (* (CallFunction|GetSkillFloat "NewEnumerator9") 0.04))))
        (:then_7
          (Variables|Default|SetHealthOnKill (Math|Float|Ceil (+ (* (* (CallFunction|GetSkillFloat "NewEnumerator22") 0.1) 25.0) 25.0))))))
    (:then_1
      (Networking|SwitchHasAuthority
        (:Authority
          (for _array_element (Variables|Default|GetEquipment)
            (CallFunction|ApplySkillstoEquipment _array_element)))))))

(fn RoundEnded
  (if (> (CallFunction|GetSkill "NewEnumerator3") 0)
    (Variables|Default|SetbHasLastChance true)))

(fn GetSkillFloat
  (params (Skill :type E_HordeSkill%20Enum :default "NewEnumerator0"))
  (return (Math|Conversions|ToFloat(Byte) (CallFunction|GetSkill Skill))))

(fn ModifyOutgoingDamage
  (params (Receiver :type Actor%20Object%20Reference) (DamageType :type EMordhauDamageType%20Enum :default "Generic") (HitInfo :type Hit%20Result%20Structure%20%28by%20ref%29) (Agent :type Actor%20Object%20Reference) (InDamage :type Float%20%28single-precision%29))
  (bind _righthandequipment (Variables|Default|GetRightHandEquipment))
  (Utilities|FlowControl|Sequence
    (:then_0
      (if (Utilities|Enum|Equal(Enum) DamageType "Melee")
        (Utilities|FlowControl|Sequence
          (:then_0
            (if (<= (Math|Random|RandomFloat) (* (CallFunction|GetSkillFloat "NewEnumerator6") 0.05))
              (LocalVariables|SetMultiplier (+ (LocalVariables|GetMultiplier) 1.0))))
          (:then_1
            (LocalVariables|SetMultiplier (+ (* (- 1e+02 (Math|Conversions|ToFloat(Byte) (Variables|Default|GetHealth))) (CallFunction|GetSkillFloat "NewEnumerator10") 0.002) (LocalVariables|GetMultiplier)))
            (bind _asmordhau_equipment (Utilities|Casting|CastToMordhauEquipment Agent))
            (if (Variables|/Script/Mordhau.MordhauEquipment|GetbIsTwoHanded _asmordhau_equipment)
              (LocalVariables|SetMultiplier (+ (* (CallFunction|GetSkillFloat "NewEnumerator14") 0.05) (LocalVariables|GetMultiplier)))
              (else
                (bind _asattack_motion (Utilities|Casting|CastToAttackMotion (Variables|Default|GetMotion)))
                (if (or (Utilities|Enum|Equal(Enum) (Variables|/Script/Mordhau.AttackMotion|GetMove _asattack_motion) "RightStrike") (Utilities|Enum|Equal(Enum) (Variables|/Script/Mordhau.AttackMotion|GetMove _asattack_motion) "LeftStrike"))
                  (LocalVariables|SetMultiplier (+ (* (CallFunction|GetSkillFloat "NewEnumerator12") 0.1) (LocalVariables|GetMultiplier)))
                  (elif (or (Utilities|Enum|Equal(Enum) (Variables|/Script/Mordhau.AttackMotion|GetMove _asattack_motion) "Stab") (Utilities|Enum|Equal(Enum) (Variables|/Script/Mordhau.AttackMotion|GetMove _asattack_motion) "AltStab"))
                    (LocalVariables|SetMultiplier (+ (* (CallFunction|GetSkillFloat "NewEnumerator13") 0.1) (LocalVariables|GetMultiplier)))
                    (elif (Utilities|Enum|Equal(Enum) (Variables|/Script/Mordhau.AttackMotion|GetMove _asattack_motion) "Kick")
                      (LocalVariables|SetMultiplier (+ (LocalVariables|GetMultiplier) (* (CallFunction|GetSkillFloat "NewEnumerator18") 0.2)))))))))
          (:then_2
            (if (> (Class|KismetMathLibrary|DegAcos (Math|Vector|DotProduct (Transformation|GetActorForwardVector Receiver) (Math|Vector|Normalize (Math|Conversions|ToVector(Vector2D) (Math|Conversions|ToVector2D(Vector) (- (Transformation|GetActorLocation Receiver) (Transformation|GetActorLocation))))))) 9e+01)
              (LocalVariables|SetMultiplier (+ (* (CallFunction|GetSkillFloat "NewEnumerator21") 0.2) (LocalVariables|GetMultiplier))))))
        (elif (Utilities|Enum|Equal(Enum) DamageType "Ranged")
          (Utilities|FlowControl|Sequence
            (:then_0
              (if (Utilities|Name|Equal(Name) (.HitBoneName (Collision|BreakHitResult HitInfo)) "head")
                (LocalVariables|SetMultiplier (+ (* (CallFunction|GetSkillFloat "NewEnumerator23") 0.1) (LocalVariables|GetMultiplier)))))
            (:then_1
              (if (<= (Math|Random|RandomFloat) (* (CallFunction|GetSkillFloat "NewEnumerator24") 0.05))
                (LocalVariables|SetMultiplier (+ (LocalVariables|GetMultiplier) 1.0))))
            (:then_2
              (Utilities|Casting|CastToBP_Crossbow _righthandequipment
                (:then
                  (LocalVariables|SetMultiplier (+ (* (CallFunction|GetSkillFloat "NewEnumerator25") 0.1) (LocalVariables|GetMultiplier))))
                (:CastFailed
                  (Utilities|Casting|CastToBP_Bow _righthandequipment)
                  (LocalVariables|SetMultiplier (+ (* (CallFunction|GetSkillFloat "NewEnumerator26") 0.1) (LocalVariables|GetMultiplier))))))))))
    (:then_1
      (return (* InDamage (LocalVariables|GetMultiplier))))))

(fn ApplySkillstoEquipment
  (params (Equip :type Mordhau%20Equipment%20Object%20Reference))
  (bind _asmordhau_shield (Utilities|Casting|CastToMordhauShield Equip))
  (Variables|/Script/Mordhau.MordhauShield|SetPassiveBlockDamageModifier _asmordhau_shield (- 1.0 (* (CallFunction|GetSkillFloat "NewEnumerator15") 0.2))))

(fn ModifyDamage
  (params (DamageAmount :type Float%20%28single-precision%29) (DamageType :type EMordhauDamageType%20Enum :default "Generic") (HitInfo :type Hit%20Result%20Structure%20%28by%20ref%29) (Source :type Actor%20Object%20Reference) (Agent :type Actor%20Object%20Reference) (EventInstigator :type Controller%20Object%20Reference))
  (bind _charactermovement (Variables|Character|GetCharacterMovement))
  (Utilities|FlowControl|Sequence
    (:then_0
      (Utilities|Casting|CastToMordhauShield (Variables|Default|GetLeftHandEquipment)
        (:then
          (Variables|Default|SetReceivedDamageAbsorption (* (CallFunction|GetSkillFloat "NewEnumerator16") 3.0)))
        (:CastFailed
          (Variables|Default|SetReceivedDamageAbsorption 0.0))))
    (:then_1
      (bind _asmordhau_movement_component (Utilities|Casting|CastToMordhauMovementComponent _charactermovement))
      (Variables|Default|SetReceivedDamageModifier (- 1.0 (+ (* (CallFunction|GetSkillFloat "NewEnumerator1") 0.05) (select (< (Math|Vector|VectorLength (Transformation|GetVelocity)) (+ (* (Variables|/Script/Engine.CharacterMovementComponent|GetMaxWalkSpeed _charactermovement) (stale _returnvalue)) 1e+01)) (* (CallFunction|GetSkillFloat "NewEnumerator17") 0.05) 0.0)))))
    (:then_2
      (return DamageAmount))))