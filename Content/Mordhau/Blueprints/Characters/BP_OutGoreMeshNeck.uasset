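; BP_OutGoreMeshNeck is a neck gore mesh Blueprint that leaves blood decals where its particles hit surfaces.
; On particle collision, it spawns a long-lived blood decal through MordhauUtilityLibrary, facing into the hit surface, then sets its fade screen size and sort order.
; A dynamic material instance randomizes Row and Column parameters to vary each splat, likely from a texture atlas.
; The construction script only calls the parent.
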(event OnParticleCollide(Particle)
  (params (EventName :type Name :default "None") (EmitterTime :type Float%20%28single-precision%29) (ParticleTime :type Integer) (Location :type Vector :default "0, 0, 0") (Velocity :type Vector :default "0, 0, 0") (Direction :type Vector :default "0, 0, 0") (Normal :type Vector :default "0, 0, 0") (BoneName :type Name :default "None") (PhysMat :type Physical%20Material%20Object%20Reference))
  (bind _returnvalue (Math|Vector|MakeVector 0.0 0.0 0.0))
  (bind _returnvalue_2 (* Normal -1.0))
  (bind _returnvalue_3 (Math|Rotator|MakeRotfromX _returnvalue_2))
  (bind _returnvalue_4 (Class|MordhauUtilityLibrary|SpawnBloodDecalatLocation "/Script/Mordhau.Default__MordhauUtilityLibrary" 0 0 _returnvalue Location _returnvalue_3 9e+01))
  (Utilities|IsValid _returnvalue_4
    (:Is%20Valid
      (Class|MordhauUtilityLibrary|SetDecalFadeScreenSize _returnvalue_4 0.05)
      (Class|DecalComponent|SetSortOrder _returnvalue_4 1)
      (bind _returnvalue_5 (Rendering|Material|CreateDynamicMaterialInstance _returnvalue_4 :!class /Script/Engine.DecalComponent))
      (Rendering|Material|SetScalarParameterValue _returnvalue_5 "Row" (Math|Conversions|ToFloat(Integer) (Math|Random|RandomIntegerinRange 0 7)) :!class /Script/Engine.MaterialInstanceDynamic)
      (Rendering|Material|SetScalarParameterValue _returnvalue_5 "Column" (Math|Conversions|ToFloat(Integer) (Math|Random|RandomIntegerinRange 0 7)) :!class /Script/Engine.MaterialInstanceDynamic))))

(event Collision|EventActorBeginOverlap
  (params (OtherActor :type Actor%20Object%20Reference)))

(event EventTick
  (params (DeltaSeconds :type Float%20%28single-precision%29)))

(fn ConstructionScript
  (|CallParentFunction))