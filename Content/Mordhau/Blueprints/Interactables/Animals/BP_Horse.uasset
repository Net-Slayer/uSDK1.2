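; Rideable horse that forwards the rider's combat, equipment and camera input to the Driver, with rearing and jumping of its own.
; Mount animation follows approach side; attack angle follows turn and look values.
; The authority randomizes replicated pattern and colors, applied through dynamic materials with enforced team colors overriding when ridden.
; Nav obstacles turn off while ridden or dead, and death triggers an impulse-driven ragdoll.
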(event EventBeginPlay
  (bind _returnvalue (Class|MordhauUtilityLibrary|GetMordhauSingleton))
  (bind _gear (Variables|Default|GetGear))
  (bind _hair (Variables|Default|GetHair))
  (bind _mesh (Variables|Character|GetMesh))
  (bind _colortables (Variables|/Script/Mordhau.MordhauSingleton|GetColorTables _returnvalue))
  (bind _output (Utilities|Array|Get(acopy) _colortables))
  (bind _entries (Utilities|Struct|BreakMordhauColorItemTable _output))
  (bind _returnvalue_2 (Utilities|Array|Length _entries))
  (bind _returnvalue_3 (- _returnvalue_2 1))
  (bind _returnvalue_4 (Math|Random|RandomIntegerinRange 0 _returnvalue_3))
  (bind _returnvalue_5 (Math|Conversions|ToByte(Integer) _returnvalue_4))
  (Utilities|FlowControl|Sequence
    (:then_0
      (bind _returnvalue_6 (Rendering|Material|CreateDynamicMaterialInstance _mesh 0 (Rendering|Material|GetMaterial _mesh 0) "None" :!class /Script/Engine.PrimitiveComponent))
      (Class|AdvancedCharacter|RegisterMaterialtoDissolve _returnvalue_6))
    (:then_1
      (bind _returnvalue_7 (Rendering|Material|CreateDynamicMaterialInstance _gear 0 (Rendering|Material|GetMaterial _gear 0) "None" :!class /Script/Engine.PrimitiveComponent))
      (Class|AdvancedCharacter|RegisterMaterialtoDissolve _returnvalue_7))
    (:then_2
      (bind _returnvalue_8 (Rendering|Material|CreateDynamicMaterialInstance _hair 0 (Rendering|Material|GetMaterial _hair 0) "None" :!class /Script/Engine.PrimitiveComponent))
      (Class|AdvancedCharacter|RegisterMaterialtoDissolve _returnvalue_8))
    (:then_3
      (Networking|SwitchHasAuthority
        (:Authority
          (Class|MordhauUtilityLibrary|SetCanEverAffectNavigation (Variables|Default|GetCapsuleComponent) false)
          (Variables|Default|SetPattern (Math|Conversions|ToByte(Integer) (Math|Random|RandomIntegerinRange 0 (- (Utilities|Array|Length (Variables|Default|GetPatterns)) 1))))
          (Variables|Default|SetColor1 _returnvalue_5)
          (Variables|Default|SetColor2 _returnvalue_5))))
    (:then_4
      (CallFunction|UpdateHorseColors))))

(event EventKnockOffDriver
  (params (Character :type Mordhau%20Character%20Object%20Reference))
  (Class|AdvancedCharacter|Trip Character)
  (Class|AdvancedCharacter|Knockback Character (* (Math|Conversions|ToVector(Vector2D) (Math|Vector2D|Normalize2D (Math|Conversions|ToVector2D(Vector) (Transformation|GetActorForwardVector)))) -2e+03)))

(event EventOnStoppedDriving
  (params (Character :type Mordhau%20Character%20Object%20Reference))
  (|CallParentFunction Character)
  (Networking|SwitchHasAuthority
    (:Authority
      (Class|MordhauUtilityLibrary|SetCanEverAffectNavigation (Variables|Default|GetNavObstacle1) true)
      (Class|MordhauUtilityLibrary|SetCanEverAffectNavigation (Variables|Default|GetNavObstalce2) true))))

(event EventOnDied
  (params (Angle :type Float%20%28single-precision%29) (Type :type EMordhauDamageType%20Enum :default "Generic") (SubType :type Byte :default 0) (bone :type Name%20%28by%20ref%29 :default "None") (Point :type Vector%20%28by%20ref%29 :default "0, 0, 0") (Source :type Actor%20Object%20Reference) (Agent :type Actor%20Object%20Reference))
  (bind _self self)
  (|CallParentFunction Angle Type SubType bone Point Source Agent)
  (Class|AdvancedCharacter|StartRagdoll)
  (Physics|AddImpulseatLocation (Variables|Character|GetMesh) (CallFunction|ComputeRagdollForce Agent Type SubType 0 _self _self) Point bone)
  (Networking|SwitchHasAuthority
    (:Authority
      (Class|MordhauUtilityLibrary|SetCanEverAffectNavigation (Variables|Default|GetNavObstacle1) false)
      (Class|MordhauUtilityLibrary|SetCanEverAffectNavigation (Variables|Default|GetNavObstalce2) false))))

(event EventSpawnTurd
  (Game|SpawnActorfromClass "/Game/Mordhau/Blueprints/Equipment/Thrown/BP_Turd.BP_Turd_C" (Transformation|GetSocketTransform (Variables|Character|GetMesh) "Poop" "RTS_World") "Undefined" 0 0))

(event EventOnStartedDriving
  (params (Character :type Mordhau%20Character%20Object%20Reference))
  (|CallParentFunction Character)
  (Networking|SwitchHasAuthority
    (:Authority
      (Class|MordhauUtilityLibrary|SetCanEverAffectNavigation (Variables|Default|GetNavObstacle1) false)
      (Class|MordhauUtilityLibrary|SetCanEverAffectNavigation (Variables|Default|GetNavObstalce2) false))))

(event EventOnDriverChanged
  (Utilities|IsValid (Variables|Default|GetDriver)
    (:Is%20Valid
      (CallFunction|UpdateHorseColors))))

(event EventOnCosmeticHit
  (params (DamageType :type EMordhauDamageType%20Enum :default "Generic") (SubType :type Byte :default 0) (Hit :type Hit%20Result%20Structure%20%28by%20ref%29) (Agent :type Actor%20Object%20Reference))
  (bind (_bblockinghit _binitialoverlap _time _distance _location _impactpoint _normal _impactnormal _physmat _hitactor _hitcomponent _hitbonename) (Collision|BreakHitResult Hit))
  (bind _self self)
  (|CallParentFunction DamageType SubType Hit Agent)
  (Physics|AddImpulseatLocation (Variables|Character|GetMesh) (CallFunction|ComputeRagdollForce Agent DamageType SubType 0 _self _self) _impactpoint _hitbonename))

(event Input|ActionEvents|InputActionCycleCamera
  (params (Key :type Key%20Structure))
  (bind _driver (Variables|Default|GetDriver))
  (:Pressed
    (Utilities|IsValid _driver
      (:Is%20Valid
        (Class|MordhauCharacter|CycleCamera _driver)))))

(event Input|ActionEvents|InputActionJump
  (params (Key :type Key%20Structure))
  (:Pressed
    (if (< (+ (Variables|Default|GetLastRearingTime) (Variables|Default|GetRearingDuration) 1.0) (Utilities|Time|GetGameTimeinSeconds))
      (bind _ashorse_movement_component (Utilities|Casting|CastToHorseMovementComponent (Variables|Character|GetCharacterMovement)))
      (if (< (Variables|/Script/Mordhau.HorseMovementComponent|GetGear _ashorse_movement_component) 2)
        (Class|Horse|RequestRearing)))))

(event Input|ActionEvents|InputActionKick
  (params (Key :type Key%20Structure))
  (bind _driver (Variables|Default|GetDriver))
  (:Pressed
    (Utilities|IsValid _driver
      (:Is%20Valid
        (Class|MordhauCharacter|RequestCouchedAttack _driver)))))

(event Input|ActionEvents|InputActionJump
  (params (Key :type Key%20Structure))
  (bind _charactermovement (Variables|Character|GetCharacterMovement))
  (:Pressed
    (if (> (Math|Float|MapRangeClamped (Math|Vector|VectorLength (Variables|/Script/Engine.MovementComponent|GetVelocity _charactermovement)) 0.0 (Variables|/Script/Engine.CharacterMovementComponent|GetMaxWalkSpeed _charactermovement) 0.0 1e+02) 5e+01)
      (Character|Jump))))

(fn ConstructionScript
  (bind _bloodreceivingskeletalmeshes (Variables|Default|GetBloodReceivingSkeletalMeshes))
  (bind _mesh (Variables|Character|GetMesh))
  (|CallParentFunction)
  (Variables|Default|SetBumpCapsule (Variables|Default|GetBumpCollider))
  (Class|SkinnedMeshComponent|SetMasterPoseComponent (Variables|Default|GetGear) _mesh false)
  (Class|SkinnedMeshComponent|SetMasterPoseComponent (Variables|Default|GetHair) _mesh false)
  (Utilities|Array|Add _bloodreceivingskeletalmeshes (Variables|Default|GetGear))
  (Utilities|Array|Add _bloodreceivingskeletalmeshes (Variables|Default|GetHair)))

(fn GetVehicleEnterInfo
  (params (Character :type Mordhau%20Character%20Object%20Reference) (FromTransform :type Transform%20%28by%20ref%29))
  (bind _location (Math|Transform|BreakTransform FromTransform))
  (bind _mesh (Variables|Character|GetMesh))
  (bind _returnvalue (Transformation|GetWorldTransform _mesh))
  (bind _returnvalue_2 (Math|Transform|InverseTransformLocation _returnvalue _location))
  (bind (_x _y) (Math|Vector|BreakVector _returnvalue_2))
  (if (< _x -55.0)
    (return (Utilities|Struct|MakeVehicleTransitionInfo "/Game/Mordhau/Animations/RawClips/Horse/Rider/GetOnHorseBehind.GetOnHorseBehind" 1.5 0.0))
    (elif (> _y 0.0)
      (return (Utilities|Struct|MakeVehicleTransitionInfo "/Game/Mordhau/Animations/RawClips/Horse/Rider/GetOnHorse.GetOnHorse" 1.5 0.0))
      (else
        (return (Utilities|Struct|MakeVehicleTransitionInfo "/Game/Mordhau/Animations/RawClips/Horse/Rider/GetOnHorseMirror.GetOnHorseMirror" 1.5 0.0))))))

(fn GetVehicleLeaveInfo
  (params (Character :type Mordhau%20Character%20Object%20Reference) (FromTransform :type Transform%20%28by%20ref%29))
  (return (Utilities|Struct|MakeVehicleTransitionInfo "/Game/Mordhau/Animations/RawClips/Horse/Rider/GetOffHorse.GetOffHorse" 1.5 0.0)))

(fn OverrideAttackAngle
  (params (Motion :type Attack%20Motion%20Object%20Reference))
  (bind _move (Variables|/Script/Mordhau.AttackMotion|GetMove Motion))
  (Utilities|FlowControl|Sequence
    (:then_0
      (bind _output_get (LocalVariables|SetFactor (Math|Float|Sign(Float) (Variables|Default|GetSecondaryTurnValue))))
      (if (or (Utilities|Enum|Equal(Enum) _move "LeftStrike") (Utilities|Enum|Equal(Enum) _move "AltStab"))
        (LocalVariables|SetFactor (* _output_get -1.0))))
    (:then_1
      (LocalVariables|SetAnglingValue (* (Math|Curves|GetFloatValue (Variables|Default|GetAttackAngleCurve) (Math|Float|Absolute(Float) (Variables|Default|GetSecondaryTurnValue))) (LocalVariables|GetFactor))))
    (:then_2
      (return (Math|Float|Lerp (LocalVariables|GetAnglingValue) 0.0 (Math|Float|MapRangeClamped (Variables|Default|GetLookUpValue) -45.0 -17.0 0.0 1.0))))))

(fn OnRepColor1
  (CallFunction|UpdateHorseColors))

(fn OnRepColor2
  (CallFunction|UpdateHorseColors))

(fn UpdateHorseColors
  (bind _returnvalue (Class|MordhauUtilityLibrary|GetMordhauSingleton))
  (bind _driver (Variables|Default|GetDriver))
  (bind _patterns (Variables|Default|GetPatterns))
  (bind _pattern (Variables|Default|GetPattern))
  (bind _returnvalue_2 (Utilities|Array|Length _patterns))
  (bind _team (Variables|/Script/Mordhau.AdvancedCharacter|GetTeam _driver))
  (bind _returnvalue_3 (Math|Conversions|ToByte(Integer) _returnvalue_2))
  (bind _returnvalue_4 (Math|Conversions|ToInteger(Byte) _team))
  (bind _returnvalue_5 (Class|KismetMathLibrary|PercentByteByte _pattern _returnvalue_3))
  (bind _returnvalue_6 (Math|Conversions|ToInteger(Byte) _returnvalue_5))
  (bind _output (Utilities|Array|Get(acopy) _patterns _returnvalue_6))
  (Networking|CanExecuteCosmeticEvents
    (:True
      (Utilities|FlowControl|Sequence
        (:then_0
          (Utilities|IsValid _driver
            (:Is%20Valid
              (bind _asmordhau_game_state (Utilities|Casting|CastToMordhauGameState (Game|GetGameState))
                (:then
                  (if (Math|Boolean|ANDBoolean (Variables|/Script/Mordhau.MordhauGameState|GetbEnforceTeamColors _asmordhau_game_state) (Variables|/Script/Mordhau.MordhauGameState|GetbIsTeamMode _asmordhau_game_state) (not (Variables|/Script/Mordhau.MordhauCharacter|GetbIgnoresTeamColors _driver)))
                    (bind _returnvalue_7 (Class|MordhauGameState|GetTeamColor _asmordhau_game_state _returnvalue_4))
                    (LocalVariables|SetColorA _returnvalue_7)
                    (bind _returnvalue_8 (Class|MordhauGameState|GetSecondaryTeamColor _asmordhau_game_state _returnvalue_4))
                    (LocalVariables|SetColorB _returnvalue_8)
                    (else
                      (bind _returnvalue_9 (Class|MordhauSingleton|GetTableColor _returnvalue 0 (Variables|Default|GetColor1) :!label _label))
                      (LocalVariables|SetColorA _returnvalue_9)
                      (bind _returnvalue_10 (Class|MordhauSingleton|GetTableColor _returnvalue 0 (Variables|Default|GetColor2)))
                      (LocalVariables|SetColorB _returnvalue_10))))
                (:CastFailed
                  (goto _label))))
            (:Is%20Not%20Valid
              (goto _label))))
        (:then_1
          (CallFunction|SetHorseColors (LocalVariables|GetColorA) (LocalVariables|GetColorB) _output (Variables|Default|GetGear))
          (CallFunction|SetHorseColors (LocalVariables|GetColorA) (LocalVariables|GetColorB) _output (Variables|Character|GetMesh)))))))

(fn SetHorseColors
  (params (Color1Color :type Linear%20Color%20Structure) (Color2Color :type Linear%20Color%20Structure) (Pattern :type Texture%202D%20Object%20Reference) (Component :type Skeletal%20Mesh%20Component%20Object%20Reference))
  (for _index (range 0 (- (Rendering|Material|GetNumMaterials Component) 1))
    (bind _asmaterial_instance_dynamic (Utilities|Casting|CastToMaterialInstanceDynamic (Rendering|Material|GetMaterial Component _index))
      (:then
        (LocalVariables|SetCurMat _asmaterial_instance_dynamic))
      (:CastFailed
        (bind _returnvalue (Rendering|Material|CreateDynamicMaterialInstance Component _index 0 "None" :!class /Script/Engine.PrimitiveComponent))
        (LocalVariables|SetCurMat _returnvalue)))
    (Rendering|Material|SetVectorParameterValue (LocalVariables|GetCurMat) "ColorA" Color1Color :!class /Script/Engine.MaterialInstanceDynamic)
    (Rendering|Material|SetVectorParameterValue (LocalVariables|GetCurMat) "ColorB" Color2Color :!class /Script/Engine.MaterialInstanceDynamic)
    (Rendering|Material|SetTextureParameterValue (LocalVariables|GetCurMat) "ColorMap" Pattern)))

(fn OnRepPattern
  (CallFunction|UpdateHorseColors))

(event Input|ActionEvents|InputActionHolster
  (params (Key :type Key%20Structure))
  (bind _driver (Variables|Default|GetDriver))
  ;[1 1 1] Equipment
  (:Pressed
    (Utilities|IsValid _driver
      (:Is%20Valid
        (Class|MordhauCharacter|EmptyHands _driver)))))

(event Input|ActionEvents|InputActionDrop
  (params (Key :type Key%20Structure))
  (bind _driver (Variables|Default|GetDriver))
  ;[1 1 1] Equipment
  (:Pressed
    (Utilities|IsValid _driver
      (:Is%20Valid
        (Class|MordhauCharacter|RequestDrop _driver)))))

(event Input|ActionEvents|InputActionEquipSlot8
  (params (Key :type Key%20Structure))
  (bind _driver (Variables|Default|GetDriver))
  ;[1 1 1] Equipment
  (:Pressed
    (Utilities|IsValid _driver
      (:Is%20Valid
        (Class|MordhauCharacter|EquipSlot8 _driver)))))

(event Input|ActionEvents|InputActionEquipSlot9
  (params (Key :type Key%20Structure))
  (bind _driver (Variables|Default|GetDriver))
  ;[1 1 1] Equipment
  (:Pressed
    (Utilities|IsValid _driver
      (:Is%20Valid
        (Class|MordhauCharacter|EquipSlot9 _driver)))))

(event Input|ActionEvents|InputActionEquipSlot1
  (params (Key :type Key%20Structure))
  (bind _driver (Variables|Default|GetDriver))
  ;[1 1 1] Equipment
  (:Pressed
    (Utilities|IsValid _driver
      (:Is%20Valid
        (Class|MordhauCharacter|EquipSlot1 _driver)))))

(event Input|ActionEvents|InputActionWeaponMode/Reload
  (params (Key :type Key%20Structure))
  (bind _driver (Variables|Default|GetDriver))
  ;[1 1 1] Equipment
  (:Pressed
    (Utilities|IsValid _driver
      (:Is%20Valid
        (Class|MordhauCharacter|RequestToggleWeaponMode _driver)))))

(event Input|ActionEvents|InputActionEquipSlot2
  (params (Key :type Key%20Structure))
  (bind _driver (Variables|Default|GetDriver))
  ;[1 1 1] Equipment
  (:Pressed
    (Utilities|IsValid _driver
      (:Is%20Valid
        (Class|MordhauCharacter|EquipSlot2 _driver)))))

(event Input|ActionEvents|InputActionEquipSlot3
  (params (Key :type Key%20Structure))
  (bind _driver (Variables|Default|GetDriver))
  ;[1 1 1] Equipment
  (:Pressed
    (Utilities|IsValid _driver
      (:Is%20Valid
        (Class|MordhauCharacter|EquipSlot3 _driver)))))

(event Input|ActionEvents|InputActionEquipSlot4
  (params (Key :type Key%20Structure))
  (bind _driver (Variables|Default|GetDriver))
  ;[1 1 1] Equipment
  (:Pressed
    (Utilities|IsValid _driver
      (:Is%20Valid
        (Class|MordhauCharacter|EquipSlot4 _driver)))))

(event Input|ActionEvents|InputActionEquipSlot5
  (params (Key :type Key%20Structure))
  (bind _driver (Variables|Default|GetDriver))
  ;[1 1 1] Equipment
  (:Pressed
    (Utilities|IsValid _driver
      (:Is%20Valid
        (Class|MordhauCharacter|EquipSlot5 _driver)))))

(event Input|ActionEvents|InputActionEquipSlot6
  (params (Key :type Key%20Structure))
  (bind _driver (Variables|Default|GetDriver))
  ;[1 1 1] Equipment
  (:Pressed
    (Utilities|IsValid _driver
      (:Is%20Valid
        (Class|MordhauCharacter|EquipSlot6 _driver)))))

(event Input|ActionEvents|InputActionEquipSlot7
  (params (Key :type Key%20Structure))
  (bind _driver (Variables|Default|GetDriver))
  ;[1 1 1] Equipment
  (:Pressed
    (Utilities|IsValid _driver
      (:Is%20Valid
        (Class|MordhauCharacter|EquipSlot7 _driver)))))

(event Input|ActionEvents|InputActionLeftStab
  (params (Key :type Key%20Structure))
  (bind _driver (Variables|Default|GetDriver))
  ;[1 1 1] Melee combat
  (:Pressed
    (Utilities|IsValid _driver
      (:Is%20Valid
        (Class|MordhauCharacter|RequestLeftStab _driver)))))

(event Input|ActionEvents|InputActionFlipAttackSide
  (params (Key :type Key%20Structure))
  (bind _driver (Variables|Default|GetDriver))
  (bind _driver_2 (Variables|Default|GetDriver))
  ;[1 1 1] Melee combat
  (:Pressed
    (Utilities|IsValid _driver
      (:Is%20Valid
        (Class|MordhauCharacter|FlipAttackSidePressed _driver))))
  (:Released
    (Utilities|IsValid _driver_2
      (:Is%20Valid
        (Class|MordhauCharacter|FlipAttackSideReleased _driver_2)))))

(event Input|ActionEvents|InputActionFeint
  (params (Key :type Key%20Structure))
  (bind _driver (Variables|Default|GetDriver))
  ;[1 1 1] Melee combat
  (:Pressed
    (Utilities|IsValid _driver
      (:Is%20Valid
        (Class|MordhauCharacter|RequestFeint _driver)))))

(event Input|ActionEvents|InputActionStab
  (params (Key :type Key%20Structure))
  (bind _driver (Variables|Default|GetDriver))
  (bind _driver_2 (Variables|Default|GetDriver))
  ;[1 1 1] Melee combat
  (:Pressed
    (Utilities|IsValid _driver_2
      (:Is%20Valid
        (Class|MordhauCharacter|ListenforStab360 _driver_2))))
  (:Released
    (Utilities|IsValid _driver
      (:Is%20Valid
        (Class|MordhauCharacter|StopListenforStab360 _driver)))))

(event Input|ActionEvents|InputActionLeftUpperStrike
  (params (Key :type Key%20Structure))
  (bind _driver (Variables|Default|GetDriver))
  ;[1 1 1] Melee combat
  (:Pressed
    (Utilities|IsValid _driver
      (:Is%20Valid
        (Class|MordhauCharacter|RequestLeftUpperStrike _driver)))))

(event Input|ActionEvents|InputActionParry
  (params (Key :type Key%20Structure))
  (bind _driver (Variables|Default|GetDriver))
  ;[1 1 1] Melee combat
  (:Pressed
    (Utilities|IsValid _driver
      (:Is%20Valid
        (Class|MordhauCharacter|BlockPressed _driver))))
  (:Released
    (Utilities|IsValid _driver
      (:Is%20Valid
        (Class|MordhauCharacter|BlockReleased _driver)))))

(event Input|ActionEvents|InputActionFeintOrParry
  (params (Key :type Key%20Structure))
  (bind _driver (Variables|Default|GetDriver))
  ;[1 1 1] Melee combat
  (:Pressed
    (Utilities|IsValid _driver
      (:Is%20Valid
        (Class|MordhauCharacter|FeintorBlockPressed _driver))))
  (:Released
    (Utilities|IsValid _driver
      (:Is%20Valid
        (Class|MordhauCharacter|FeintorBlockReleased _driver)))))

(event Input|ActionEvents|InputActionRightUpperStrike
  (params (Key :type Key%20Structure))
  (bind _driver (Variables|Default|GetDriver))
  ;[1 1 1] Melee combat
  (:Pressed
    (Utilities|IsValid _driver
      (:Is%20Valid
        (Class|MordhauCharacter|RequestRightUpperStrike _driver)))))

(event Input|ActionEvents|InputActionRightLowerStrike
  (params (Key :type Key%20Structure))
  (bind _driver (Variables|Default|GetDriver))
  ;[1 1 1] Melee combat
  (:Pressed
    (Utilities|IsValid _driver
      (:Is%20Valid
        (Class|MordhauCharacter|RequestRightLowerStrike _driver)))))

(event Input|ActionEvents|InputActionRightStrike
  (params (Key :type Key%20Structure))
  (bind _driver (Variables|Default|GetDriver))
  ;[1 1 1] Melee combat
  (:Pressed
    (Utilities|IsValid _driver
      (:Is%20Valid
        (Class|MordhauCharacter|RequestRightStrike _driver)))))

(event Input|ActionEvents|InputActionStrike
  (params (Key :type Key%20Structure))
  (bind _driver (Variables|Default|GetDriver))
  (bind _driver_2 (Variables|Default|GetDriver))
  ;[1 1 1] Melee combat
  (:Pressed
    (Utilities|IsValid _driver_2
      (:Is%20Valid
        (Class|MordhauCharacter|ListenforStrike360 _driver_2))))
  (:Released
    (Utilities|IsValid _driver
      (:Is%20Valid
        (Class|MordhauCharacter|StopListenforStrike360 _driver)))))

(event Input|ActionEvents|InputActionRightStab
  (params (Key :type Key%20Structure))
  (bind _driver (Variables|Default|GetDriver))
  ;[1 1 1] Melee combat
  (:Pressed
    (Utilities|IsValid _driver
      (:Is%20Valid
        (Class|MordhauCharacter|RequestRightStab _driver)))))

(event Input|ActionEvents|InputActionLeftLowerStrike
  (params (Key :type Key%20Structure))
  (bind _driver (Variables|Default|GetDriver))
  ;[1 1 1] Melee combat
  (:Pressed
    (Utilities|IsValid _driver
      (:Is%20Valid
        (Class|MordhauCharacter|RequestLeftLowerStrike _driver)))))

(event Input|ActionEvents|InputActionLeftStrike
  (params (Key :type Key%20Structure))
  (bind _driver (Variables|Default|GetDriver))
  ;[1 1 1] Melee combat
  (:Pressed
    (Utilities|IsValid _driver
      (:Is%20Valid
        (Class|MordhauCharacter|RequestLeftStrike _driver)))))

(event Input|ActionEvents|InputActionRangedCancel
  (params (Key :type Key%20Structure))
  (bind _driver (Variables|Default|GetDriver))
  ;[1 1 1] Ranged
  (:Pressed
    (Utilities|IsValid _driver
      (:Is%20Valid
        (Class|MordhauCharacter|RequestRangedCancel _driver)))))

(event Input|ActionEvents|InputActionFire
  (params (Key :type Key%20Structure))
  (bind _driver (Variables|Default|GetDriver))
  (bind _driver_2 (Variables|Default|GetDriver))
  ;[1 1 1] Ranged
  (:Pressed
    (Utilities|IsValid _driver
      (:Is%20Valid
        (Class|MordhauCharacter|FirePressed _driver))))
  (:Released
    (Utilities|IsValid _driver_2
      (:Is%20Valid
        (Class|MordhauCharacter|FireReleased _driver_2)))))