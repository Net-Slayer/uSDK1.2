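; BP_SwitchInteractable is an environment interactable switch that flips a boolean Value whenever an interaction starts.
; Value's RepNotify fires the empty OnValueToggled hook, then locks interaction for MinDelayBetweenUses via a retriggerable delay when that delay is nonzero.
; With StartInverted set, the authority toggles Value on BeginPlay, so that initial flip also runs through the notify.
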(event Custom|OnValueToggled)

(event Custom|PreventInteraction
  (Variables|Default|SetbIsInteractable false)
  (Utilities|FlowControl|RetriggerableDelay (Variables|Default|GetMinDelayBetweenUses))
  (Variables|Default|SetbIsInteractable true))

(event Custom|ToggleValue
  (Variables|Default|SetValue (not (Variables|Default|GetValue))))

(event EventBeginPlay
  (Networking|SwitchHasAuthority
    (:Authority
      (if (Variables|Default|GetStartInverted)
        (CallFunction|ToggleValue)))))

(event Collision|EventActorBeginOverlap
  (params (OtherActor :type Actor%20Object%20Reference)))

(event EventTick
  (params (DeltaSeconds :type Float%20%28single-precision%29)))

(event EventOnInteractionStart
  (params (Character :type Mordhau%20Character%20Object%20Reference))
  (CallFunction|ToggleValue))

(fn ConstructionScript
  (|CallParentFunction))

(fn OnRepValue
  (Utilities|FlowControl|Sequence
    (:then_0
      (CallFunction|OnValueToggled))
    (:then_1
      (if (not (Math|Float|NearlyEqual(Float) (Variables|Default|GetMinDelayBetweenUses) 0.0 1e-06))
        (CallFunction|PreventInteraction)))))