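; BP_EquipmentRack is an interactable environment rack that stores equipment from the interacting character's hands, up to MaxItems.
; Interaction is allowed when the character holds droppable equipment, with the right hand taking priority over the left.
; On interaction it recounts items, clearing slots no longer attached to it, then drops the equipment if space remains.
; The item loses its physics proxy, fills a slot and attaches at the single AttachPoint transform.
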(event EventBeginPlay
  (|CallParentFunction) ; This node is disabled and will not be called.\nDrag off pins to build functionality.
)

(event Collision|EventActorBeginOverlap
  (params (OtherActor :type Actor%20Object%20Reference))
  (|CallParentFunction OtherActor) ; This node is disabled and will not be called.\nDrag off pins to build functionality.
)

(event EventOnInteractionStart
  (params (Character :type Mordhau%20Character%20Object%20Reference))
  (CallFunction|ValidateCurrentItems)
  (if (< (Variables|Default|GetTotalItems) (Variables|Default|GetMaxItems))
    (bind _equipment (CallFunction|GetEquipmenttoPlace Character))
    (Utilities|IsValid _equipment
      (:Is%20Valid
        (Class|MordhauCharacter|DropEquipment Character _equipment)
        (CallFunction|AttachEquipment _equipment)))))

(event EventTick
  (params (DeltaSeconds :type Float%20%28single-precision%29))
  (|CallParentFunction DeltaSeconds) ; This node is disabled and will not be called.\nDrag off pins to build functionality.
)

(fn ConstructionScript
  (|CallParentFunction))

(fn CanInteract
  (params (Character :type Mordhau%20Character%20Object%20Reference))
  (if (stale _returnvalue)
    (bind _equipment (CallFunction|GetEquipmenttoPlace Character))
    (Utilities|IsValid _equipment
      (:Is%20Valid
        (return true))
      (:Is%20Not%20Valid
        _)))
  (return false))

(fn AttachEquipment
  (params (Equipment :type Mordhau%20Equipment%20Object%20Reference))
  (bind _currentitems (Variables|Default|GetCurrentItems))
  (Utilities|FlowControl|Sequence
    (:then_0
      (Class|MordhauEquipment|DestroyPhysicsProxy Equipment)
      (if (< (Utilities|Array|Length _currentitems) (Variables|Default|GetMaxItems))
        (bind _returnvalue (Utilities|Array|Add _currentitems Equipment))
        (LocalVariables|SetFoundSlot _returnvalue)
        (else
          (bind (_array_element _array_index) (Utilities|Array|ForEachLoopwithBreak _currentitems :!label _label)
            (:LoopBody
              (if (== _array_element 0)
                (LocalVariables|SetFoundSlot _array_index)
                (goto _label Break)))
            (:Completed
              (Utilities|Array|SetArrayElem (Variables|Default|GetCurrentItems) (LocalVariables|GetFoundSlot) Equipment))))))
    (:then_1
      (Transformation|SetActorTransform Equipment (Transformation|GetWorldTransform (Variables|Default|GetAttachPoint)))
      (Transformation|AttachActorToActor self "None" "KeepWorld" "KeepWorld" "KeepWorld" false))))

(fn GetEquipmenttoPlace
  (params (Character :type Mordhau%20Character%20Object%20Reference))
  (bind _lefthandequipment (Variables|/Script/Mordhau.MordhauCharacter|GetLeftHandEquipment Character))
  (bind _righthandequipment (Variables|/Script/Mordhau.MordhauCharacter|GetRightHandEquipment Character))
  (Utilities|FlowControl|Sequence
    (:then_0
      (Utilities|FlowControl|Sequence
        (:then_0
          (Utilities|IsValid _righthandequipment
            (:Is%20Valid
              (if (Variables|/Script/Mordhau.MordhauEquipment|GetbAllowDrop _righthandequipment)
                (LocalVariables|SetToDrop _righthandequipment)))))
        (:then_1
          (Utilities|IsValid (LocalVariables|GetToDrop)
            (:Is%20Not%20Valid
              (Utilities|IsValid _lefthandequipment
                (:Is%20Valid
                  (if (Variables|/Script/Mordhau.MordhauEquipment|GetbAllowDrop _lefthandequipment)
                    (LocalVariables|SetToDrop _lefthandequipment)))))))))
    (:then_1
      (return (LocalVariables|GetToDrop)))))

(fn ValidateCurrentItems
  (bind _currentitems (Variables|Default|GetCurrentItems))
  (Variables|Default|SetTotalItems 0)
  (for (_array_element _array_index) _currentitems
    (if (not (== _array_element 0))
      (Utilities|IsValid _array_element
        (:Is%20Valid
          (if (== (Actor|GetAttachParentActor _array_element) self)
            (Variables|Default|SetTotalItems (+ (Variables|Default|GetTotalItems) 1))
            (else
              (Utilities|Array|SetArrayElem _currentitems _array_index 0 :!label _label))))
        (:Is%20Not%20Valid
          (goto _label))))))