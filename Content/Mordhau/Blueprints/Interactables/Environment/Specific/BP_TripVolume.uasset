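; BP_TripVolume is an environment volume that trips Mordhau characters who enter it moving too fast.
; On begin overlap, it checks on the authority that the character's speed meets a threshold and that they are not in a vehicle.
; DoTrip calls the character's Trip and, if that succeeds, applies a knockback along their horizontal direction of travel, scaled by a configurable force.
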(event EventBeginPlay)

(event Collision|EventActorBeginOverlap
  (params (OtherActor :type Actor%20Object%20Reference))
  (bind _asbp_mordhau_character (Utilities|Casting|CastToBP_MordhauCharacter OtherActor))
  (if (Math|Boolean|ANDBoolean (Ability|HasAuthority _asbp_mordhau_character) (>= (Math|Vector|VectorLength (Transformation|GetVelocity _asbp_mordhau_character)) (Variables|Default|GetTripIfVelocityExceeds)) (not (Utilities|IsValid (Variables|/Script/Mordhau.MordhauCharacter|GetCurrentVehicle _asbp_mordhau_character))))
    (CallFunction|DoTrip _asbp_mordhau_character)))

(event EventTick
  (params (DeltaSeconds :type Float%20%28single-precision%29)))

(fn ConstructionScript)

(fn DoTrip
  (params (Character :type BP%20Mordhau%20Character%20Object%20Reference))
  (bind _output_get (LocalVariables|SetForceDir (* (Math|Vector|Normalize (Math|Conversions|ToVector(Vector2D) (Math|Conversions|ToVector2D(Vector) (Transformation|GetVelocity Character)))) (Variables|Default|GetTripForce))))
  (bind _returnvalue (Class|AdvancedCharacter|Trip Character))
  (if _returnvalue
    (Class|AdvancedCharacter|Knockback Character _output_get)))