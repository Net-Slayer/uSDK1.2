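; Secondary crank interactable that forwards interaction to a linked MasterCrank and visually follows a progress value.
; Interaction requires a valid master whose own check passes, and toggles the master's value on authority.
; Progress updates scrub the skeletal animation and an optional dynamic material through an optional curve, outside the end values.
; A movement sound with direction-based speed plays during travel, then fades into raised or lowered stop sounds.
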(event EventBeginPlay
  (bind _animatedmaterialindex (Variables|Default|GetAnimatedMaterialIndex))
  (bind _skeletalmesh (Variables|Default|GetSkeletalMesh))
  (Utilities|FlowControl|Sequence
    (:then_0
      (if (>= _animatedmaterialindex 0)
        (bind _returnvalue (Rendering|Material|CreateDynamicMaterialInstance _skeletalmesh 1 (Rendering|Material|GetMaterial _skeletalmesh _animatedmaterialindex) "None" :!class /Script/Engine.PrimitiveComponent))
        (Variables|Default|SetAnimatedMaterial _returnvalue)))
    (:then_1
      (|CallParentFunction))))

(event EventOnInteractionStart
  (params (Character :type Mordhau%20Character%20Object%20Reference))
  (bind _mastercrank (Variables|Default|GetMasterCrank))
  (Utilities|IsValid _mastercrank
    (:Is%20Valid
      (if (Ability|HasAuthority _mastercrank)
        (Default|ToggleValue _mastercrank)))))

(fn ConstructionScript
  (|CallParentFunction))

(fn CanInteract
  (params (Character :type Mordhau%20Character%20Object%20Reference))
  (Utilities|IsValid (Variables|Default|GetMasterCrank)
    (:Is%20Valid
      (if (stale _returnvalue)
        (return (stale _returnvalue))
        (else
          _)))
    (:Is%20Not%20Valid
      _))
  (return false))

(fn UpdateProgress
  (params (Progress :type Float%20%28single-precision%29))
  (bind _skeletalmesh (Variables|Default|GetSkeletalMesh))
  (bind _animatedmaterial (Variables|Default|GetAnimatedMaterial))
  (bind _raisespeed (Variables|Default|GetRaiseSpeed))
  (bind _lowerspeed (Variables|Default|GetLowerSpeed))
  (bind _curve (Variables|Default|GetCurve))
  (bind _returnvalue (Transformation|GetSocketLocation _skeletalmesh "Crank"))
  (LocalVariables|SetPrevSmoothedValue (Variables|Default|GetSmoothedValue))
  (Variables|Default|SetSmoothedValue Progress)
  (if (or (== (Variables|Default|GetSmoothedValue) 0.0) (== (Variables|Default|GetSmoothedValue) 1.0))
    (if (== (Variables|Default|GetSmoothedValue) 1.0)
      (Audio|PlaySoundatLocation "/Game/Mordhau/Audio/Cues/Misc/SC_Crank_StopRaised.SC_Crank_StopRaised" _returnvalue "0, 0, 0" 1.0 1.0 0.0 0 0 0)
      (else
        (Audio|PlaySoundatLocation "/Game/Mordhau/Audio/Cues/Misc/SC_Crank_StopLowered.SC_Crank_StopLowered" _returnvalue "0, 0, 0" 1.0 1.0 0.0 0 0 0)))
    (Utilities|IsValid (Variables|Default|GetCurrentMovementSound)
      (:Is%20Valid
        (Audio|Components|Audio|FadeOut (Variables|Default|GetCurrentMovementSound) 0.2 0.0 :!class /Script/Engine.AudioComponent)
        (Variables|Default|SetCurrentMovementSound 0)))
    (else
      (Networking|CanExecuteCosmeticEvents
        (:True
          (Utilities|FlowControl|Sequence
            (:then_0
              (Utilities|IsValid (Variables|Default|GetCurrentMovementSound)
                (:Is%20Not%20Valid
                  (bind _returnvalue_2 (Audio|SpawnSoundatLocation "/Game/Mordhau/Audio/Cues/Misc/SC_Crank_Movement.SC_Crank_Movement" _returnvalue "0, 0, 0" 1.0 1.0 0.0 0 0))
                  (bind _output_get (Variables|Default|SetCurrentMovementSound _returnvalue_2))
                  (Utilities|IsValid _output_get
                    (:Is%20Valid
                      (Audio|Parameter|SetFloatParameter _output_get "Speed" (/ (Math|Float|MapRangeClamped (Math|Conversions|ToFloat(Boolean) (< (LocalVariables|GetPrevSmoothedValue) (Variables|Default|GetSmoothedValue))) 0.0 1.0 _lowerspeed _raisespeed) (Math|Float|Min(Float) _raisespeed _lowerspeed)) :!class /Script/Engine.AudioComponent))))))
            (:then_1
              (Utilities|IsValid _curve
                (:Is%20Valid
                  (Variables|Default|SetSmoothedValuePostCurve (Math|Curves|GetFloatValue _curve (Variables|Default|GetSmoothedValue))))
                (:Is%20Not%20Valid
                  (Variables|Default|SetSmoothedValuePostCurve (Variables|Default|GetSmoothedValue))))
              (Components|Animation|SetPosition (Variables|Default|GetSkeletalMesh) (* (Variables|Default|GetSmoothedValuePostCurve) 0.983) true)
              (Utilities|IsValid _animatedmaterial
                (:Is%20Valid
                  (Rendering|Material|SetScalarParameterValue _animatedmaterial "NormalizedTime" (Variables|Default|GetSmoothedValuePostCurve) :!class /Script/Engine.MaterialInstanceDynamic))))))))))