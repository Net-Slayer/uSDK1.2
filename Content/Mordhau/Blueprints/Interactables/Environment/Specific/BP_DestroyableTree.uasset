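; Destroyable tree that falls when its replicated health reaches zero and crushes whatever lies along its landing line.
; UpdateReplicatedHealth reveals the log, plays sound and particles, and enables Tick, which blends the log toward the PreviewTree transform along a bounce curve.
; A fixed delay times the impact: effects, camera shake and radial damage at three Impact points, credited to the last health-change instigator.
; Tick disables itself once the timed fall completes.
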(event Collision|EventActorBeginOverlap
  (params (OtherActor :type Actor%20Object%20Reference))
  (|CallParentFunction OtherActor) ; This node is disabled and will not be called.\nDrag off pins to build functionality.
)

(event EventTick
  (params (DeltaSeconds :type Float%20%28single-precision%29))
  (bind _returnvalue (Utilities|Time|GetTimeSeconds))
  (bind _fallstarttime (Variables|Default|GetFallStartTime))
  (bind _returnvalue_2 (+ _fallstarttime 5.0))
  (bind _returnvalue_3 (Class|MordhauUtilityLibrary|GetNormalizedTime _fallstarttime _returnvalue_2 _returnvalue))
  (|CallParentFunction DeltaSeconds)
  (if (not (== (Variables|Default|GetFallStartTime) -1.0))
    (Transformation|SetRelativeTransform (Variables|Default|GetBreakableTree_Log) (Math|Transform|Lerp(Transform) (Variables|Default|GetFallingLogOrigin) (Transformation|GetRelativeTransform (Variables|Default|GetPreviewTree)) (Math|Curves|GetFloatValue (Variables|Default|GetBounceCurve) _returnvalue_3)) false false)
    (if (== _returnvalue_3 1.0)
      (Actor|Tick|SetActorTickEnabled false))))

(event EventUpdateReplicatedHealth
  (bind _self self)
  (bind _breakabletree_log (Variables|Default|GetBreakableTree_Log))
  (bind _impact3 (Variables|Default|GetImpact3))
  (bind _impact2 (Variables|Default|GetImpact2))
  (bind _returnvalue (Transformation|GetWorldLocation _impact2))
  (bind _returnvalue_2 (Transformation|GetWorldLocation _impact3))
  (bind _returnvalue_3 (Transformation|GetWorldLocation _breakabletree_log))
  (|CallParentFunction)
  (Variables|Default|SetFinalChopperController (Variables|Default|GetLastHealthChangeInstigator))
  (if (== (Variables|Default|GetReplicatedHealth) 0)
    (if (== (Variables|Default|GetFallStartTime) -1.0)
      (Variables|Default|SetFallingLogOrigin (Transformation|GetRelativeTransform (Variables|Default|GetBreakableTree_Log)))
      (Variables|Default|SetFallStartTime (Utilities|Time|GetTimeSeconds))
      (Actor|Tick|SetActorTickEnabled true)
      (Development|SetHiddeninGame (Variables|Default|GetBreakableTree_Log) false false)
      (Audio|PlaySoundatLocation 0 _returnvalue_3 "0, 0, 0" 1.0 1.0 0.0 0 0 0)
      (Effects|SpawnEmitteratLocation 0 _returnvalue_3)
      (Utilities|FlowControl|Delay 3.3)
      (Effects|SpawnEmitteratLocation 0 _returnvalue_2 "90.000000, 0,0.000000")
      (Audio|PlaySoundatLocation 0 _returnvalue_2 "0, 0, 0" 1.0 1.0 0.0 0 0 0)
      (Class|MordhauUtilityLibrary|MordhauApplyRadialDamagewithFalloff 2.5e+03 1.0 4e+02 2e+01 _returnvalue_2 5e+01 1e+02 5.0 (Utilities|Array|MakeArray 0) 1e+03 5e+02 2e+02 _self (Variables|Default|GetFinalChopperController) "ECC_WorldStatic" false)
      (Class|MordhauUtilityLibrary|MordhauApplyRadialDamagewithFalloff 2.5e+03 1.0 4e+02 2e+01 (Transformation|GetWorldLocation (Variables|Default|GetImpact1)) 5e+01 1e+02 5.0 (Utilities|Array|MakeArray 0) 1e+03 5e+02 2e+02 _self (Variables|Default|GetFinalChopperController) "ECC_WorldStatic" false)
      (Class|MordhauUtilityLibrary|MordhauApplyRadialDamagewithFalloff 2.5e+03 1.0 4e+02 2e+01 _returnvalue 5e+01 1e+02 5.0 (Utilities|Array|MakeArray 0) 1e+03 5e+02 2e+02 _self (Variables|Default|GetFinalChopperController) "ECC_WorldStatic" false)
      (Camera|PlayWorldCameraShake "/Game/Mordhau/Blueprints/CameraShakes/ImpactShake.ImpactShake_C" _returnvalue 2.5e+02 7.5e+03 1e+01))))

(fn ConstructionScript
  (|CallParentFunction))