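; Base interactable that gives each player their own cooldown, so it appears depleted only to players who recently depleted it.
; Deplete queues the PlayerState with an expiry time, and a single chained timer pops entries in order.
; CanInteract rejects queued players, while UpdateValue mirrors the local player's state into IsDepleted.
; Empty Depleted, Refilled, AvailableInteractionStart and NotAvailableInteractionStart events serve as hooks.
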(event Custom|Deplete
  (params (PlayerState :type Player%20State%20Object%20Reference))
  (bind _incooldown (Variables|Default|GetInCooldown))
  (bind _incooldownendtime (Variables|Default|GetInCooldownEndTime))
  (if (not (Utilities|Array|ContainsItem _incooldown PlayerState))
    (Utilities|Array|Add _incooldownendtime (+ (Utilities|Time|GetTimeSeconds) (Variables|Default|GetRefillDelay)))
    (Utilities|Array|Add _incooldown PlayerState)
    (CallFunction|UpdateValue)
    (if (== (Utilities|Array|Length _incooldownendtime) 1)
      (Utilities|Time|SetTimerbyEvent (delegate Custom|PopCooldown) (Math|Float|Max(Float) (- (Utilities|Array|Get(acopy) _incooldownendtime) (Utilities|Time|GetTimeSeconds)) 0.001)))))

(event Custom|PopCooldown
  (bind _incooldownendtime (Variables|Default|GetInCooldownEndTime))
  (Utilities|Array|RemoveIndex (Variables|Default|GetInCooldownEndTime))
  (Utilities|Array|RemoveIndex (Variables|Default|GetInCooldown))
  (CallFunction|UpdateValue)
  (if (> (Utilities|Array|Length _incooldownendtime) 0)
    (Utilities|Time|SetTimerbyEvent (delegate Custom|PopCooldown) (Math|Float|Max(Float) (- (Utilities|Array|Get(acopy) _incooldownendtime) (Utilities|Time|GetTimeSeconds)) 0.001))))

(event Custom|NotAvailableInteractionStart
  (params (Character :type Mordhau%20Character%20Object%20Reference)))

(event Custom|AvailableInteractionStart
  (params (Character :type Mordhau%20Character%20Object%20Reference)))

(event Custom|Refilled)

(event Custom|Depleted)

(event EventBeginPlay)

(event Collision|EventActorBeginOverlap
  (params (OtherActor :type Actor%20Object%20Reference)))

(event EventTick
  (params (DeltaSeconds :type Float%20%28single-precision%29)))

(event EventOnInteractionStart
  (params (Character :type Mordhau%20Character%20Object%20Reference))
  (if (Variables|Default|GetIsDepleted)
    (CallFunction|NotAvailableInteractionStart Character)
    (else
      (CallFunction|AvailableInteractionStart Character))))

(fn ConstructionScript
  (|CallParentFunction))

(fn CanInteract
  (params (Character :type Mordhau%20Character%20Object%20Reference))
  (bind _playerstate (Variables|/Script/Engine.Pawn|GetPlayerState Character))
  (Utilities|IsValid Character
    (:Is%20Valid
      (Utilities|IsValid _playerstate
        (:Is%20Valid
          (if (Utilities|Array|ContainsItem (Variables|Default|GetInCooldown) _playerstate)
            (return false)
            (else
              _)))
        (:Is%20Not%20Valid
          (return false))))
    (:Is%20Not%20Valid
      _))
  (return (stale _returnvalue)))

(fn UpdateValue
  (bind _returnvalue (Game|GetPlayerController 0))
  (bind _playerstate (Variables|/Script/Engine.Controller|GetPlayerState _returnvalue))
  (Utilities|IsValid _returnvalue
    (:Is%20Valid
      (if (Pawn|IsLocalPlayerController _returnvalue)
        (Utilities|IsValid _playerstate
          (:Is%20Valid
            (if (Math|Boolean|NotEqual(Boolean) (Utilities|Array|ContainsItem (Variables|Default|GetInCooldown) _playerstate) (Variables|Default|GetIsDepleted))
              (bind _output_get (Variables|Default|SetIsDepleted (not (Variables|Default|GetIsDepleted))))
              (if _output_get
                (CallFunction|Depleted)
                (else
                  (CallFunction|Refilled))))))))))