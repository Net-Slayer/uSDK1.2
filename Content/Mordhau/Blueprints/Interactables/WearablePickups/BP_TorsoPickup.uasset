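; BP_TorsoPickup is a chest armor pickup that gives battle royale characters tiered torso upgrades.
; On assignment it has the character spawn its current chest piece, records its own class as ChestArmor, then calls the parent assignment.
; CanInteract rejects non-upgrades for battle royale characters, comparing Tier against the worn class's defaults.
; Otherwise it returns the parent CanInteract output, though that parent call is never executed.
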(event EventBeginPlay)

(event Collision|EventActorBeginOverlap
  (params (OtherActor :type Actor%20Object%20Reference))
  (|CallParentFunction OtherActor) ; This node is disabled and will not be called.\nDrag off pins to build functionality.
)

(event EventTick
  (params (DeltaSeconds :type Float%20%28single-precision%29))
  (|CallParentFunction DeltaSeconds) ; This node is disabled and will not be called.\nDrag off pins to build functionality.
)

(event EventAssigntoCharacter
  (params (Character :type Mordhau%20Character%20Object%20Reference) (CustomizatonReplicationActor :type Customization%20Replication%20Actor%20Object%20Reference))
  (Utilities|FlowControl|Sequence
    (:then_0
      (bind _asbp_battle_royale_character (Utilities|Casting|CastToBP_BattleRoyaleCharacter Character))
      (Default|SpawnArmorPiece _asbp_battle_royale_character (Variables|/Game/Mordhau/Blueprints/Characters/BP_BattleRoyaleCharacter.BP_BattleRoyaleCharacter_C|GetChestArmor _asbp_battle_royale_character))
      (Variables|/Game/Mordhau/Blueprints/Characters/BP_BattleRoyaleCharacter.BP_BattleRoyaleCharacter_C|SetChestArmor _asbp_battle_royale_character (Utilities|GetClass self)))
    (:then_1
      (|CallParentFunction Character CustomizatonReplicationActor))))

(fn ConstructionScript
  (|CallParentFunction))

(fn CanInteract
  (params (Character :type Mordhau%20Character%20Object%20Reference))
  (bind _asbp_battle_royale_character (Utilities|Casting|CastToBP_BattleRoyaleCharacter Character)
    (:then
      (if (CallFunction|IsAnUpgrade _asbp_battle_royale_character)
        _
        (else
          (return false))))
    (:CastFailed
      _))
  (return (stale _returnvalue)))

(fn IsAnUpgrade
  (params (Char :type BP%20Battle%20Royale%20Character%20Object%20Reference))
  (bind _chestarmor (Variables|/Game/Mordhau/Blueprints/Characters/BP_BattleRoyaleCharacter.BP_BattleRoyaleCharacter_C|GetChestArmor Char))
  (if (Utilities|IsValidClass _chestarmor)
    (if (< (.Tier (Utilities|GetClassDefaults _chestarmor)) (Variables|Default|GetTier))
      _
      (else
        (return false))))
  (return true))