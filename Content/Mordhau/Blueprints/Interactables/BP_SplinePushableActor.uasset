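; Pushable actor that travels along a target actor's spline as its Progress changes, with its construction script assigning Area as the push area.
; On begin play and each progress update, it maps Progress into SplineRange and snaps to that constant-velocity spline transform.
; The server then checks skeletal mesh overlaps, shifting characters by the movement delta, skipping those in vehicles, and destroying other overlapping Mordhau actors with massive damage.
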(event EventBeginPlay
  (bind _splinerange (Variables|Default|GetSplineRange))
  (bind _skeletalmesh (Variables|Default|GetSkeletalMesh))
  (bind (_x _y) (Math|Vector2D|BreakVector2D _splinerange))
  (|CallParentFunction)
  (Variables|Default|SetPreviousLocation (Transformation|GetActorLocation))
  (Transformation|SetActorTransform (Spline|GetTransformatTime (Variables|/Game/Mordhau/Blueprints/Interactables/BP_SplineActor.BP_SplineActor_C|GetSpline (Variables|Default|GetTargetSplineActor)) (Math|Float|Lerp _x _y (Variables|Default|GetProgress)) "World" true false))
  (Networking|SwitchHasAuthority
    (:Authority
      (bind _outactors (Collision|ComponentOverlapActors _skeletalmesh (Transformation|GetWorldTransform _skeletalmesh) (Utilities|Array|MakeArray "ObjectTypeQuery3" "ObjectTypeQuery5" "ObjectTypeQuery1") 0))
      (for _array_element _outactors
        (bind _asmordhau_character (Utilities|Casting|CastToMordhauCharacter _array_element)
          (:then
            (Utilities|IsValid (Variables|/Script/Mordhau.MordhauCharacter|GetCurrentVehicle _asmordhau_character)
              (:Is%20Not%20Valid
                _)))
          (:CastFailed
            _))
        (bind _asadvanced_character (Utilities|Casting|CastToAdvancedCharacter _array_element)
          (:then
            (Transformation|AddActorWorldOffset _asadvanced_character (- (Transformation|GetActorLocation) (Variables|Default|GetPreviousLocation))))
          (:CastFailed
            (bind _asmordhau_actor (Utilities|Casting|CastToMordhauActor _array_element))
            (Game|Damage|ApplyDamage _asmordhau_actor 1e+07 0 0)))))))

(event Collision|EventActorBeginOverlap
  (params (OtherActor :type Actor%20Object%20Reference)))

(event EventTick
  (params (DeltaSeconds :type Float%20%28single-precision%29)))

(event EventOnProgressUpdated
  (params (OldProgress :type Float%20%28single-precision%29))
  (bind _splinerange (Variables|Default|GetSplineRange))
  (bind _skeletalmesh (Variables|Default|GetSkeletalMesh))
  (bind (_x _y) (Math|Vector2D|BreakVector2D _splinerange))
  (Variables|Default|SetPreviousLocation (Transformation|GetActorLocation))
  (Transformation|SetActorTransform (Spline|GetTransformatTime (Variables|/Game/Mordhau/Blueprints/Interactables/BP_SplineActor.BP_SplineActor_C|GetSpline (Variables|Default|GetTargetSplineActor)) (Math|Float|Lerp _x _y (Variables|Default|GetProgress)) "World" true false))
  (Networking|SwitchHasAuthority
    (:Authority
      (bind _outactors (Collision|ComponentOverlapActors _skeletalmesh (Transformation|GetWorldTransform _skeletalmesh) (Utilities|Array|MakeArray "ObjectTypeQuery3" "ObjectTypeQuery5" "ObjectTypeQuery1") 0))
      (for _array_element _outactors
        (bind _asmordhau_character (Utilities|Casting|CastToMordhauCharacter _array_element)
          (:then
            (Utilities|IsValid (Variables|/Script/Mordhau.MordhauCharacter|GetCurrentVehicle _asmordhau_character)
              (:Is%20Not%20Valid
                _)))
          (:CastFailed
            _))
        (bind _asadvanced_character (Utilities|Casting|CastToAdvancedCharacter _array_element)
          (:then
            (Transformation|AddActorWorldOffset _asadvanced_character (- (Transformation|GetActorLocation) (Variables|Default|GetPreviousLocation))))
          (:CastFailed
            (bind _asmordhau_actor (Utilities|Casting|CastToMordhauActor _array_element))
            (Game|Damage|ApplyDamage _asmordhau_actor 1e+07 0 0)))))))

(fn ConstructionScript
  (Variables|Default|SetPushArea (Variables|Default|GetArea)))

(fn GetTransformAlongSplineOffset
  (params (OffsetA :type Float%20%28single-precision%29) (OffsetB :type Float%20%28single-precision%29))
  (return ""))