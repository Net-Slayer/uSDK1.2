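; BP_Trebuchet is an automatic siege engine that repeatedly reloads and fires projectiles with randomized pitch and yaw.
; A timer and delay loop drives animation and audio, scaling playback rate to fit reload time.
; Only the authority spawns BP_TrebuchetProjectile.
; Clients run the same loop locally, first waiting six seconds, then deriving their cycle position from server world time rather than replicated events.
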(event Custom|Fire
  (bind _reloadsound (Variables|Default|GetReloadSound))
  (bind _audio (Variables|Default|GetAudio))
  (bind _projectilespawn (Variables|Default|GetProjectileSpawn))
  (bind _skeletalmesh (Variables|Default|GetSkeletalMesh))
  (bind _skeletalmesh_2 (Variables|Default|GetSkeletalMesh))
  (bind _hornsound (Variables|Default|GetHornSound))
  (bind _firesound (Variables|Default|GetFireSound))
  (bind _audio_2 (Variables|Default|GetAudio))
  (bind _returnvalue (Transformation|GetWorldTransform _projectilespawn))
  (bind (_location _rotation _scale) (Math|Transform|BreakTransform _returnvalue))
  (Utilities|FlowControl|Sequence
    (:then_0
      (Utilities|FlowControl|Sequence
        (:then_0
          (if (Variables|Default|GetPlayHornSound)
            (Utilities|IsValid _hornsound
              (:Is%20Valid
                (Audio|PlaySoundatLocation _hornsound (Transformation|GetWorldLocation (Variables|Default|GetAudio)) "0, 0, 0" 1.0 1.0 0.0 0 0 0)))))
        (:then_1
          (Utilities|IsValid _firesound
            (:Is%20Valid
              (Audio|Components|Audio|SetSound _audio_2 _firesound)
              (Audio|Components|Audio|Play _audio_2 0.0))))))
    (:then_1
      (Variables|/Script/Engine.SkeletalMeshComponent|SetGlobalAnimRateScale _skeletalmesh 1.0)
      (Components|Animation|PlayAnimation _skeletalmesh 0 false)
      (Utilities|FlowControl|Delay (Variables|Default|GetFireTime))
      (Utilities|FlowControl|Sequence
        (:then_0
          (Networking|SwitchHasAuthority
            (:Authority
              (bind _returnvalue_2 (Game|SpawnActorfromClass "/Game/Mordhau/Blueprints/Interactables/SiegeEngines/BP_TrebuchetProjectile.BP_TrebuchetProjectile_C" (Math|Transform|MakeTransform _location (Math|Rotator|CombineRotators (Math|Rotator|MakeRotator 0.0 (- (* (Math|Random|RandomFloat) (Variables|Default|GetRandomPitch) 2.0) (Variables|Default|GetRandomPitch)) (- (* (Math|Random|RandomFloat) (Variables|Default|GetRandomYaw) 2.0) (Variables|Default|GetRandomYaw))) _rotation) _scale) "AlwaysSpawn" self 0))
              (Class|MordhauProjectile|InitializeProjectile _returnvalue_2 0 false self)
              (Class|MordhauProjectile|Fire _returnvalue_2))))
        (:then_1
          (Utilities|FlowControl|Sequence
            (:then_0
              (Utilities|IsValid _reloadsound
                (:Is%20Valid
                  (Audio|Components|Audio|SetSound _audio _reloadsound)
                  (Audio|Components|Audio|Play _audio 0.0))))
            (:then_1
              (Utilities|FlowControl|Delay (Variables|Default|GetRecoveryTime))
              (Variables|/Script/Engine.SkeletalMeshComponent|SetGlobalAnimRateScale _skeletalmesh_2 (/ 1.0 (Variables|Default|GetReloadTime)))
              (Components|Animation|PlayAnimation _skeletalmesh_2 0 false)
              (Utilities|Time|SetTimerbyEvent (delegate Custom|Fire) (Variables|Default|GetReloadTime)))))))))

(event Custom|SyncTreb
  (bind _returnvalue (Game|GetGameState))
  (bind _initialdelay (Variables|Default|GetInitialDelay))
  (bind _reloadtime (Variables|Default|GetReloadTime))
  (bind _firetime (Variables|Default|GetFireTime))
  (bind _recoverytime (Variables|Default|GetRecoveryTime))
  (bind _reloadsound (Variables|Default|GetReloadSound))
  (bind _audio (Variables|Default|GetAudio))
  (bind _skeletalmesh (Variables|Default|GetSkeletalMesh))
  (bind _returnvalue_2 (GameState|GetServerWorldTimeSeconds _returnvalue))
  (bind _returnvalue_3 (+ _initialdelay _reloadtime))
  (bind _returnvalue_4 (+ _reloadtime _firetime _recoverytime))
  (bind _returnvalue_5 (- _returnvalue_2 _returnvalue_3))
  (Utilities|IsValid _returnvalue
    (:Is%20Valid
      (if (< _returnvalue_2 _returnvalue_3)
        (Variables|Default|SetInitialReloadTime (- _returnvalue_3 _returnvalue_2))
        (else
          (Variables|Default|SetInitialReloadTime (- (* (Math|Conversions|ToFloat(Integer) (+ (.ReturnValue (Math|Float|Division(WholeandRemainder) _returnvalue_5 _returnvalue_4)) 1)) _returnvalue_4) _returnvalue_5))))
      (Variables|/Script/Engine.SkeletalMeshComponent|SetGlobalAnimRateScale _skeletalmesh (/ 1.0 (Variables|Default|GetInitialReloadTime)))
      (Components|Animation|PlayAnimation _skeletalmesh 0 false)
      (Utilities|FlowControl|Sequence
        (:then_0
          (Utilities|IsValid _reloadsound
            (:Is%20Valid
              (Audio|Components|Audio|SetSound _audio _reloadsound)
              (Audio|Components|Audio|Play _audio 0.0))))
        (:then_1
          (Utilities|Time|SetTimerbyEvent (delegate Custom|Fire) (Variables|Default|GetInitialReloadTime)))))
    (:Is%20Not%20Valid
      (Utilities|Time|SetTimerbyEvent (delegate Custom|SyncTreb) 6.0))))

(event EventBeginPlay
  (bind _reloadsound (Variables|Default|GetReloadSound))
  (bind _audio (Variables|Default|GetAudio))
  (bind _skeletalmesh (Variables|Default|GetSkeletalMesh))
  (Variables|/Script/Engine.SkeletalMeshComponent|SetGlobalAnimRateScale _skeletalmesh 0.0)
  (Components|Animation|PlayAnimation _skeletalmesh 0 false)
  (Networking|SwitchHasAuthority
    (:Authority
      (Variables|Default|SetInitialReloadTime (+ (Variables|Default|GetReloadTime) (Variables|Default|GetInitialDelay)))
      (Variables|/Script/Engine.SkeletalMeshComponent|SetGlobalAnimRateScale _skeletalmesh (/ 1.0 (Variables|Default|GetInitialReloadTime)))
      (Components|Animation|PlayAnimation _skeletalmesh 0 false)
      (Utilities|FlowControl|Sequence
        (:then_0
          (Utilities|IsValid _reloadsound
            (:Is%20Valid
              (Audio|Components|Audio|SetSound _audio _reloadsound)
              (Audio|Components|Audio|Play _audio 0.0))))
        (:then_1
          (Utilities|Time|SetTimerbyEvent (delegate Custom|Fire) (Variables|Default|GetInitialReloadTime)))))
    (:Remote
      (Utilities|Time|SetTimerbyEvent (delegate Custom|SyncTreb) 6.0))))

(fn ConstructionScript)