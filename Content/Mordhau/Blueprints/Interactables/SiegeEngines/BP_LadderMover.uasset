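; Drivable mover pawn that carries a character along a ladder, self-destroying on the server shortly after driving stops.
; Replicated Ladder sets a one-dimensional movement line between its start and end, and picks the exit point.
; Look and turn inputs drive the character's animation and first-person camera, while equipment, melee and ranged inputs forward to the Driver.
; Also plays step sounds and knocks drivers off with a trip and backward knockback.
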(event EventOnStepChanged
  (bind _driver (Variables|Default|GetDriver))
  (|CallParentFunction)
  (Utilities|IsValid _driver
    (:Is%20Valid
      (Class|AdvancedCharacter|PlayCharacterSound _driver "/Game/Mordhau/Audio/Cues/Footsteps/SC_LadderStep.SC_LadderStep" "Hips" (Math|Vector|MakeVector 0.0 0.0 0.0) "0, 0, 0" false 0 0.0 0.0))))

(event EventKnockOffDriver
  (params (Character :type Mordhau%20Character%20Object%20Reference))
  (Class|AdvancedCharacter|Trip Character)
  (Class|AdvancedCharacter|Knockback Character (* (Math|Conversions|ToVector(Vector2D) (Math|Vector2D|Normalize2D (Math|Conversions|ToVector2D(Vector) (Transformation|GetActorForwardVector)))) -1.75e+03)))

(event EventBeginPlay)

(event EventActorBeginOverlap
  (params (OtherActor :type Actor%20Object%20Reference)))

(event EventTick
  (params (DeltaSeconds :type Float%20%28single-precision%29)))

(event EventOnStoppedDriving
  (params (Character :type Mordhau%20Character%20Object%20Reference))
  (Networking|SwitchHasAuthority
    (:Authority
      (Actor|SetLifeSpan 0.5))))

(event EventUpdateAnimationfor
  (params (Character :type Mordhau%20Character%20Object%20Reference) (AnimInst :type Mordhau%20Anim%20Instance%20Object%20Reference) (DeltaTime :type Float%20%28single-precision%29))
  (|CallParentFunction Character AnimInst DeltaTime)
  (bind _asab_mordhau_character_animation (Utilities|Casting|CastToAB_MordhauCharacterAnimation AnimInst))
  (Variables|/Script/Mordhau.MordhauAnimInstance|SetVehicleTurn _asab_mordhau_character_animation (Variables|Default|GetSecondaryTurnValue))
  (Variables|/Script/Mordhau.MordhauAnimInstance|SetVehicleLookUp _asab_mordhau_character_animation (Variables|Default|GetLookUpValue))
  (Variables|/Script/Mordhau.MordhauAnimInstance|SetVehicleVelocity _asab_mordhau_character_animation (Math|Vector|VectorLength (- (Transformation|GetWorldLocation (Variables|Character|GetMesh)) (Transformation|GetWorldLocation (Variables|/Game/Mordhau/Blueprints/Interactables/SiegeEngines/BP_Ladder.BP_Ladder_C|GetLadderStart (Variables|Default|GetLadder)))))))

(event EventUpdateFPCamerafor
  (params (Character :type Mordhau%20Character%20Object%20Reference) (DeltaSeconds :type Float%20%28single-precision%29) (bRotationOnly :type Boolean))
  (|CallParentFunction Character DeltaSeconds bRotationOnly)
  (Class|MordhauCharacter|UpdateFPCamera Character DeltaSeconds (Variables|Default|GetLookUpValue) bRotationOnly (Math|Rotator|MakeRotator 0.0 0.0 (Variables|Default|GetSecondaryTurnValue))))

(event Input|ActionEvents|InputActionCycleCamera
  (params (Key :type Key%20Structure))
  (bind _driver (Variables|Default|GetDriver))
  (:Pressed
    (Utilities|IsValid _driver
      (:Is%20Valid
        (Class|MordhauCharacter|CycleCamera _driver)))))

(event Input|AxisEvents|InputAxisLookUp
  (params (AxisValue :type Float%20%28single-precision%29))
  (Class|AdvancedCharacter|LookUp AxisValue false))

(event Input|AxisEvents|InputAxisTurnRight
  (params (AxisValue :type Float%20%28single-precision%29))
  (Class|MordhauVehicle|SecondaryTurn AxisValue false))

(fn ConstructionScript
  (|CallParentFunction))

(fn OnRepLadder
  (bind _ladder (Variables|Default|GetLadder))
  (bind _asone_dimensional_movement_component (Utilities|Casting|CastToOneDimensionalMovementComponent (Variables|Character|GetCharacterMovement)))
  (Utilities|IsValid _ladder
    (:Is%20Valid
      (Class|OneDimensionalMovementComponent|SetMovementLine _asone_dimensional_movement_component (Transformation|GetWorldLocation (Variables|/Game/Mordhau/Blueprints/Interactables/SiegeEngines/BP_Ladder.BP_Ladder_C|GetLadderStart _ladder)) (Transformation|GetWorldLocation (Variables|/Game/Mordhau/Blueprints/Interactables/SiegeEngines/BP_Ladder.BP_Ladder_C|GetLadderEnd _ladder)))
      (Collision|IgnoreActorwhenMoving (Variables|Default|GetCapsuleComponent) _ladder true))))

(fn GetExitTransform
  (bind _ladder (Variables|Default|GetLadder))
  (bind _returnvalue (|CallParentFunction))
  (Utilities|IsValid _ladder
    (:Is%20Valid
      (if (< (Math|Vector|VectorLength (- (Transformation|GetWorldLocation (Variables|/Game/Mordhau/Blueprints/Interactables/SiegeEngines/BP_Ladder.BP_Ladder_C|GetLadderEnd _ladder)) (Transformation|GetActorLocation))) 5e+01)
        (return (Math|Transform|MakeTransform (Transformation|GetWorldLocation (Variables|/Game/Mordhau/Blueprints/Interactables/SiegeEngines/BP_Ladder.BP_Ladder_C|GetLadderExit _ladder)) (.Rotation (Math|Transform|BreakTransform _returnvalue)) (.Scale (Math|Transform|BreakTransform _returnvalue))))
        (else
          _)))
    (:Is%20Not%20Valid
      _))
  (return (Math|Transform|MakeTransform (+ (* (Math|Vector|GetForwardVector (Transformation|GetActorRotation (Variables|Default|GetLadder))) -5e+01) (.Location (Math|Transform|BreakTransform _returnvalue))) (.Rotation (Math|Transform|BreakTransform _returnvalue)) (.Scale (Math|Transform|BreakTransform _returnvalue)))))

(fn OverrideAttackAngle
  (params (Motion :type Attack%20Motion%20Object%20Reference))
  (return -1.0))

(event Input|ActionEvents|InputActionHolster
  (params (Key :type Key%20Structure))
  (bind _driver (Variables|Default|GetDriver))
  ;[1 1 1] Equipment
  (:Pressed
    (Utilities|IsValid _driver
      (:Is%20Valid
        (Class|MordhauCharacter|EmptyHands _driver)))))

(event Input|ActionEvents|InputActionDrop
  (params (Key :type Key%20Structure))
  (bind _driver (Variables|Default|GetDriver))
  ;[1 1 1] Equipment
  (:Pressed
    (Utilities|IsValid _driver
      (:Is%20Valid
        (Class|MordhauCharacter|RequestDrop _driver)))))

(event Input|ActionEvents|InputActionEquipSlot8
  (params (Key :type Key%20Structure))
  (bind _driver (Variables|Default|GetDriver))
  ;[1 1 1] Equipment
  (:Pressed
    (Utilities|IsValid _driver
      (:Is%20Valid
        (Class|MordhauCharacter|EquipSlot8 _driver)))))

(event Input|ActionEvents|InputActionEquipSlot9
  (params (Key :type Key%20Structure))
  (bind _driver (Variables|Default|GetDriver))
  ;[1 1 1] Equipment
  (:Pressed
    (Utilities|IsValid _driver
      (:Is%20Valid
        (Class|MordhauCharacter|EquipSlot9 _driver)))))

(event Input|ActionEvents|InputActionEquipSlot1
  (params (Key :type Key%20Structure))
  (bind _driver (Variables|Default|GetDriver))
  ;[1 1 1] Equipment
  (:Pressed
    (Utilities|IsValid _driver
      (:Is%20Valid
        (Class|MordhauCharacter|EquipSlot1 _driver)))))

(event Input|ActionEvents|InputActionWeaponMode/Reload
  (params (Key :type Key%20Structure))
  (bind _driver (Variables|Default|GetDriver))
  ;[1 1 1] Equipment
  (:Pressed
    (Utilities|IsValid _driver
      (:Is%20Valid
        (Class|MordhauCharacter|RequestToggleWeaponMode _driver)))))

(event Input|ActionEvents|InputActionEquipSlot2
  (params (Key :type Key%20Structure))
  (bind _driver (Variables|Default|GetDriver))
  ;[1 1 1] Equipment
  (:Pressed
    (Utilities|IsValid _driver
      (:Is%20Valid
        (Class|MordhauCharacter|EquipSlot2 _driver)))))

(event Input|ActionEvents|InputActionEquipSlot3
  (params (Key :type Key%20Structure))
  (bind _driver (Variables|Default|GetDriver))
  ;[1 1 1] Equipment
  (:Pressed
    (Utilities|IsValid _driver
      (:Is%20Valid
        (Class|MordhauCharacter|EquipSlot3 _driver)))))

(event Input|ActionEvents|InputActionEquipSlot4
  (params (Key :type Key%20Structure))
  (bind _driver (Variables|Default|GetDriver))
  ;[1 1 1] Equipment
  (:Pressed
    (Utilities|IsValid _driver
      (:Is%20Valid
        (Class|MordhauCharacter|EquipSlot4 _driver)))))

(event Input|ActionEvents|InputActionEquipSlot5
  (params (Key :type Key%20Structure))
  (bind _driver (Variables|Default|GetDriver))
  ;[1 1 1] Equipment
  (:Pressed
    (Utilities|IsValid _driver
      (:Is%20Valid
        (Class|MordhauCharacter|EquipSlot5 _driver)))))

(event Input|ActionEvents|InputActionEquipSlot6
  (params (Key :type Key%20Structure))
  (bind _driver (Variables|Default|GetDriver))
  ;[1 1 1] Equipment
  (:Pressed
    (Utilities|IsValid _driver
      (:Is%20Valid
        (Class|MordhauCharacter|EquipSlot6 _driver)))))

(event Input|ActionEvents|InputActionEquipSlot7
  (params (Key :type Key%20Structure))
  (bind _driver (Variables|Default|GetDriver))
  ;[1 1 1] Equipment
  (:Pressed
    (Utilities|IsValid _driver
      (:Is%20Valid
        (Class|MordhauCharacter|EquipSlot7 _driver)))))

(event Input|ActionEvents|InputActionLeftStab
  (params (Key :type Key%20Structure))
  (bind _driver (Variables|Default|GetDriver))
  ;[1 1 1] Melee combat
  (:Pressed
    (Utilities|IsValid _driver
      (:Is%20Valid
        (Class|MordhauCharacter|RequestLeftStab _driver)))))

(event Input|ActionEvents|InputActionFlipAttackSide
  (params (Key :type Key%20Structure))
  (bind _driver (Variables|Default|GetDriver))
  (bind _driver_2 (Variables|Default|GetDriver))
  ;[1 1 1] Melee combat
  (:Pressed
    (Utilities|IsValid _driver
      (:Is%20Valid
        (Class|MordhauCharacter|FlipAttackSidePressed _driver))))
  (:Released
    (Utilities|IsValid _driver_2
      (:Is%20Valid
        (Class|MordhauCharacter|FlipAttackSideReleased _driver_2)))))

(event Input|ActionEvents|InputActionFeint
  (params (Key :type Key%20Structure))
  (bind _driver (Variables|Default|GetDriver))
  ;[1 1 1] Melee combat
  (:Pressed
    (Utilities|IsValid _driver
      (:Is%20Valid
        (Class|MordhauCharacter|RequestFeint _driver)))))

(event Input|ActionEvents|InputActionStab
  (params (Key :type Key%20Structure))
  (bind _driver (Variables|Default|GetDriver))
  (bind _driver_2 (Variables|Default|GetDriver))
  ;[1 1 1] Melee combat
  (:Pressed
    (Utilities|IsValid _driver_2
      (:Is%20Valid
        (Class|MordhauCharacter|ListenforStab360 _driver_2))))
  (:Released
    (Utilities|IsValid _driver
      (:Is%20Valid
        (Class|MordhauCharacter|StopListenforStab360 _driver)))))

(event Input|ActionEvents|InputActionLeftUpperStrike
  (params (Key :type Key%20Structure))
  (bind _driver (Variables|Default|GetDriver))
  ;[1 1 1] Melee combat
  (:Pressed
    (Utilities|IsValid _driver
      (:Is%20Valid
        (Class|MordhauCharacter|RequestLeftUpperStrike _driver)))))

(event Input|ActionEvents|InputActionParry
  (params (Key :type Key%20Structure))
  (bind _driver (Variables|Default|GetDriver))
  ;[1 1 1] Melee combat
  (:Pressed
    (Utilities|IsValid _driver
      (:Is%20Valid
        (Class|MordhauCharacter|BlockPressed _driver))))
  (:Released
    (Utilities|IsValid _driver
      (:Is%20Valid
        (Class|MordhauCharacter|BlockReleased _driver)))))

(event Input|ActionEvents|InputActionFeintOrParry
  (params (Key :type Key%20Structure))
  (bind _driver (Variables|Default|GetDriver))
  ;[1 1 1] Melee combat
  (:Pressed
    (Utilities|IsValid _driver
      (:Is%20Valid
        (Class|MordhauCharacter|FeintorBlockPressed _driver))))
  (:Released
    (Utilities|IsValid _driver
      (:Is%20Valid
        (Class|MordhauCharacter|FeintorBlockReleased _driver)))))

(event Input|ActionEvents|InputActionRightUpperStrike
  (params (Key :type Key%20Structure))
  (bind _driver (Variables|Default|GetDriver))
  ;[1 1 1] Melee combat
  (:Pressed
    (Utilities|IsValid _driver
      (:Is%20Valid
        (Class|MordhauCharacter|RequestRightUpperStrike _driver)))))

(event Input|ActionEvents|InputActionRightLowerStrike
  (params (Key :type Key%20Structure))
  (bind _driver (Variables|Default|GetDriver))
  ;[1 1 1] Melee combat
  (:Pressed
    (Utilities|IsValid _driver
      (:Is%20Valid
        (Class|MordhauCharacter|RequestRightLowerStrike _driver)))))

(event Input|ActionEvents|InputActionRightStrike
  (params (Key :type Key%20Structure))
  (bind _driver (Variables|Default|GetDriver))
  ;[1 1 1] Melee combat
  (:Pressed
    (Utilities|IsValid _driver
      (:Is%20Valid
        (Class|MordhauCharacter|RequestRightStrike _driver)))))

(event Input|ActionEvents|InputActionStrike
  (params (Key :type Key%20Structure))
  (bind _driver (Variables|Default|GetDriver))
  (bind _driver_2 (Variables|Default|GetDriver))
  ;[1 1 1] Melee combat
  (:Pressed
    (Utilities|IsValid _driver_2
      (:Is%20Valid
        (Class|MordhauCharacter|ListenforStrike360 _driver_2))))
  (:Released
    (Utilities|IsValid _driver
      (:Is%20Valid
        (Class|MordhauCharacter|StopListenforStrike360 _driver)))))

(event Input|ActionEvents|InputActionRightStab
  (params (Key :type Key%20Structure))
  (bind _driver (Variables|Default|GetDriver))
  ;[1 1 1] Melee combat
  (:Pressed
    (Utilities|IsValid _driver
      (:Is%20Valid
        (Class|MordhauCharacter|RequestRightStab _driver)))))

(event Input|ActionEvents|InputActionLeftLowerStrike
  (params (Key :type Key%20Structure))
  (bind _driver (Variables|Default|GetDriver))
  ;[1 1 1] Melee combat
  (:Pressed
    (Utilities|IsValid _driver
      (:Is%20Valid
        (Class|MordhauCharacter|RequestLeftLowerStrike _driver)))))

(event Input|ActionEvents|InputActionLeftStrike
  (params (Key :type Key%20Structure))
  (bind _driver (Variables|Default|GetDriver))
  ;[1 1 1] Melee combat
  (:Pressed
    (Utilities|IsValid _driver
      (:Is%20Valid
        (Class|MordhauCharacter|RequestLeftStrike _driver)))))

(event Input|ActionEvents|InputActionRangedCancel
  (params (Key :type Key%20Structure))
  (bind _driver (Variables|Default|GetDriver))
  ;[1 1 1] Ranged
  (:Pressed
    (Utilities|IsValid _driver
      (:Is%20Valid
        (Class|MordhauCharacter|RequestRangedCancel _driver)))))

(event Input|ActionEvents|InputActionFire
  (params (Key :type Key%20Structure))
  (bind _driver (Variables|Default|GetDriver))
  (bind _driver_2 (Variables|Default|GetDriver))
  ;[1 1 1] Ranged
  (:Pressed
    (Utilities|IsValid _driver
      (:Is%20Valid
        (Class|MordhauCharacter|FirePressed _driver))))
  (:Released
    (Utilities|IsValid _driver_2
      (:Is%20Valid
        (Class|MordhauCharacter|FireReleased _driver_2)))))