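; Projectile Blueprint for thrown weapons that updates the weapon's trail and blood state when the projectile hits.
; On hit, it casts the projectile creator to MordhauEquipment and stops the thrown trail once the projectile has stopped.
; If that equipment is also a MordhauWeapon and the surface is SurfaceType1, it raises the weapon's blood level.
; A sequence node then runs the parent hit handler even when a cast fails.
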(event EventOnProjectileHit
  (params (HitLocation :type Vector%20%28by%20ref%29 :default "0, 0, 0") (HitNormal :type Vector%20%28by%20ref%29 :default "0, 0, 0") (BounceForce :type Float%20%28single-precision%29) (Surface :type Byte :default 0) (bHasHitWorld :type Boolean) (bHasStopped :type Boolean))
  (Utilities|FlowControl|Sequence
    (:then_0
      (bind _returnvalue (Class|MordhauProjectile|GetProjectileCreator))
      (bind _asmordhau_equipment (Utilities|Casting|CastToMordhauEquipment _returnvalue))
      (if bHasStopped
        (Class|MordhauEquipment|StopThrownTrail _asmordhau_equipment))
      (bind _asmordhau_weapon (Utilities|Casting|CastToMordhauWeapon _asmordhau_equipment))
      (if (== Surface (Utilities|Enum|LiteralenumEPhysicalSurface "SurfaceType1"))
        (Class|MordhauWeapon|IncreaseBloodLevel _asmordhau_weapon 3.0)))
    (:then_1
      (|CallParentFunction HitLocation HitNormal BounceForce Surface bHasHitWorld bHasStopped))))

(fn ConstructionScript
  (|CallParentFunction))