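; BP_Bullet1411 is a projectile variant that shakes cameras and spawns a BP_2HStickOgre where it hits.
; On each hit it plays a distance-attenuated world camera shake around the hit location.
; Only the authority spawns the actor, ignoring collision and without checking what was hit or whether the projectile stopped.
; The hit is then passed to the parent projectile's handling.
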(event EventBeginPlay
  (|CallParentFunction) ; This node is disabled and will not be called.\nDrag off pins to build functionality.
)

(event Collision|EventActorBeginOverlap
  (params (OtherActor :type Actor%20Object%20Reference))
  (|CallParentFunction OtherActor) ; This node is disabled and will not be called.\nDrag off pins to build functionality.
)

(event EventTick
  (params (DeltaSeconds :type Float%20%28single-precision%29))
  (|CallParentFunction DeltaSeconds) ; This node is disabled and will not be called.\nDrag off pins to build functionality.
)

(event EventOnProjectileHit
  (params (HitLocation :type Vector%20%28by%20ref%29 :default "0, 0, 0") (HitNormal :type Vector%20%28by%20ref%29 :default "0, 0, 0") (BounceForce :type Float%20%28single-precision%29) (Surface :type Byte :default 0) (bHasHitWorld :type Boolean) (bHasStopped :type Boolean))
  (Utilities|FlowControl|Sequence
    (:then_0
      (Camera|PlayWorldCameraShake 0 HitLocation 5e+02 1.5e+04 1e+01))
    (:then_2
      (Networking|SwitchHasAuthority
        (:Authority
          (Game|SpawnActorfromClass "/Game/Mordhau/Blueprints/Equipment/Weapons/Specific/TwoHandedBlunt/BP_2HStickOgre.BP_2HStickOgre_C" (Math|Transform|MakeTransform HitLocation) "AlwaysSpawn" 0 0))))
    (:then_3
      (|CallParentFunction HitLocation HitNormal BounceForce Surface bHasHitWorld bHasStopped))))

(fn ConstructionScript
  (|CallParentFunction))