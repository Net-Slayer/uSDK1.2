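; Placeable bear trap equipment that damages characters and horses stepping on it, tripping humans; crouching characters are spared.
; Firing plants it on a validated ground spot (slope, nearby traps, team areas) under a per-player limit.
; IsLoaded false means planted: overlap arms after a safe delay, and only the planter can retrieve it.
; Zero ammo means sprung, via overlap or damage; it expires afterwards or when the planter dies.
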(event Custom|PlanterDied
  (params (Character :type Advanced%20Character%20Object%20Reference))
  (if (<= (Actor|GetLifeSpan) 0.0)
    (Networking|SwitchHasAuthority
      (:Authority
        (Actor|SetLifeSpan 5.0)))))

(event Custom|PlanterDestroyed
  (params (Character :type Advanced%20Character%20Object%20Reference))
  (if (<= (Actor|GetLifeSpan) 0.0)
    (Networking|SwitchHasAuthority
      (:Authority
        (Actor|SetLifeSpan 5.0)))))

(event EventOnHeldInteractionStart
  (params (Character :type Mordhau%20Character%20Object%20Reference))
  (if (Variables|Default|GetbIsLoaded)
    _
    (else
      (Class|MordhauEquipment|SetLoaded true)))
  (|CallParentFunction Character))

(event EventOnLoadedChanged
  (bind _box (Variables|Default|GetBox))
  (bind _box_2 (Variables|Default|GetBox))
  (bind _bisloaded (Variables|Default|GetbIsLoaded))
  (bind _plantercharacter (Variables|Default|GetPlanterCharacter))
  (|CallParentFunction)
  (Variables|Default|SetbCanRagdoll _bisloaded)
  (Utilities|FlowControl|Sequence
    (:then_0
      (if _bisloaded
        (Utilities|FlowControl|Sequence
          (:then_0
            (Networking|SwitchHasAuthority
              (:Authority
                (Transformation|DetachFromActor "KeepWorld" "KeepWorld" "KeepWorld")
                (bind _asbp_mordhau_player_controller (Utilities|Casting|CastToBP_MordhauPlayerController (Variables|Default|GetPlanterController)))
                (Default|RemovefromPlaceableArray _asbp_mordhau_player_controller (Variables|Default|GetPlaceableLimitName) self))))
          (:then_1
            (Utilities|IsValid _plantercharacter
              (:Is%20Valid
                (EventDispatchers|UnbindEventfromOnCharacterDied _plantercharacter (delegate Custom|PlanterDied))
                (EventDispatchers|UnbindEventfromOnCharacterDestroyed _plantercharacter (delegate Custom|PlanterDestroyed)))))
          (:then_2
            (Utilities|IsValid _box_2
              (:Is%20Valid
                (Collision|SetCollisionEnabled _box_2 "NoCollision")
                (Variables|/Script/Engine.PrimitiveComponent|SetbGenerateOverlapEvents _box_2 false)))))
        (else
          (Networking|SwitchHasAuthority
            (:Authority
              (Utilities|FlowControl|RetriggerableDelay (Variables|Default|GetSafeTime))
              (Utilities|IsValid self
                (:Is%20Valid
                  (if (not (Variables|Default|GetbIsLoaded))
                    (Utilities|IsValid _box :!label _label
                      (:Is%20Valid
                        (Collision|SetCollisionEnabled _box "QueryOnly")
                        (Variables|/Script/Engine.PrimitiveComponent|SetbGenerateOverlapEvents _box true)))))))
            (:Remote
              (goto _label))))))
    (:then_1
      (Class|MordhauEquipment|UpdateEquipmentState))))

(event Collision|EventActorBeginOverlap
  (params (OtherActor :type Actor%20Object%20Reference))
  (Networking|SwitchHasAuthority
    (:Authority
      (bind _asadvanced_character (Utilities|Casting|CastToAdvancedCharacter OtherActor))
      (if (Math|Boolean|ANDBoolean (not (stale _returnvalue)) (Ability|HasAuthority _asadvanced_character) (not (AI|Components|NavMovement|IsCrouching (Variables|/Script/Engine.Character|GetCharacterMovement _asadvanced_character))))
        (Utilities|FlowControl|Sequence
          (:then_0
            (Class|MordhauEquipment|SetAmmo))
          (:then_1
            (CallFunction|DealDamage _asadvanced_character)))))))

(event EventOnUsedtoKillOther
  (params (Character :type Advanced%20Character%20Object%20Reference) (Type :type EMordhauDamageType%20Enum :default "Generic") (SubType :type Byte :default 0) (bone :type Name%20%28by%20ref%29 :default "None") (Point :type Vector%20%28by%20ref%29 :default "0, 0, 0") (Source :type Actor%20Object%20Reference))
  (|CallParentFunction Character Type SubType bone Point Source)
  (bind _asmordhau_character (Utilities|Casting|CastToMordhauCharacter Character)))

(event EventOnPostDismemberedOther
  (params (bone :type Name%20%28by%20ref%29 :default "None") (Part :type Separated%20Body%20Part%20Object%20Reference))
  (Physics|SetSimulatePhysics (Variables|/Script/Mordhau.SeparatedBodyPart|GetMesh Part) false)
  (Transformation|AttachComponentToComponent Part (Variables|Default|GetSkeletalMeshComponent) "FootAttachPoint" "SnapToTarget" "KeepWorld" "KeepWorld" false))

(event EventOnAmmoChanged
  (bind _box (Variables|Default|GetBox))
  (|CallParentFunction)
  (if (== (Class|MordhauEquipment|GetAmmo) 0)
    (Variables|Default|SetbIsInteractable false)
    (Components|Animation|PlayAnimation (Variables|Default|GetSkeletalMeshComponent) 0 false)
    (Audio|SpawnSoundatLocation (Variables|Default|GetTrapTriggerSound) (Transformation|GetWorldLocation (Variables|Default|GetSkeletalMeshComponent)) "0, 0, 0" 1.0 1.0 0.0 0 0)
    (Utilities|FlowControl|Sequence
      (:then_0
        (Utilities|IsValid _box
          (:Is%20Valid
            (Components|DestroyComponent _box))))
      (:then_1
        (Networking|SwitchHasAuthority
          (:Authority
            (Actor|SetLifeSpan 1e+01)
            (bind _asbp_mordhau_player_controller (Utilities|Casting|CastToBP_MordhauPlayerController (Variables|Default|GetPlanterController)))
            (Default|RemovefromPlaceableArray _asbp_mordhau_player_controller (Variables|Default|GetPlaceableLimitName) self)))))))

(event EventOnInteractionStart
  (params (Character :type Mordhau%20Character%20Object%20Reference))
  (if (Variables|Default|GetbIsLoaded)
    _
    (else
      (Class|MordhauEquipment|SetLoaded true)))
  (|CallParentFunction Character))

(event EventFireProjectile
  (params (Origin :type Vector%20%28by%20ref%29 :default "0, 0, 0") (Orientation :type Rotator%20%28by%20ref%29 :default "0, 0, 0") (OwningController :type Controller%20Object%20Reference) (ExpectedDelay :type Float%20%28single-precision%29))
  (bind _returnvalue (Class|MordhauEquipment|GetParentCharacter))
  (Audio|SpawnSoundAttached (Variables|Default|GetFireSound) (Variables|Default|GetSkeletalMeshComponent) "None" "0, 0, 0" "0, 0, 0" "SnapToTarget" false 1.0 1.0 0.0 0 0)
  (Variables|Default|SetPlanterController 0)
  (Variables|Default|SetPlanterCharacter 0)
  (Utilities|IsValid _returnvalue
    (:Is%20Valid
      (bind _output_get (Variables|Default|SetPlanterCharacter _returnvalue))
      (Variables|Default|SetPlanterController (Pawn|GetController _output_get))
      (Networking|SwitchHasAuthority
        (:Authority
          (EventDispatchers|BindEventtoOnCharacterDied _output_get (delegate Custom|PlanterDied))
          (EventDispatchers|BindEventtoOnCharacterDestroyed _output_get (delegate Custom|PlanterDestroyed))
          (bind (_succeeded _location _rotation _attachtocomponent) (CallFunction|ValidatePlantSpot (Transformation|GetActorLocation _returnvalue) Orientation))
          (if _succeeded
            (Utilities|FlowControl|Sequence
              (:then_0
                (bind _asbp_mordhau_player_controller (Utilities|Casting|CastToBP_MordhauPlayerController (Variables|Default|GetPlanterController)))
                (bind _removedactor (Default|PlaceinPlaceableArray _asbp_mordhau_player_controller (Variables|Default|GetPlaceableLimitName) self (Variables|Default|GetMaxTrapsPerPlayer)))
                (Utilities|IsValid _removedactor
                  (:Is%20Valid
                    (Actor|DestroyActor _removedactor))))
              (:then_1
                (Class|MordhauEquipment|SetLoaded false)
                (Class|MordhauCharacter|DropEquipment _returnvalue self)
                (Transformation|SetActorLocationAndRotation _location _rotation)
                (Transformation|AttachComponentToComponent _attachtocomponent "None" "KeepWorld" "KeepWorld" "KeepWorld" false)))))))))

(event Game|Damage|EventAnyDamage
  (params (Damage :type Float%20%28single-precision%29) (DamageType :type Damage%20Type%20Object%20Reference) (InstigatedBy :type Controller%20Object%20Reference) (DamageCauser :type Actor%20Object%20Reference))
  (Class|MordhauEquipment|SetAmmo))

(fn ConstructionScript)

(fn OnRequestFire
  (params (Character :type Mordhau%20Character%20Object%20Reference))
  (bind _returnvalue (Class|AdvancedCharacter|IsAirborne Character))
  (if _returnvalue
    _
    (else
      (bind _succeeded (CallFunction|ValidatePlantSpot (Transformation|GetActorLocation Character) (Variables|/Script/Mordhau.MordhauCharacter|GetCameraRotation1P Character)))
      (if _succeeded
        (bind _returnvalue_2 (|CallParentFunction Character))
        (return _returnvalue_2)
        (else
          _))))
  (Variables|/Script/Mordhau.MordhauCharacter|SetbWantsFire Character false)
  (Class|MordhauCharacter|OnActionFailed Character (Utilities|Name|MakeLiteralName "None"))
  (return false))

(fn ValidatePlantSpot
  (params (CameraLocation1P :type Vector) (CameraRotattion1P :type Rotator))
  (bind _yaw (Math|Rotator|BreakRotator CameraRotattion1P))
  (bind _array (Utilities|Array|MakeArray "ObjectTypeQuery1"))
  (bind _returnvalue (Math|Rotator|MakeRotator 0.0 0.0 _yaw))
  (bind _returnvalue_2 (Math|Vector|GetForwardVector _returnvalue))
  (bind _returnvalue_3 (Math|Vector|GetRightVector _returnvalue))
  (bind _returnvalue_4 (* _returnvalue_2 5e+01))
  (bind _returnvalue_5 (* _returnvalue_2 1e+02))
  (bind _returnvalue_6 (+ CameraLocation1P _returnvalue_5))
  (bind _returnvalue_7 (+ CameraLocation1P _returnvalue_4))
  (bind _returnvalue_8 (+ _returnvalue_6 _returnvalue_7))
  (bind _returnvalue_9 (* _returnvalue_8 0.5))
  (bind (_lefthit _righthit _forwardhit _backhit _outright _outforward _returnvalue_10) (Class|MordhauUtilityLibrary|PlaneTrace (+ _returnvalue_9 (* _returnvalue_3 -25.0)) (+ _returnvalue_9 (* _returnvalue_3 25.0)) _returnvalue_6 _returnvalue_7 "0, 0,-150.000000" _array false 0 false true "0, 0,10.000000" true))
  (if _returnvalue_10
    (LocalVariables|SetMiddleSpot (* (+ (.ImpactPoint (Collision|BreakHitResult _forwardhit)) (.ImpactPoint (Collision|BreakHitResult _backhit))) 0.5))
    (bind _output_get (LocalVariables|SetFoundRot (Class|KismetMathLibrary|MakeRotfromYX _outforward (* _outright -1.0))))
    (if (< (Class|KismetMathLibrary|DegAcos (Math|Vector|DotProduct (Math|Vector|GetUpVector _output_get) "0, 0,1.000000")) 45.0)
      (bind _outactors (Collision|SphereOverlapActors (LocalVariables|GetMiddleSpot) 64.0 _array "BP_BearTrap_C"))
      (for _array_element _outactors
        (bind _asbp_bear_trap (Utilities|Casting|CastToBP_BearTrap _array_element))
        (if (not (Variables|/Script/Mordhau.MordhauEquipment|GetbIsLoaded _asbp_bear_trap))
          (return false "0, 0, 0" "0, 0, 0" 0)))
      (Utilities|IsValid (Class|MordhauEquipment|GetParentCharacter)
        (:Is%20Valid
          (if (stale _returnvalue)
            _
            (else
              (return true (LocalVariables|GetMiddleSpot) (LocalVariables|GetFoundRot) (.HitComponent (Collision|BreakHitResult _forwardhit))))))
        (:Is%20Not%20Valid
          _))))
  (return false "0, 0, 0" "0, 0, 0" 0))

(fn DealDamage
  (params (Character :type Advanced%20Character%20Object%20Reference))
  (bind _skeletalmeshcomponent (Variables|Default|GetSkeletalMeshComponent))
  (bind _returnvalue (Transformation|GetWorldLocation _skeletalmeshcomponent))
  (LocalVariables|SetDamageFactor 1.0)
  (bind _output_get (LocalVariables|SetEventInstigator (Variables|Default|GetPlanterController)))
  (Utilities|FlowControl|Sequence
    (:then_0
      (if (== (Pawn|GetController Character) _output_get)
        (LocalVariables|SetEventInstigator 0 :!label _label)
        (bind _asmordhau_game_mode (Utilities|Casting|CastToMordhauGameMode (Game|GetGameMode)))
        (LocalVariables|SetDamageFactor (Variables|/Script/Mordhau.MordhauGameMode|GetTeamDamageFactor _asmordhau_game_mode))
        (else
          (bind _asmordhau_game_state (Utilities|Casting|CastToMordhauGameState (Game|GetGameState)))
          (bind _returnvalue_2 (Class|MordhauGameState|IsFriendly _asmordhau_game_state Character (LocalVariables|GetEventInstigator)))
          (if _returnvalue_2
            (goto _label)))))
    (:then_1
      (bind _asmordhau_character (Utilities|Casting|CastToMordhauCharacter Character)
        (:then
          (bind _output_get_2 (LocalVariables|SetMordhauCharacter _asmordhau_character))
          (bind _returnvalue_3 (Class|AdvancedCharacter|GetArmorTierforBone _output_get_2 (Utilities|Name|MakeLiteralName "None")))
          (Utilities|FlowControl|Sequence
            (:then_0
              (LocalVariables|SetClosestFoot "RightFoot")
              (bind _output_get_3 (LocalVariables|SetClosestFootDistance (Math|Vector|VectorLength (- (Transformation|GetSocketLocation (Variables|/Script/Engine.Character|GetMesh (LocalVariables|GetMordhauCharacter)) "RightFoot") _returnvalue))))
              (if (> _output_get_3 (Math|Vector|VectorLength (- (Transformation|GetSocketLocation (Variables|/Script/Engine.Character|GetMesh (LocalVariables|GetMordhauCharacter)) "LeftFoot") _returnvalue)))
                (LocalVariables|SetClosestFoot "LeftFoot")))
            (:then_1
              (Class|AdvancedCharacter|MordhauTakeDamage (LocalVariables|GetMordhauCharacter) (* (Utilities|Array|Get(acopy) (Variables|Default|GetDamageByArmorTier) (Math|Conversions|ToInteger(Byte) _returnvalue_3)) (LocalVariables|GetDamageFactor)) (Collision|MakeHitResult false false 0.0 0.0 "0, 0, 0" (Transformation|GetSocketLocation _skeletalmeshcomponent (LocalVariables|GetClosestFoot)) "0,0,1" "0,0,1" 0 0 0 (LocalVariables|GetClosestFoot)) "Generic" 0 self self (LocalVariables|GetEventInstigator)))
            (:then_2
              (if (not (stale _returnvalue))
                (Class|AdvancedCharacter|Trip (LocalVariables|GetMordhauCharacter))
                (Class|AdvancedCharacter|Knockback (LocalVariables|GetMordhauCharacter) (Math|Conversions|ToVector(Vector2D) (* (Math|Vector2D|Normalize2D (Math|Conversions|ToVector2D(Vector) (- (Transformation|GetActorLocation) (Transformation|GetActorLocation (LocalVariables|GetMordhauCharacter))))) 2e+02)))))))
        (:CastFailed
          (bind _ashorse (Utilities|Casting|CastToHorse Character))
          (Class|AdvancedCharacter|MordhauTakeDamage _ashorse (* (Variables|Default|GetDamageToHorse) (LocalVariables|GetDamageFactor)) (Collision|MakeHitResult false false 0.0 0.0 "0, 0, 0" "0, 0, 0" "0,0,1" "0,0,1" 0 0) "Generic" 0 self self (LocalVariables|GetEventInstigator)))))))

(fn CanInteract
  (params (Character :type Mordhau%20Character%20Object%20Reference))
  (if (Variables|Default|GetbIsLoaded)
    _
    (else
      (Utilities|IsValid Character
        (:Is%20Valid
          (if (== (Pawn|GetController Character) (Variables|Default|GetPlanterController))
            _
            (else
              (return false))))
        (:Is%20Not%20Valid
          _))))
  (return (stale _returnvalue)))

(fn ShouldShine
  (if (Variables|Default|GetbIsLoaded)
    (bind _returnvalue (|CallParentFunction))
    (return _returnvalue)
    (else
      (return false))))

(fn CanHeldInteract
  (params (Character :type Mordhau%20Character%20Object%20Reference))
  (Utilities|IsValid Character
    (:Is%20Valid
      (if (Variables|Default|GetbIsLoaded)
        _
        (elif (== (Pawn|GetController Character) (Variables|Default|GetPlanterController))
          _
          (else
            (return false)))))
    (:Is%20Not%20Valid
      _))
  (return (stale _returnvalue)))