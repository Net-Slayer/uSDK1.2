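; Interactable equipment pickup point with a limited, self-restocking supply of one equipment class.
; Interaction decrements Ammo, spawns the equipment for the character to pick up, and starts a timer chain that refills one unit per interval until full.
; Ammo's RepNotify shows one mesh per unit, disables interaction when empty, and plays restock or grab effects after the first seconds.
; Characters already holding that equipment in the right hand cannot interact.
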(event Custom|ReplenishAmmo
  (Variables|Default|SetAmmo (+ (Variables|Default|GetAmmo) 1))
  (if (== (Variables|Default|GetAmmo) (Variables|Default|GetMaxAmmo))
    (Variables|Default|SetReplenishingAmmo false)
    (else
      (Utilities|Time|SetTimerbyEvent (delegate Custom|ReplenishAmmo) (Variables|Default|GetAmmoReplenishInterval)))))

(event EventBeginPlay
  (|CallParentFunction)
  (Networking|SwitchHasAuthority
    (:Authority
      (Variables|Default|SetAmmo (Variables|Default|GetMaxAmmo)))))

(event Collision|EventActorBeginOverlap
  (params (OtherActor :type Actor%20Object%20Reference))
  (|CallParentFunction OtherActor) ; This node is disabled and will not be called.\nDrag off pins to build functionality.
)

(event EventTick
  (params (DeltaSeconds :type Float%20%28single-precision%29))
  (|CallParentFunction DeltaSeconds) ; This node is disabled and will not be called.\nDrag off pins to build functionality.
)

(event EventOnInteractionStart
  (params (Character :type Mordhau%20Character%20Object%20Reference))
  (Variables|Default|SetAmmo (- (Variables|Default|GetAmmo) 1))
  (Utilities|FlowControl|Sequence
    (:then_0
      (if (not (Variables|Default|GetReplenishingAmmo))
        (Variables|Default|SetReplenishingAmmo true)
        (Utilities|Time|SetTimerbyEvent (delegate Custom|ReplenishAmmo) (Variables|Default|GetAmmoReplenishInterval))))
    (:then_1
      (bind _returnvalue (Game|SpawnActorfromClass (Variables|Default|GetEquipment) (Transformation|GetActorTransform Character) "Undefined" 0 0))
      (bind _asmordhau_equipment (Utilities|Casting|CastToMordhauEquipment _returnvalue))
      (Class|MordhauCharacter|PickUp Character _asmordhau_equipment))))

(fn ConstructionScript
  (|CallParentFunction))

(fn CanInteract
  (params (Character :type Mordhau%20Character%20Object%20Reference))
  (Utilities|IsValid Character
    (:Is%20Valid
      (if (== (Utilities|GetClass (Variables|/Script/Mordhau.MordhauCharacter|GetRightHandEquipment Character)) (Variables|Default|GetEquipment))
        (return false)
        (else
          _)))
    (:Is%20Not%20Valid
      _))
  (return (stale _returnvalue)))

(fn OnRepAmmo
  (bind _ammo (Variables|Default|GetAmmo))
  (for (_array_element _array_index) (Variables|Default|GetMeshes)
    (Development|SetHiddeninGame _array_element (< _ammo (Math|Conversions|ToByte(Integer) (+ _array_index 1))) false))
  (Variables|Default|SetbIsInteractable (> _ammo 0))
  (Utilities|FlowControl|Sequence
    (:then_0
      (if (> (Utilities|Time|GetTimeSeconds) 4.0)
        (if (> _ammo (Variables|Default|GetPreviousAmmo))
          (Components|Activation|Activate (Variables|Default|GetSC_RockSpawner) false)
          (else
            (Components|Activation|Activate (Variables|Default|GetSC_Grab) false)))))
    (:then_1
      (Variables|Default|SetPreviousAmmo _ammo))))