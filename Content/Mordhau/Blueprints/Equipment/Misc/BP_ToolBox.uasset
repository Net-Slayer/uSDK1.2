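; Toolbox equipment that lets a player build placeable objects, cycled by mode switch and paid for with ammo.
; Each tick it shows a preview mesh placed by ValidateSpot, which traces ahead for slope, clearance, line of sight and restricted areas.
; Firing sends the spot relative to the hit component to the server, which rechecks distance and cost, then spawns and usually attaches the object.
; Exceeding a per-player limit kills or destroys the returned placeable.
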(event Custom|ServerRequestPlant
  (params (Location :type Vector) (Rotation :type Rotator) (ObjectType :type Byte) (AttachTo :type Scene%20Component%20Object%20Reference))
  (CallFunction|RequestPlant Location Rotation ObjectType AttachTo))

(event EventUpdateEquipmentState
  (|CallParentFunction)
  (CallFunction|DestroyMeshPreview))

(event EventLocalPlayerLateTick
  (params (DeltaTime :type Float%20%28single-precision%29))
  (bind _returnvalue (Class|MordhauEquipment|GetAmmo))
  (bind _returnvalue_2 (Class|MordhauEquipment|GetParentCharacter))
  (bind _previewmeshcomponent (Variables|Default|GetPreviewMeshComponent))
  (bind _spawnableobjects (Variables|Default|GetSpawnableObjects))
  (bind _objecttype (Variables|Default|GetObjectType))
  (bind _output (Utilities|Array|Get(acopy) _spawnableobjects _objecttype))
  (bind (_preview _previewskeletal _cost _rotationoffset _rotationoffsetpreview _scalepreview) (Utilities|Struct|BreakBP_ToolBoxSpawnable _output))
  (bind _returnvalue_3 (< _returnvalue _cost))
  (if (or (<= (Utilities|Time|GetTimeSeconds) (Variables|Default|GetNextAvailableTime)) _returnvalue_3)
    (CallFunction|DestroyMeshPreview)
    (if _returnvalue_3
      (CallFunction|CycleObjectType))
    (else
      (Utilities|IsValid _preview
        (:Is%20Valid
          (CallFunction|AddStaticMeshPreviewifNone _preview))
        (:Is%20Not%20Valid
          (Utilities|IsValid _previewskeletal
            (:Is%20Valid
              (CallFunction|AddSkeletalMeshPreviewifNone _previewskeletal)))))
      (bind (_succeeded _location _rotation) (CallFunction|ValidateSpot (Transformation|GetActorLocation _returnvalue_2) (Variables|/Script/Mordhau.MordhauCharacter|GetCameraRotation1P _returnvalue_2) "0, 0, 0"))
      (Transformation|SetWorldTransform _previewmeshcomponent (Math|Transform|MakeTransform _location (Math|Rotator|CombineRotators _rotationoffsetpreview _rotation) _scalepreview) false false)
      (Rendering|Material|SetScalarParameterValueonMaterials _previewmeshcomponent "Valid" (Math|Conversions|ToFloat(Boolean) _succeeded)))))

(fn ConstructionScript)

(fn OnRequestFire
  (params (Character :type Mordhau%20Character%20Object%20Reference))
  (bind _returnvalue (Class|MordhauEquipment|GetParentCharacter))
  (bind _returnvalue_2 (Utilities|Time|GetTimeSeconds))
  (bind _spawnableobjects (Variables|Default|GetSpawnableObjects))
  (bind _objecttype (Variables|Default|GetObjectType))
  (bind _output (Utilities|Array|Get(acopy) _spawnableobjects _objecttype))
  (bind (_preview _previewskeletal _cost _rotationoffset _rotationoffsetpreview _scalepreview _class _placeablelimitname _pleaceablelimitmax _performcapsulecheck _capsulecheckradius _capsulecheckhalfheight _spawnactoroffset) (Utilities|Struct|BreakBP_ToolBoxSpawnable _output))
  (Utilities|IsValid Character
    (:Is%20Valid
      (Variables|/Script/Mordhau.MordhauCharacter|SetbWantsFire Character false))
    (:Is%20Not%20Valid
      _))
  (if (and (> _returnvalue_2 (Variables|Default|GetNextAvailableTime)) (>= (Class|MordhauEquipment|GetAmmo) _cost))
    (bind (_succeeded _location _rotation _attachtocomponent) (CallFunction|ValidateSpot (Transformation|GetActorLocation _returnvalue) (Variables|/Script/Mordhau.MordhauCharacter|GetCameraRotation1P _returnvalue) "0, 0, 0"))
    (if _succeeded
      (Variables|Default|SetNextAvailableTime (+ _returnvalue_2 (Variables|Default|GetCooldown)))
      (CallFunction|ServerRequestPlant (Math|Transform|InverseTransformLocation (Transformation|GetWorldTransform _attachtocomponent) (+ _location (Math|Vector|RotateVector _spawnactoroffset (Math|Rotator|CombineRotators _rotationoffset _rotation)))) (Math|Transform|InverseTransformRotation (Transformation|GetWorldTransform _attachtocomponent) (Math|Rotator|CombineRotators _rotationoffset _rotation)) (Math|Conversions|ToByte(Integer) (Variables|Default|GetObjectType)) _attachtocomponent)))
  (return false))

(fn OnRequestModeSwitch
  (params (Character :type Mordhau%20Character%20Object%20Reference))
  (CallFunction|CycleObjectType)
  (return true))

(fn ValidateSpot
  (params (PlanterLocation :type Vector) (CameraRotation1P :type Rotator) (Offset :type Vector))
  (bind _yaw (Math|Rotator|BreakRotator CameraRotation1P))
  (bind _array (Utilities|Array|MakeArray "ObjectTypeQuery1" "ObjectTypeQuery5" "ObjectTypeQuery3"))
  (bind _spawnableobjects (Variables|Default|GetSpawnableObjects))
  (bind _objecttype (Variables|Default|GetObjectType))
  (bind _returnvalue (Math|Rotator|MakeRotator 0.0 0.0 _yaw))
  (bind _output (Utilities|Array|Get(acopy) _spawnableobjects _objecttype))
  (bind (_preview _previewskeletal _cost _rotationoffset _rotationoffsetpreview _scalepreview _class _placeablelimitname _pleaceablelimitmax _performcapsulecheck _capsulecheckradius _capsulecheckhalfheight) (Utilities|Struct|BreakBP_ToolBoxSpawnable _output))
  (bind _returnvalue_2 (Math|Vector|GetForwardVector _returnvalue))
  (bind _returnvalue_3 (Math|Vector|GetRightVector _returnvalue))
  (bind _returnvalue_4 (* _returnvalue_2 2e+02))
  (bind _returnvalue_5 (+ PlanterLocation _returnvalue_4))
  (bind (_lefthit _righthit _forwardhit _backhit _outright _outforward _returnvalue_6) (Class|MordhauUtilityLibrary|PlaneTrace (+ (* _returnvalue_3 -25.0) _returnvalue_5) (+ _returnvalue_5 (* _returnvalue_3 25.0)) _returnvalue_5 (+ PlanterLocation (* _returnvalue_2 1e+02)) "0, 0,-150.000000" _array false 0 false true "0, 0,10.000000" true))
  (if _returnvalue_6
    (Utilities|FlowControl|Sequence
      (:then_0
        (Utilities|Casting|CastToBP_DestroyableActor (.HitActor (Collision|BreakHitResult _forwardhit))
          (:CastFailed
            (LocalVariables|SetValidBase true))))
      (:then_1
        (bind _output_get (LocalVariables|SetFoundRot (Math|Rotator|MakeRotfromXY (* _outforward -1.0) (* _outright -1.0))))
        (if (and (< (Class|KismetMathLibrary|DegAcos (Math|Vector|DotProduct (Math|Vector|GetUpVector _output_get) "0, 0,1.000000")) 2e+01) (LocalVariables|GetValidBase))
          (if (> _capsulecheckradius 0.0)
            (bind _returnvalue_7 (Class|KismetSystemLibrary|BoxTraceSingleforObjects (+ (Math|Vector|RotateVector (Math|Vector|MakeVector 0.0 0.0 (+ _capsulecheckhalfheight 2.0)) (LocalVariables|GetFoundRot)) (+ (.ImpactPoint (Collision|BreakHitResult _forwardhit)) (Math|Vector|RotateVector Offset (LocalVariables|GetFoundRot)))) (+ (Math|Vector|RotateVector (Math|Vector|MakeVector 0.0 0.0 (+ _capsulecheckhalfheight 2.0)) (LocalVariables|GetFoundRot)) (+ (.ImpactPoint (Collision|BreakHitResult _forwardhit)) (Math|Vector|RotateVector Offset (LocalVariables|GetFoundRot)))) (Math|Vector|MakeVector _capsulecheckradius _capsulecheckradius _capsulecheckhalfheight) (LocalVariables|GetFoundRot) _array false 0 "None" true))
            (if _returnvalue_7
              _
              (else
                (bind _returnvalue_8 (Collision|LineTraceForObjects PlanterLocation (+ (+ (.ImpactPoint (Collision|BreakHitResult _forwardhit)) (Math|Vector|RotateVector Offset (LocalVariables|GetFoundRot))) "0, 0,50.000000") (Utilities|Array|MakeArray "ObjectTypeQuery1") false 0 "None" :!label _label))
                (if _returnvalue_8
                  _
                  (else
                    (bind _asbp_mordhau_character (Utilities|Casting|CastToBP_MordhauCharacter (Class|MordhauEquipment|GetParentCharacter))
                      (:then
                        (if (or (stale _returnvalue) (> (Variables|/Game/Mordhau/Blueprints/Characters/BP_MordhauCharacter.BP_MordhauCharacter_C|GetToolboxPreventionAreaCounter _asbp_mordhau_character) 0))
                          _
                          (else
                            (return true (+ (.ImpactPoint (Collision|BreakHitResult _forwardhit)) (Math|Vector|RotateVector Offset (LocalVariables|GetFoundRot))) (LocalVariables|GetFoundRot) (.HitComponent (Collision|BreakHitResult _forwardhit))))))
                      (:CastFailed
                        _))))))
            (else
              (goto _label))))
        (return false (+ (.ImpactPoint (Collision|BreakHitResult _forwardhit)) (Math|Vector|RotateVector Offset (LocalVariables|GetFoundRot))) (LocalVariables|GetFoundRot) 0)))
    (else
      (return false (+ _returnvalue_5 "0, 0,-150.000000") (Math|Rotator|CombineRotators _returnvalue "0,180.000000, 0") 0))))

(fn RequestPlant
  (params (Location :type Vector) (Rotation :type Rotator) (ObjectType :type Byte) (AttachTo :type Scene%20Component%20Object%20Reference))
  (bind _returnvalue (Class|MordhauEquipment|GetParentCharacter))
  (bind _returnvalue_2 (Transformation|GetWorldTransform AttachTo))
  (bind _returnvalue_3 (Class|MordhauEquipment|GetAmmo))
  (bind _returnvalue_4 (Math|Conversions|ToInteger(Byte) ObjectType))
  (bind _spawnableobjects (Variables|Default|GetSpawnableObjects))
  (bind _returnvalue_5 (Math|Transform|TransformLocation _returnvalue_2 Location))
  (bind _returnvalue_6 (Math|Conversions|ToInteger(Byte) _returnvalue_3))
  (bind _output (Utilities|Array|Get(acopy) _spawnableobjects _returnvalue_4))
  (bind (_preview _previewskeletal _cost _rotationoffset _rotationoffsetpreview _scalepreview _class _placeablelimitname _pleaceablelimitmax _performcapsulecheck _capsulecheckradius _capsulecheckhalfheight _spawnactoroffset _donotattach) (Utilities|Struct|BreakBP_ToolBoxSpawnable _output))
  (bind _returnvalue_7 (Math|Conversions|ToInteger(Byte) _cost))
  (Utilities|IsValid AttachTo
    (:Is%20Valid
      (Utilities|IsValid _returnvalue
        (:Is%20Valid
          (bind _asbp_mordhau_player_controller (Utilities|Casting|CastToBP_MordhauPlayerController (Pawn|GetController _returnvalue)))
          (if (Math|Vector|Equal(Vector) _returnvalue_5 (Transformation|GetActorLocation _returnvalue) 5e+02)
            (if (Utilities|Array|IsValidIndex _spawnableobjects _returnvalue_4)
              (if (>= _returnvalue_6 _returnvalue_7)
                (bind _returnvalue_8 (Game|SpawnActorfromClass _class (Math|Transform|MakeTransform _returnvalue_5 (Math|Transform|TransformRotation _returnvalue_2 Rotation)) "Undefined" 0 0))
                (Utilities|IsValid _returnvalue_8
                  (:Is%20Valid
                    (Utilities|FlowControl|Sequence
                      (:then_0
                        (bind _asbp_destroyable_deploy_spike_wall (Utilities|Casting|CastToBP_DestroyableDeploySpikeWall _returnvalue_8))
                        (Variables|/Game/Mordhau/Blueprints/Interactables/Environment/Specific/BP_DestroyableDeploySpikeWall.BP_DestroyableDeploySpikeWall_C|SetPlanterController _asbp_destroyable_deploy_spike_wall _asbp_mordhau_player_controller))
                      (:then_1
                        (if (not _donotattach)
                          (Transformation|AttachComponentToComponent _returnvalue_8 AttachTo "None" "KeepWorld" "KeepWorld" "KeepWorld" false)))
                      (:then_2
                        (Class|MordhauEquipment|SetAmmo (Math|Conversions|ToByte(Integer) (- _returnvalue_6 _returnvalue_7)))
                        (bind _removedactor (Default|PlaceinPlaceableArray _asbp_mordhau_player_controller _placeablelimitname _returnvalue_8 _pleaceablelimitmax))
                        (Utilities|IsValid _removedactor
                          (:Is%20Valid
                            (bind _asbp_destroyable_actor (Utilities|Casting|CastToBP_DestroyableActor _removedactor)
                              (:then
                                (Default|SetHealth _asbp_destroyable_actor 0.0))
                              (:CastFailed
                                (bind _asadvanced_character (Utilities|Casting|CastToAdvancedCharacter _removedactor)
                                  (:then
                                    (Utilities|FlowControl|Sequence
                                      (:then_0
                                        (bind _asmordhau_vehicle (Utilities|Casting|CastToMordhauVehicle _asadvanced_character))
                                        (Class|MordhauVehicle|StopDriving _asmordhau_vehicle))
                                      (:then_1
                                        (Class|AdvancedCharacter|Suicide _asadvanced_character))))
                                  (:CastFailed
                                    (Actor|DestroyActor _removedactor)))))))))))))))))))

(fn AddSkeletalMeshPreviewifNone
  (params (SkeletalMesh :type Skeletal%20Mesh%20Object%20Reference))
  (bind _asskeletal_mesh_component (Utilities|Casting|CastToSkeletalMeshComponent (Variables|Default|GetPreviewMeshComponent))
    (:then
      (if (!= (Variables|/Script/Engine.SkinnedMeshComponent|GetSkeletalMesh _asskeletal_mesh_component) SkeletalMesh)
        (CallFunction|DestroyMeshPreview :!label _label)
        (bind _returnvalue (AddComponent|AddSkeletalMeshComponent false))
        (Class|SkinnedMeshComponent|SetSkeletalMesh _returnvalue SkeletalMesh true)
        (Variables|Default|SetPreviewMeshComponent _returnvalue)
        (CallFunction|SetupMeshPreview)))
    (:CastFailed
      (goto _label))))

(fn AddStaticMeshPreviewifNone
  (params (StaticMesh :type Static%20Mesh%20Object%20Reference))
  (bind _asstatic_mesh_component (Utilities|Casting|CastToStaticMeshComponent (Variables|Default|GetPreviewMeshComponent))
    (:then
      (if (!= (Variables|/Script/Engine.StaticMeshComponent|GetStaticMesh _asstatic_mesh_component) StaticMesh)
        (CallFunction|DestroyMeshPreview :!label _label)
        (bind _returnvalue (AddComponent|AddStaticMeshComponent false))
        (Components|StaticMesh|SetStaticMesh _returnvalue StaticMesh)
        (Variables|Default|SetPreviewMeshComponent _returnvalue)
        (CallFunction|SetupMeshPreview)))
    (:CastFailed
      (goto _label))))

(fn DestroyMeshPreview
  (Utilities|FlowControl|Sequence
    (:then_0
      (Utilities|IsValid (Variables|Default|GetWidgetDisplay)
        (:Is%20Valid
          (Components|DestroyComponent (Variables|Default|GetWidgetDisplay))
          (Variables|Default|SetWidgetDisplay 0))))
    (:then_1
      (Utilities|IsValid (Variables|Default|GetPreviewMeshComponent)
        (:Is%20Valid
          (Components|DestroyComponent (Variables|Default|GetPreviewMeshComponent))
          (Variables|Default|SetPreviewMeshComponent 0))))))

(fn SetupMeshPreview
  (bind _previewmeshcomponent (Variables|Default|GetPreviewMeshComponent))
  (Utilities|IsValid _previewmeshcomponent
    (:Is%20Valid
      (Utilities|FlowControl|Sequence
        (:then_1
          (Transformation|SetAbsolute _previewmeshcomponent true true true)
          (Collision|SetCollisionEnabled _previewmeshcomponent "NoCollision")
          (for _index (range 0 (- (Rendering|Material|GetNumMaterials _previewmeshcomponent) 1))
            (Rendering|Material|CreateDynamicMaterialInstance _previewmeshcomponent _index 0 "None" :!class /Script/Engine.PrimitiveComponent)))))))

(fn CycleObjectType
  (bind _spawnableobjects (Variables|Default|GetSpawnableObjects))
  (bind _returnvalue (Utilities|Array|Length _spawnableobjects))
  (bind _returnvalue_2 (- _returnvalue 0))
  (bind _index (Utilities|FlowControl|ForLoopwithBreak 1 _returnvalue_2 :!label _label)
    (:LoopBody
      (if (<= (.Cost (Utilities|Struct|BreakBP_ToolBoxSpawnable (Utilities|Array|Get(acopy) _spawnableobjects (Math|Integer|%(Integer) (+ (Variables|Default|GetObjectType) _index) _returnvalue_2)))) (Class|MordhauEquipment|GetAmmo))
        (Variables|Default|SetObjectType (Math|Integer|%(Integer) (+ (Variables|Default|GetObjectType) _index) _returnvalue_2))
        (goto _label Break)))))